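; Wall control for a left or right door, with a lever to open and close it and a button for its light.
; Timelines rotate the lever, then fire dispatchers for the side chosen by Door; the light also drives an emissive material, point light and audio.
; Door and light changes adjust the Usage actor's counter.
; CanInteract gates normal input, with separate events for disabling and power-out.
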(event `DoorOpenPowerOut`
  (bind (_direction _rot) (`Timeline|DoorLeverLift` :!via `PlayFromStart` :!label _label)
    (:`Update`
      (`SceneComponent.K2_SetRelativeRotation` (`self.SM_DoorLever`) (`KismetMathLibrary.MakeRotator` 0.0 _rot) false false))
    (:`Finished`
      (switch `int` (`self.Door`)
        (:`0`
          (`self.LeftDoorOpen`))
        (:`1`
          (`self.RightDoorOpen`)))
      (bind _returnvalue (`GameplayStatics.GetActorOfClass` "/Game/Core/Assets/Interactables/Usage.Usage_C"))
      (set `/Game/Core/Assets/Interactables/Usage.Usage` (- (`/Game/Core/Assets/Interactables/Usage.Usage` _returnvalue) 1) _returnvalue)
      (`/Game/Core/Assets/Interactables/Usage.Update` _returnvalue)
      (set `self.DoorClosed` false))))

(event `DoorOpen`
  (`GameplayStatics.PlaySound2D` "/Game/Core/Player/sounds/crank1.crank1" 1.0 1.0 0.0 null null)
  (`KismetSystemLibrary.Delay` 0.1)
  (if (`self.CanInteract`)
    (goto _label :!via `PlayFromStart`)))

(event `DoorClose`
  (`GameplayStatics.PlaySound2D` "/Game/Core/Player/sounds/crank2.crank2" 1.0 1.0 0.0 null null)
  (`KismetSystemLibrary.Delay` 0.1)
  (if (`self.CanInteract`)
    (bind (_direction _rot) (`Timeline|DoorLeverAnim` :!via `PlayFromStart`)
      (:`Update`
        (`SceneComponent.K2_SetRelativeRotation` (`self.SM_DoorLever`) (`KismetMathLibrary.MakeRotator` 0.0 _rot) false false))
      (:`Finished`
        (switch `int` (`self.Door`)
          (:`0`
            (`self.LeftDoorClosed`))
          (:`1`
            (`self.RightDoorClosed`)))
        (bind _returnvalue (`GameplayStatics.GetActorOfClass` "/Game/Core/Assets/Interactables/Usage.Usage_C"))
        (set `/Game/Core/Assets/Interactables/Usage.Usage` (+ (`/Game/Core/Assets/Interactables/Usage.Usage` _returnvalue) 1) _returnvalue)
        (`/Game/Core/Assets/Interactables/Usage.Update` _returnvalue)
        (set `self.DoorClosed` true)))))

(event `self.ReceiveBeginPlay`
  (bind _returnvalue (`PrimitiveComponent.CreateDynamicMaterialInstance` (`self.Light`) 0 "/Game/Core/Assets/Props/LightButton/MI_LightBulb.MI_LightBulb" "None"))
  (bind _output_get (set `self.LightButton` _returnvalue))
  (`MaterialInstanceDynamic.SetScalarParameterValue` _output_get "EmissiveColor Intensity" 1.0))

(event `LightOn`
  (`GameplayStatics.PlaySound2D` "/Game/Core/Assets/Widgets/Textures/open_lights.open_lights" 1.0 1.0 0.0 null null)
  (if (`self.LightActive`)
    _
    (elif (`self.CanInteract`)
      (switch `int` (`self.Door`)
        (:`0`
          (`self.LightLeftOn`))
        (:`1`
          (`self.LightRightOn`)))
      (set `self.LightActive` true)
      (bind _returnvalue (`GameplayStatics.GetActorOfClass` "/Game/Core/Assets/Interactables/Usage.Usage_C"))
      (set `/Game/Core/Assets/Interactables/Usage.Usage` (+ (`/Game/Core/Assets/Interactables/Usage.Usage` _returnvalue) 1) _returnvalue)
      (`/Game/Core/Assets/Interactables/Usage.Update` _returnvalue)
      (`MaterialInstanceDynamic.SetScalarParameterValue` (`self.LightButton`) "EmissiveColor Intensity" 16.0)
      (`AudioComponent.Play` (`self.Audio`) 0.0)
      (`SceneComponent.SetVisibility` (`self.PointLight`) true false))))

(event `LightOff`
  (if (`self.LightActive`)
    (if (`self.CanInteract`)
      (switch `int` (`self.Door`)
        (:`0`
          (`self.LightLeftOff`))
        (:`1`
          (`self.LightRightOff`)))
      (set `self.LightActive` false)
      (bind _returnvalue (`GameplayStatics.GetActorOfClass` "/Game/Core/Assets/Interactables/Usage.Usage_C"))
      (set `/Game/Core/Assets/Interactables/Usage.Usage` (- (`/Game/Core/Assets/Interactables/Usage.Usage` _returnvalue) 1) _returnvalue)
      (`/Game/Core/Assets/Interactables/Usage.Update` _returnvalue)
      (`MaterialInstanceDynamic.SetScalarParameterValue` (`self.LightButton`) "EmissiveColor Intensity" 1.0)
      (`AudioComponent.Stop` (`self.Audio`) :!label _label_2)
      (`SceneComponent.SetVisibility` (`self.PointLight`) false false))))

(event `CharacterDisable`
  (set `self.CanInteract` false)
  (`self.LightLeftOff`)
  (`self.LightRightOff`)
  (set `self.LightActive` false)
  (`MaterialInstanceDynamic.SetScalarParameterValue` (`self.LightButton`) "Emmisive Multiplier" 0.05)
  (goto _label_2))

(event `TemporaryDisable`
  (`self.LightOff`)
  (set `self.CanInteract` false)
  (`KismetSystemLibrary.Delay` 1.25)
  (set `self.CanInteract` true))

(event `Powerout`
  (switch `int` (`self.Door`)
    (:`0`
      (`self.LightLeftOff`))
    (:`1`
      (`self.LightRightOff`)))
  (set `self.LightActive` false)
  (bind _returnvalue (`GameplayStatics.GetActorOfClass` "/Game/Core/Assets/Interactables/Usage.Usage_C"))
  (set `/Game/Core/Assets/Interactables/Usage.Usage` (- (`/Game/Core/Assets/Interactables/Usage.Usage` _returnvalue) 1) _returnvalue)
  (`/Game/Core/Assets/Interactables/Usage.Update` _returnvalue)
  (`MaterialInstanceDynamic.SetScalarParameterValue` (`self.LightButton`) "EmissiveColor Intensity" 0.0)
  (`AudioComponent.Stop` (`self.Audio`))
  (`SceneComponent.SetVisibility` (`self.PointLight`) false false))

(fn `UserConstructionScript`)