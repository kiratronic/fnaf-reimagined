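; BP_Power drains the power supply during a night, one unit at a time, and calls CallPowerOff when it runs out.
; On BeginPlay it loads the current night from the save game and sets per-night drain intervals for each usage tier.
; UsageUpdate maps UsageRate to the active delay, with a fixed interval for the top tier.
; A self-retriggering Delay loop through PowerCycle performs the countdown.
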(event `UsageUpdate`
  (switch `int` (`self.UsageRate`)
    (:`0`
      (set `self.DelayTime` (`self.lowtime`)))
    (:`1`
      (set `self.DelayTime` (`self.mediumtime`)))
    (:`2`
      (set `self.DelayTime` (`self.hightime`)))
    (:`3`
      (set `self.DelayTime` (`self.verhightime`)))
    (:`4`
      (set `self.DelayTime` 1.0))))

(event `self.ReceiveBeginPlay`
  (`|ExecutionSequence`
    (:`then_0`
      (bind _returnvalue (`GameplayStatics.LoadGameFromSlot` "SaveData"))
      (bind _assave_game_object (cast `/Game/Core/SaveGameObject` _returnvalue))
      (switch `int` (`/Game/Core/SaveGameObject.Night` _assave_game_object)
        (:`1`
          (set `self.lowtime` 10.0)
          (set `self.mediumtime` 6.0)
          (set `self.hightime` 3.5)
          (set `self.verhightime` 2.0))
        (:`2`
          (set `self.lowtime` 9.0)
          (set `self.mediumtime` 5.0)
          (set `self.hightime` 2.5)
          (set `self.verhightime` 1.0))
        (:`3`
          (set `self.lowtime` 9.0)
          (set `self.mediumtime` 4.5)
          (set `self.hightime` 2.5)
          (set `self.verhightime` 0.75))
        (:`4`
          (set `self.lowtime` 8.0)
          (set `self.mediumtime` 4.0)
          (set `self.hightime` 2.0)
          (set `self.verhightime` 0.5))
        (:`5`
          (set `self.lowtime` 7.0)
          (set `self.mediumtime` 3.0)
          (set `self.hightime` 1.5)
          (set `self.verhightime` 0.5))
        (:`6`
          (set `self.lowtime` 6.0)
          (set `self.mediumtime` 2.5)
          (set `self.hightime` 1.0)
          (set `self.verhightime` 0.25))
        (:`7`
          (set `self.lowtime` 8.0)
          (set `self.mediumtime` 5.0)
          (set `self.hightime` 2.5)
          (set `self.verhightime` 1.75))))
    (:`then_1`
      (`self.UsageUpdate`)
      (`KismetSystemLibrary.Delay` (`self.DelayTime`) :!label _label)
      (if (== (`self.Power`) 1)
        (set `self.Power` 0)
        (`self.PowerOff`)
        (else
          (set `self.Power` (- (`self.Power`) 1))
          (`self.Power Cycle`))))))

(event `Power Cycle`
  (goto _label))

(fn `UserConstructionScript`)