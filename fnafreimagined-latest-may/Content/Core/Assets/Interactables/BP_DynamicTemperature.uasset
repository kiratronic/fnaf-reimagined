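; BP_DynamicTemperature simulates drifting temperatures for four camera rooms (1A, 1B, 5, 7), with debug prints.
; Duplicated per-room chains randomly nudge goals in RoomGoalTemperatureShared, while a DoOnce gated by ActivityInRoom leads to sharp goal drops.
; Delay-driven monitor and change events step each temperature one degree toward its goal.
; BeginPlay is empty, monitor start calls are unconnected, and Camera 7's monitor calls Camera 5's change event.
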(event `self.ReceiveBeginPlay`)

(event `1A Reset`
  (bind _returnvalue (- (`self.1A Temperature`) (`KismetMathLibrary.RandomIntegerInRange` 20 40)))
  ;[1 1 1] Camera 1A
  (goto _label_2 :!via `Reset`))

(event `1A Generate`
  (bind _1a_temperature (`self.1A Temperature`))
  (bind _returnvalue (- (`self.1A Temperature`) (`KismetMathLibrary.RandomIntegerInRange` 20 40)))
  ;[1 1 1] Camera 1A
  (for (_array_element _array_index) (`self.ActivityInRoom#`) :!label _label
    (if (== _array_index 0)
      (`|ExecutionSequence`
        (:`then_0`
          (`KismetSystemLibrary.Delay` 0.4)
          (break))
        (:`then_1`
          (if _array_element
            (`/Engine/EditorBlueprintResources/StandardMacros.DoOnce` false :!label _label_2
              (:`Completed`
                (for (_array_element_2 _array_index_2) (`self.RoomGoalTemperature(Shared)`)
                  (if (== _array_index_2 0)
                    (if (not (== (`self.1A Temperature`) 32))
                      (`KismetArrayLibrary.Array_Set` (`self.RoomGoalTemperature(Shared)`) _array_element_2 _returnvalue))
                    (`KismetSystemLibrary.PrintString` (`KismetStringLibrary.Conv_IntToString` _returnvalue) true true (struct :`G` 0.110118 :`B` 1.0 :`A` 1.0))))))
            (else
              (for (_ _array_index_3) (`self.RoomGoalTemperature(Shared)`)
                (if (== _array_index_3 0)
                  (if (`KismetMathLibrary.RandomBool`)
                    (if (>= _1a_temperature 74) :!label _label_3
                      (if (<= (`self.1A Temperature`) 60) :!label _label_4
                        (goto _label_3)
                        (else
                          (`KismetArrayLibrary.Array_Set` (`self.RoomGoalTemperature(Shared)`) _array_index_3 (- (`self.1A Temperature`) (`KismetMathLibrary.RandomIntegerInRange` 0 3)))))
                      (else
                        (`KismetArrayLibrary.Array_Set` (`self.RoomGoalTemperature(Shared)`) _array_index_3 (+ (`self.1A Temperature`) (`KismetMathLibrary.RandomIntegerInRange` 0 3)))
                        (`KismetSystemLibrary.PrintString` (`KismetStringLibrary.Conv_IntToString` _1a_temperature) true true (struct :`R` 0.304449 :`G` 1.0 :`A` 1.0))))
                    (else
                      (goto _label_4)))
                  (for (_array_element_3 _array_index_4) (`self.RoomGoalTemperature(Shared)`)
                    (if (== _array_index_4 0)
                      (`KismetSystemLibrary.PrintString` (`KismetStringLibrary.Conv_IntToString` _array_element_3) true true (struct :`R` 1.0 :`G` 0.297604 :`A` 1.0) 3.0)
                      (`self.1A Reset`))))))))))))

(event `Camera 1A Temperature Monitor`
  ;[1 1 1] Camera 1A
  (`KismetSystemLibrary.Delay` 2.0)
  (`|ExecutionSequence`
    (:`then_0`
      (goto _label))
    (:`then_1`
      (`self.1A Temperature Change`))))

(event `1A Temperature Change`
  (bind _1a_temperature (`self.1A Temperature`))
  ;[1 1 1] Camera 1A
  (`KismetSystemLibrary.Delay` 0.5)
  (for (_array_element _array_index) (`self.RoomGoalTemperature(Shared)`)
    (if (== _array_index 0)
      (if (== _array_element _1a_temperature)
        (`self.Camera 1A Temperature Monitor`)
        (else
          (if (> _array_element _1a_temperature)
            (`KismetSystemLibrary.Delay` 5.0)
            (set `self.1A Temperature` (+ (`self.1A Temperature`) 1))
            (else
              (`KismetSystemLibrary.Delay` 5.0)
              (set `self.1A Temperature` (- (`self.1A Temperature`) 1))))
          (`self.1A Temperature Change`)
          (`KismetSystemLibrary.PrintString` (`KismetStringLibrary.Conv_IntToString` (`self.1A Temperature`)) true true (struct :`G` 0.66 :`B` 1.0 :`A` 1.0) 3.0))))))

(event `1B Reset`
  (bind _returnvalue (- (`self.1B Temperature`) (`KismetMathLibrary.RandomIntegerInRange` 20 40)))
  ;[1 1 1] Camera 2B
  (goto _label_6 :!via `Reset`))

(event `1B Generate`
  (bind _1b_temperature (`self.1B Temperature`))
  (bind _returnvalue (- (`self.1B Temperature`) (`KismetMathLibrary.RandomIntegerInRange` 20 40)))
  ;[1 1 1] Camera 2B
  (for (_array_element _array_index) (`self.ActivityInRoom#`) :!label _label_5
    (if (== _array_index 1)
      (`|ExecutionSequence`
        (:`then_0`
          (`KismetSystemLibrary.Delay` 0.4)
          (break))
        (:`then_1`
          (if _array_element
            (`/Engine/EditorBlueprintResources/StandardMacros.DoOnce` false :!label _label_6
              (:`Completed`
                (for (_array_element_2 _array_index_2) (`self.RoomGoalTemperature(Shared)`)
                  (if (== _array_index_2 1)
                    (if (not (== (`self.1B Temperature`) 32))
                      (`KismetArrayLibrary.Array_Set` (`self.RoomGoalTemperature(Shared)`) _array_element_2 _returnvalue))
                    (`KismetSystemLibrary.PrintString` (`KismetStringLibrary.Conv_IntToString` _returnvalue) true true (struct :`G` 0.110118 :`B` 1.0 :`A` 1.0))))))
            (else
              (for (_ _array_index_3) (`self.RoomGoalTemperature(Shared)`)
                (if (== _array_index_3 1)
                  (if (`KismetMathLibrary.RandomBool`)
                    (if (>= _1b_temperature 74) :!label _label_7
                      (if (<= (`self.1B Temperature`) 60) :!label _label_8
                        (goto _label_7)
                        (else
                          (`KismetArrayLibrary.Array_Set` (`self.RoomGoalTemperature(Shared)`) _array_index_3 (- (`self.1B Temperature`) (`KismetMathLibrary.RandomIntegerInRange` 0 3)))))
                      (else
                        (`KismetArrayLibrary.Array_Set` (`self.RoomGoalTemperature(Shared)`) _array_index_3 (+ (`self.1B Temperature`) (`KismetMathLibrary.RandomIntegerInRange` 0 3)))
                        (`KismetSystemLibrary.PrintString` (`KismetStringLibrary.Conv_IntToString` _1b_temperature) true true (struct :`R` 0.304449 :`G` 1.0 :`A` 1.0))))
                    (else
                      (goto _label_8)))
                  (for (_ _array_index_4) (`self.RoomGoalTemperature(Shared)`)
                    (if (== _array_index_4 1)
                      (`KismetSystemLibrary.PrintString` (`KismetStringLibrary.Conv_IntToString` _array_index_4) true true (struct :`R` 1.0 :`G` 0.297604 :`A` 1.0) 3.0)
                      (`self.1B Reset`))))))))))))

(event `Camera 1B Temperature Monitor`
  ;[1 1 1] Camera 2B
  (`KismetSystemLibrary.Delay` 2.0)
  (`|ExecutionSequence`
    (:`then_0`
      (goto _label_5))
    (:`then_1`
      (`self.1B Temperature Change`))))

(event `1B Temperature Change`
  (bind _1b_temperature (`self.1B Temperature`))
  ;[1 1 1] Camera 2B
  (`KismetSystemLibrary.Delay` 0.5)
  (for (_array_element _array_index) (`self.RoomGoalTemperature(Shared)`)
    (if (== _array_index 1)
      (if (== _array_element _1b_temperature)
        (`self.Camera 1B Temperature Monitor`)
        (else
          (if (> _array_element _1b_temperature)
            (`KismetSystemLibrary.Delay` 5.0)
            (set `self.1B Temperature` (+ (`self.1B Temperature`) 1))
            (else
              (`KismetSystemLibrary.Delay` 5.0)
              (set `self.1B Temperature` (- (`self.1B Temperature`) 1))))
          (`self.1B Temperature Change`)
          (`KismetSystemLibrary.PrintString` (`KismetStringLibrary.Conv_IntToString` (`self.1B Temperature`)) true true (struct :`G` 0.66 :`B` 1.0 :`A` 1.0) 3.0))))))

(event `5 Reset`
  (bind _returnvalue (- (`self.5 Temperature`) (`KismetMathLibrary.RandomIntegerInRange` 20 40)))
  ;[1 1 1] Camera 5
  (goto _label_10 :!via `Reset`))

(event `5 Generate`
  (bind _5_temperature (`self.5 Temperature`))
  (bind _returnvalue (- (`self.5 Temperature`) (`KismetMathLibrary.RandomIntegerInRange` 20 40)))
  ;[1 1 1] Camera 5
  (for (_array_element _array_index) (`self.ActivityInRoom#`) :!label _label_9
    (if (== _array_index 2)
      (`|ExecutionSequence`
        (:`then_0`
          (`KismetSystemLibrary.Delay` 0.4)
          (break))
        (:`then_1`
          (if _array_element
            (`/Engine/EditorBlueprintResources/StandardMacros.DoOnce` false :!label _label_10
              (:`Completed`
                (for (_array_element_2 _array_index_2) (`self.RoomGoalTemperature(Shared)`)
                  (if (== _array_index_2 2)
                    (if (not (== (`self.5 Temperature`) 32))
                      (`KismetArrayLibrary.Array_Set` (`self.RoomGoalTemperature(Shared)`) _array_element_2 _returnvalue))
                    (`KismetSystemLibrary.PrintString` (`KismetStringLibrary.Conv_IntToString` _returnvalue) true true (struct :`G` 0.110118 :`B` 1.0 :`A` 1.0))))))
            (else
              (for (_ _array_index_3) (`self.RoomGoalTemperature(Shared)`)
                (if (== _array_index_3 2)
                  (if (`KismetMathLibrary.RandomBool`)
                    (if (>= _5_temperature 74) :!label _label_11
                      (if (<= (`self.5 Temperature`) 60) :!label _label_12
                        (goto _label_11)
                        (else
                          (`KismetArrayLibrary.Array_Set` (`self.RoomGoalTemperature(Shared)`) _array_index_3 (- (`self.5 Temperature`) (`KismetMathLibrary.RandomIntegerInRange` 0 3)))))
                      (else
                        (`KismetArrayLibrary.Array_Set` (`self.RoomGoalTemperature(Shared)`) _array_index_3 (+ (`self.5 Temperature`) (`KismetMathLibrary.RandomIntegerInRange` 0 3)))
                        (`KismetSystemLibrary.PrintString` (`KismetStringLibrary.Conv_IntToString` _5_temperature) true true (struct :`R` 0.304449 :`G` 1.0 :`A` 1.0))))
                    (else
                      (goto _label_12)))
                  (for (_array_element_3 _array_index_4) (`self.RoomGoalTemperature(Shared)`)
                    (if (== _array_index_4 2)
                      (`KismetSystemLibrary.PrintString` (`KismetStringLibrary.Conv_IntToString` _array_element_3) true true (struct :`R` 1.0 :`G` 0.297604 :`A` 1.0) 3.0)
                      (`self.5 Reset`))))))))))))

(event `Camera 5 Temperature Monitor`
  ;[1 1 1] Camera 5
  (`KismetSystemLibrary.Delay` 2.0)
  (`|ExecutionSequence`
    (:`then_0`
      (goto _label_9))
    (:`then_1`
      (`self.5 Temperature Change`))))

(event `5 Temperature Change`
  (bind _5_temperature (`self.5 Temperature`))
  ;[1 1 1] Camera 5
  (`KismetSystemLibrary.Delay` 0.5)
  (for (_array_element _array_index) (`self.RoomGoalTemperature(Shared)`)
    (if (== _array_index 2)
      (if (== _array_element _5_temperature)
        (`self.Camera 5 Temperature Monitor`)
        (else
          (if (> _array_element _5_temperature)
            (`KismetSystemLibrary.Delay` 5.0)
            (set `self.5 Temperature` (+ (`self.5 Temperature`) 1))
            (else
              (`KismetSystemLibrary.Delay` 5.0)
              (set `self.5 Temperature` (- (`self.5 Temperature`) 1))))
          (`self.5 Temperature Change`)
          (`KismetSystemLibrary.PrintString` (`KismetStringLibrary.Conv_IntToString` (`self.5 Temperature`)) true true (struct :`G` 0.66 :`B` 1.0 :`A` 1.0) 3.0))))))

(event `7 Reset`
  (bind _returnvalue (- (`self.7 Temperature`) (`KismetMathLibrary.RandomIntegerInRange` 20 40)))
  ;[1 1 1] Camera 7
  (goto _label_14 :!via `Reset`))

(event `7 Generate`
  (bind _7_temperature (`self.7 Temperature`))
  (bind _returnvalue (- (`self.7 Temperature`) (`KismetMathLibrary.RandomIntegerInRange` 20 40)))
  ;[1 1 1] Camera 7
  (for (_array_element _array_index) (`self.ActivityInRoom#`) :!label _label_13
    (if (== _array_index 3)
      (`|ExecutionSequence`
        (:`then_0`
          (`KismetSystemLibrary.Delay` 0.4)
          (break))
        (:`then_1`
          (if _array_element
            (`/Engine/EditorBlueprintResources/StandardMacros.DoOnce` false :!label _label_14
              (:`Completed`
                (for (_array_element_2 _array_index_2) (`self.RoomGoalTemperature(Shared)`)
                  (if (== _array_index_2 3)
                    (if (not (== (`self.7 Temperature`) 32))
                      (`KismetArrayLibrary.Array_Set` (`self.RoomGoalTemperature(Shared)`) _array_element_2 _returnvalue))
                    (`KismetSystemLibrary.PrintString` (`KismetStringLibrary.Conv_IntToString` _returnvalue) true true (struct :`G` 0.110118 :`B` 1.0 :`A` 1.0))))))
            (else
              (for (_ _array_index_3) (`self.RoomGoalTemperature(Shared)`)
                (if (== _array_index_3 3)
                  (if (`KismetMathLibrary.RandomBool`)
                    (if (>= _7_temperature 74) :!label _label_15
                      (if (<= (`self.7 Temperature`) 60) :!label _label_16
                        (goto _label_15)
                        (else
                          (`KismetArrayLibrary.Array_Set` (`self.RoomGoalTemperature(Shared)`) _array_index_3 (- (`self.7 Temperature`) (`KismetMathLibrary.RandomIntegerInRange` 0 3)))))
                      (else
                        (`KismetArrayLibrary.Array_Set` (`self.RoomGoalTemperature(Shared)`) _array_index_3 (+ (`self.7 Temperature`) (`KismetMathLibrary.RandomIntegerInRange` 0 3)))
                        (`KismetSystemLibrary.PrintString` (`KismetStringLibrary.Conv_IntToString` _7_temperature) true true (struct :`R` 0.304449 :`G` 1.0 :`A` 1.0))))
                    (else
                      (goto _label_16)))
                  (for (_array_element_3 _array_index_4) (`self.RoomGoalTemperature(Shared)`)
                    (if (== _array_index_4 3)
                      (`KismetSystemLibrary.PrintString` (`KismetStringLibrary.Conv_IntToString` _array_element_3) true true (struct :`R` 1.0 :`G` 0.297604 :`A` 1.0) 3.0)
                      (`self.7 Reset`))))))))))))

(event `Camera 7 Temperature Monitor`
  ;[1 1 1] Camera 7
  (`KismetSystemLibrary.Delay` 2.0)
  (`|ExecutionSequence`
    (:`then_0`
      (goto _label_13))
    (:`then_1`
      (`self.5 Temperature Change`))))

(event `7 Temperature Change`
  (bind _7_temperature (`self.7 Temperature`))
  ;[1 1 1] Camera 7
  (`KismetSystemLibrary.Delay` 0.5)
  (for (_array_element _array_index) (`self.RoomGoalTemperature(Shared)`)
    (if (== _array_index 3)
      (if (== _array_element _7_temperature)
        (`self.Camera 7 Temperature Monitor`)
        (else
          (if (> _array_element _7_temperature)
            (`KismetSystemLibrary.Delay` 5.0)
            (set `self.7 Temperature` (+ (`self.7 Temperature`) 1))
            (else
              (`KismetSystemLibrary.Delay` 5.0)
              (set `self.7 Temperature` (- (`self.7 Temperature`) 1))))
          (`self.Camera 7 Temperature Monitor`)
          (`KismetSystemLibrary.PrintString` (`KismetStringLibrary.Conv_IntToString` (`self.7 Temperature`)) true true (struct :`G` 0.66 :`B` 1.0 :`A` 1.0) 3.0))))))

(fn `UserConstructionScript`)