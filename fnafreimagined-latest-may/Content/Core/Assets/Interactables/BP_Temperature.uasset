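; Per-room temperature simulator that maps its RoomID to an index into shared activity and goal-temperature arrays.
; A delayed monitor loop drives goal generation, intended to nudge idle rooms slightly and sharply lower the goal for rooms with activity through a DoOnce.
; A recursive, delay-based event steps Temperature one degree at a time toward the goal, then resumes monitoring.
; Debug prints trace the values.
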(event `self.ReceiveBeginPlay`
  (`KismetSystemLibrary.PrintString` (`KismetStringLibrary.Conv_IntToString` (`self.RoomIndex#`)))
  (`self.Temperature Monitor`))

(event `Reset`
  (bind _temperature (`self.Temperature`))
  (bind _returnvalue (- _temperature (`KismetMathLibrary.RandomIntegerInRange` 20 40)))
  ;[1 1 1] Camera 1A
  (goto _label_2 :!via `Reset`))

(event `Generate`
  (bind _temperature (`self.Temperature`))
  (bind _temperature_2 (`self.Temperature`))
  (bind _returnvalue (- _temperature_2 (`KismetMathLibrary.RandomIntegerInRange` 20 40)))
  ;[1 1 1] Camera 1A
  (for (_array_element _array_index) (`self.ActivityInRoom#`) :!label _label
    (if (== _array_index (`self.RoomIndex#`))
      (`|ExecutionSequence`
        (:`then_0`
          (`KismetSystemLibrary.Delay` 0.4)
          (break))
        (:`then_1`
          (if _array_element
            (`/Engine/EditorBlueprintResources/StandardMacros.DoOnce` false :!label _label_2
              (:`Completed`
                (for (_array_element_2 _array_index_2) (`self.RoomGoalTemperature(Shared)`)
                  (if (== _array_index_2 (`self.RoomIndex#`))
                    (if (not (== _temperature_2 32))
                      (`KismetArrayLibrary.Array_Set` (`self.RoomGoalTemperature(Shared)`) _array_element_2 _returnvalue))
                    (`KismetSystemLibrary.PrintString` (`KismetStringLibrary.Conv_IntToString` _returnvalue) true true (struct :`G` 0.110118 :`B` 1.0 :`A` 1.0))))))
            (else
              (for (_array_element_3 _array_index_3) (`self.RoomGoalTemperature(Shared)`) :!label _label_3
                (if (== _array_element_3 (`self.RoomIndex#`))
                  (`|ExecutionSequence`
                    (:`then_0`
                      (`KismetSystemLibrary.Delay` 0.4)
                      (break))
                    (:`then_1`
                      (if (`KismetMathLibrary.RandomBool`)
                        (if (>= (`self.Temperature`) 74) :!label _label_4
                          (if (<= (`self.Temperature`) 60) :!label _label_5
                            (goto _label_4)
                            (else
                              (`KismetArrayLibrary.Array_Set` (`self.RoomGoalTemperature(Shared)`) 0 (- (`self.Temperature`) (`KismetMathLibrary.RandomIntegerInRange` 0 3)))))
                          (else
                            (`KismetArrayLibrary.Array_Set` (`self.RoomGoalTemperature(Shared)`) _array_index_3 (+ _temperature (`KismetMathLibrary.RandomIntegerInRange` 0 3)))
                            (`KismetSystemLibrary.PrintString` (`KismetStringLibrary.Conv_IntToString` _temperature) true true (struct :`R` 0.304449 :`G` 1.0 :`A` 1.0))))
                        (else
                          (goto _label_5)))
                      (for (_array_element_4 _array_index_4) (`self.RoomGoalTemperature(Shared)`)
                        (if (== _array_index_4 (`self.RoomIndex#`))
                          (`KismetSystemLibrary.PrintString` (`KismetStringLibrary.Conv_IntToString` _array_element_4) true true (struct :`R` 1.0 :`G` 0.297604 :`A` 1.0) 3.0)
                          (`self.Reset`)))))
                  (else
                    (`KismetSystemLibrary.Delay` 0.2)
                    (goto _label_3)))))))))))

(event `Temperature Monitor`
  ;[1 1 1] Camera 1A
  (`KismetSystemLibrary.Delay` 2.0)
  (`|ExecutionSequence`
    (:`then_0`
      (goto _label))
    (:`then_1`
      (`self.Temperature Change`))))

(event `Temperature Change`
  (bind _temperature (`self.Temperature`))
  ;[1 1 1] Camera 1A
  (`KismetSystemLibrary.Delay` 0.5)
  (for (_array_element _array_index) (`self.RoomGoalTemperature(Shared)`)
    (if (== _array_index (`self.RoomIndex#`))
      (if (== _array_element _temperature)
        (`self.Temperature Monitor`)
        (else
          (if (> _array_element _temperature)
            (`KismetSystemLibrary.Delay` 5.0)
            (bind _output_get (set `self.Temperature` (+ (`self.Temperature`) 1)))
            (else
              (`KismetSystemLibrary.Delay` 5.0)
              (set `self.Temperature` (- (`self.Temperature`) 1))))
          (`self.Temperature Change`)
          (switch `int` (`self.RoomIndex#`)
            (:`0`
              (`KismetSystemLibrary.PrintString` "1a"))
            (:`1`
              (`KismetSystemLibrary.PrintString` "1b"))
            (:`2`
              (`KismetSystemLibrary.PrintString` "5"))
            (:`3`
              (`KismetSystemLibrary.PrintString` "7"))
            (:`12`
              (`KismetSystemLibrary.PrintString` "Office"))))))))

(fn `UserConstructionScript`
  (switch `string` (`self.RoomID`)
    (:`1A`
      (set `self.RoomIndex#` 0))
    (:`1B`
      (set `self.RoomIndex#` 1))
    (:`5`
      (set `self.RoomIndex#` 2))
    (:`7`
      (set `self.RoomIndex#` 3))
    (:`1C`
      (set `self.RoomIndex#` 4))
    (:`2A`
      (set `self.RoomIndex#` 5))
    (:`2B`
      (set `self.RoomIndex#` 6))
    (:`3`
      (set `self.RoomIndex#` 7))
    (:`4A`
      (set `self.RoomIndex#` 8))
    (:`4B`
      (set `self.RoomIndex#` 9))
    (:`6`
      (set `self.RoomIndex#` 10))
    (:`8`
      (set `self.RoomIndex#` 11))
    (:`Office`
      (set `self.RoomIndex#` 12))))