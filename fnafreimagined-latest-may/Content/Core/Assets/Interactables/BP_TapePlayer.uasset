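; BP_TapePlayer is a tape player prop that mirrors the main menu's hovered option in the LVL_Room level.
; BeginPlay enables this menu behavior only when the current level is LVL_Room.
; Tick then finds the BP_n1menu widget, polls its New Game, Options and Quit flags into Selection, and swaps StaticMesh2's material to match.
; The NewGameHovered event is an empty stub.
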(event `self.ReceiveBeginPlay`
  (bind _returnvalue (`GameplayStatics.GetCurrentLevelName` true))
  (if (`KismetStringLibrary.EqualEqual_StrStr` _returnvalue "LVL_Room")
    (set `self.ActivateMenuBehavior` true)))

(event `self.ReceiveTick`
  (params (DeltaSeconds :type "Float (single-precision)"))
  (if (`self.ActivateMenuBehavior`)
    (bind _foundwidgets (`WidgetBlueprintLibrary.GetAllWidgetsOfClass` "/Game/Core/Assets/Widgets/BP_n1menu.BP_n1menu_C"))
    (`|ExecutionSequence`
      (:`then_0`
        (bind _output (`|GetArrayItem` _foundwidgets))
        (if (`/Game/Core/Assets/Widgets/BP_n1menu.newgamehovered` _output)
          (set `self.selection` 1)))
      (:`then_1`
        (if (`/Game/Core/Assets/Widgets/BP_n1menu.optionshovered` _output)
          (set `self.selection` 2)))
      (:`then_2`
        (if (`/Game/Core/Assets/Widgets/BP_n1menu.quitvariable` _output)
          (set `self.selection` 3)))
      (:`then_3`
        (switch `int` (`self.selection`)
          (:`1`
            (`PrimitiveComponent.SetMaterial` (`self.StaticMesh2`) 0 "/Game/Core/Assets/Props/MAINMENU/takerecorder/hovers/newgamehovered.newgamehovered"))
          (:`2`
            (`PrimitiveComponent.SetMaterial` (`self.StaticMesh2`) 0 "/Game/Core/Assets/Props/MAINMENU/takerecorder/hovers/optionshovered.optionshovered"))
          (:`3`
            (`PrimitiveComponent.SetMaterial` (`self.StaticMesh2`) 0 "/Game/Core/Assets/Props/MAINMENU/takerecorder/hovers/quithovered.quithovered")))))))

(event `NewGameHovered`)

(fn `UserConstructionScript`)