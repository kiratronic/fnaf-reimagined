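; Foxy's AI actor, which advances through Pirate's Cove stages toward a run and also plays the jumpscare.
; Night-based difficulty sets start delay, wait time and the odds for a looping d20 movement roll.
; Active cameras block advances, as does Bonnie on the left side for later stages.
; Each stage teleports Foxy and updates BP_PiratesCove; the last hides Foxy and activates FoxyRunBP through a resettable DoOnce.
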(event `BeginCycle`
  ;[1 1 1] Cycle Logic
  (`KismetSystemLibrary.Delay` (`self.WaitTime`))
  (if (`self.CanMove`)
    (if (and (`self.Running`) (`self.HoldingPosition`))
      (`self.BeginCycle`)
      (elif (<= (`KismetMathLibrary.RandomIntegerInRange` 1 20) (`self.AIDifficulty`))
        (`self.CameraCheck`)
        (`KismetSystemLibrary.Delay` 0.2)
        (if (`self.CamerasActive`)
          (`self.BeginCycle`)
          (elif (not (`self.Running`))
            (`self.MovementCycle`)))
        (else
          (`self.BeginCycle`))))
    (else
      (`self.BeginCycle`))))

(event `MovementCycle`
  ;[1 1 1] Movement Stage Logic
  (switch `int` (`self.CurrentStage`)
    (:`0`
      (`self.Peeking`))
    (:`1`
      (`self.AboutToRun`))
    (:`2`
      (`self.Run`))))

(event `PositionUpdate`
  ;[1 1 1] Movement Stage
  (`|ExecutionSequence`
    (:`then_0`
      (switch `int` (`self.CurrentStage`)
        (:`0`
          (`self.K2_TeleportTo` (0.0 0.0 500.0))
          (goto _label :!via `Reset`))
        (:`1`
          (`self.K2_TeleportTo` (1510.947742 -604.463649 77.005675) (struct :`Yaw` -50.0))
          (`SkeletalMeshComponent.PlayAnimation` (`self.SkeletalMesh`) "/Game/Core/Assets/Characters/Foxy/Animations/Stage01.Stage01" true)
          (bind _returnvalue (`GameplayStatics.GetActorOfClass` "/Game/Core/Assets/Props/PiratesCove/Stage/BP_PiratesCove.BP_PiratesCove_C"))
          (`/Game/Core/Assets/Props/PiratesCove/Stage/BP_PiratesCove.Peek` _returnvalue)
          (bind _returnvalue_2 (`GameplayStatics.GetActorOfClass` "/Game/Core/Assets/Characters/Foxy/Blueprint/FoxyRunBP.FoxyRunBP_C"))
          (set `/Game/Core/Assets/Characters/Foxy/Blueprint/FoxyRunBP.CanRun` false _returnvalue_2)
          (goto _label :!via `Reset`))
        (:`2`
          (`self.K2_TeleportTo` (1623.34468 -513.208414 63.34387) (struct :`Yaw` -50.0))
          (`SkeletalMeshComponent.PlayAnimation` (`self.SkeletalMesh`) "/Game/Core/Assets/Characters/Foxy/Animations/Stage02.Stage02" true)
          (bind _returnvalue_3 (`GameplayStatics.GetActorOfClass` "/Game/Core/Assets/Props/PiratesCove/Stage/BP_PiratesCove.BP_PiratesCove_C"))
          (`/Game/Core/Assets/Props/PiratesCove/Stage/BP_PiratesCove.AboutToRun` _returnvalue_3)
          (`/Game/Core/Assets/Characters/Foxy/Blueprint/FoxyRunBP.CanRunAgain` _returnvalue_2)
          (goto _label :!via `Reset`))
        (:`3`
          (`/Engine/EditorBlueprintResources/StandardMacros.DoOnce` false :!label _label
            (:`Completed`
              (`self.K2_TeleportTo` (0.0 0.0 500.0))
              (bind _returnvalue_4 (`GameplayStatics.GetActorOfClass` "/Game/Core/Assets/Props/PiratesCove/Stage/BP_PiratesCove.BP_PiratesCove_C"))
              (`/Game/Core/Assets/Props/PiratesCove/Stage/BP_PiratesCove.Run` _returnvalue_4)
              (bind _returnvalue_5 (`GameplayStatics.GetActorOfClass` "/Game/Core/Assets/Characters/Foxy/Blueprint/FoxyRunBP.FoxyRunBP_C"))
              (set `/Game/Core/Assets/Characters/Foxy/Blueprint/FoxyRunBP.CanRun` true _returnvalue_5)
              (`/Game/Core/Assets/Characters/Foxy/Blueprint/FoxyRunBP.Activate` _returnvalue_5)
              (set `self.Running` true))))))
    (:`then_1`
      (`KismetSystemLibrary.Delay` 3.0)
      (`self.BeginCycle`))))

(event `BehindCurtain`
  ;[1 1 1] Movement Check Logic
  (`self.CameraCheck`)
  (if (`self.CamerasActive`)
    (`self.BeginCycle`)
    (else
      (bind _output_get (set `self.ArrivalStage` 0))
      (set `self.CurrentStage` _output_get)
      (`self.PositionUpdate`))))

(event `Peeking`
  ;[1 1 1] Movement Check Logic
  (`self.CameraCheck`)
  (if (`self.CamerasActive`)
    (`self.BeginCycle`)
    (else
      (bind _output_get (set `self.ArrivalStage` 1))
      (set `self.CurrentStage` _output_get)
      (`self.PositionUpdate`))))

(event `AboutToRun`
  ;[1 1 1] Movement Check Logic
  (`self.CameraCheck`)
  (if (`self.CamerasActive`)
    (`self.BeginCycle` :!label _label_2)
    (else
      (bind _returnvalue (`GameplayStatics.GetActorOfClass` "/Game/Core/Assets/Characters/Bonnie/Blueprint/BonnieBP.BonnieBP_C"))
      (bind _currentlocation (`/Game/Core/Assets/Characters/Bonnie/Blueprint/BonnieBP.CurrentLocation` _returnvalue))
      (if (or (`KismetStringLibrary.EqualEqual_StrStr` _currentlocation "LeftHallway") (`KismetStringLibrary.EqualEqual_StrStr` _currentlocation "LeftCorner") (`KismetStringLibrary.EqualEqual_StrStr` _currentlocation "LeftDoor"))
        (goto _label_2)
        (elif (`self.CamerasActive`)
          (goto _label_2)
          (else
            (bind _output_get (set `self.ArrivalStage` 2))
            (set `self.CurrentStage` _output_get)
            (`self.PositionUpdate`)))))))

(event `Run`
  ;[1 1 1] Run Logic
  (`self.CameraCheck`)
  (if (not (`self.CamerasActive`))
    (bind _returnvalue (`GameplayStatics.GetActorOfClass` "/Game/Core/Assets/Characters/Bonnie/Blueprint/BonnieBP.BonnieBP_C"))
    (bind _currentlocation (`/Game/Core/Assets/Characters/Bonnie/Blueprint/BonnieBP.CurrentLocation` _returnvalue))
    (if (or (`KismetStringLibrary.EqualEqual_StrStr` _currentlocation "LeftHallway") (`KismetStringLibrary.EqualEqual_StrStr` _currentlocation "LeftCorner") (`KismetStringLibrary.EqualEqual_StrStr` _currentlocation "LeftDoor"))
      (`self.BeginCycle` :!label _label_3)
      (elif (`self.CamerasActive`)
        (goto _label_3)
        (else
          (bind _output_get (set `self.ArrivalStage` 3))
          (set `self.CurrentStage` _output_get)
          (`self.PositionUpdate`))))))

(event `self.ReceiveBeginPlay`
  ;[1 1 1] Difficulty
  (`KismetSystemLibrary.Delay` 2.0)
  (`self.Difficulty Define`))

(event `Difficulty Define`
  ;[1 1 1] Difficulty
  (switch `string` (`self.Night`)
    (:`Night1`
      (set `self.AIDifficulty` 1)
      (set `self.WaitTime` (`KismetMathLibrary.RandomFloatInRange` 15.0 25.0))
      (`KismetSystemLibrary.Delay` 75.0)
      (set `self.CanMove` true)
      (`self.BeginCycle`))
    (:`Night2`
      (set `self.AIDifficulty` 5)
      (set `self.WaitTime` (`KismetMathLibrary.RandomFloatInRange` 13.0 20.0))
      (`KismetSystemLibrary.Delay` 60.0)
      (set `self.CanMove` true)
      (`self.BeginCycle`))
    (:`Night3`
      (set `self.AIDifficulty` 20 :!label _label_4)
      (set `self.WaitTime` 5.0)
      (`KismetSystemLibrary.Delay` 0.1)
      (set `self.CanMove` true)
      (`self.BeginCycle`))
    (:`Night4`
      (set `self.AIDifficulty` 9)
      (set `self.WaitTime` (`KismetMathLibrary.RandomFloatInRange` 7.0 10.0))
      (`KismetSystemLibrary.Delay` 40.0)
      (set `self.CanMove` true)
      (`self.BeginCycle`))
    (:`Night5`
      (set `self.AIDifficulty` 12)
      (set `self.WaitTime` (`KismetMathLibrary.RandomFloatInRange` 5.0 12.0))
      (`KismetSystemLibrary.Delay` 30.0)
      (set `self.CanMove` true)
      (`self.BeginCycle`))
    (:`CustomNight`
      (goto _label_4))))

(event `Jumpscare`
  ;[1 1 1] Jumpscare
  (`/Engine/EditorBlueprintResources/StandardMacros.DoOnce` false
    (:`Completed`
      (`self.K2_TeleportTo` (-174.787033 -271.966705 20.0) (struct :`Yaw` -9.14))
      (`|ExecutionSequence`
        (:`then_0`
          (`KismetSystemLibrary.Delay` 0.25)
          (`/Engine/EditorBlueprintResources/StandardMacros.DoOnce` false
            (:`Completed`
              (`GameplayStatics.PlaySound2D` "/Game/Core/Player/XSCREAM.XSCREAM" 1.0 1.0 0.0 null null)
              (`SkeletalMeshComponent.PlayAnimation` (`self.CameraLink`) "/Game/Core/Assets/Characters/Foxy/Animations/foxjumpycube3_Anim_Cube_001_CameraAction.foxjumpycube3_Anim_Cube_001_CameraAction" false))))
        (:`then_1`
          (`SkeletalMeshComponent.PlayAnimation` (`self.SkeletalMesh`) "/Game/Core/Assets/Characters/Foxy/Animations/FoxJump.FoxJump" false))))))

(fn `UserConstructionScript`)