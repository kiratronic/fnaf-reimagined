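; Bonnie animatronic for a Five Nights at Freddy's-style game, roaming from the stage to the left office door and jumpscaring the player.
; Night sets difficulty and delay for a timed random roll that picks the next location from a branching route.
; Moves teleport Bonnie into posed animations and fire camera blur, pausing left-side advances during Foxy's attack.
; Tick polls the door for office entry; higher difficulty adds creepy corner whispers and poses.
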(event `Door Sequence`
  ;[1 1 1] Door Logic
  (if (`self.AtDoor`)
    (if (`self.LeftDoorClosed`)
      (`KismetSystemLibrary.Delay` 0.05)
      (if (not (`self.LeftDoorClosed`))
        (`KismetSystemLibrary.Delay` 1.0)
        (if (not (`self.LeftDoorClosed`)) :!label _label
          (set `self.InOffice` true)
          (`self.InOfficeLogic`)))
      (elif (`self.LightOn`)
        (`KismetSystemLibrary.Delay` 3.0)
        (goto _label)))))

(event `StageMove`
  ;[1 1 1] Teleport And Animation
  (`self.K2_TeleportTo` (3012.802862 -195.494781 90.0) (struct :`Yaw` 90.0) :!label _label_2)
  (`SkeletalMeshComponent.PlayAnimation` (`self.SkeletalMesh`) "/Game/Core/Assets/Characters/Bonnie/Animations/BonnieStagePose.BonnieStagePose" true))

(event `BeginCycle`
  ;[1 1 1] MovementChance
  (`KismetSystemLibrary.Delay` (`self.WaitTime`))
  (if (`self.CanMove`)
    (if (and (`self.InOffice`) (`self.HoldingPosition`))
      (`self.BeginCycle`)
      (elif (<= (`KismetMathLibrary.RandomIntegerInRange` 0 20) (`self.AIDifficulty`))
        (`self.MovementCycle`)
        (else
          (`self.BeginCycle`))))
    (else
      (`self.BeginCycle`))))

(event `InOfficeLogic`
  ;[1 1 1] Jumpscare
  (if (`self.CanMove`)
    (`/Engine/EditorBlueprintResources/StandardMacros.DoOnce` false
      (:`Completed`
        (`self.BonnieInOffice`)
        (`self.K2_TeleportTo` (0.0 0.0 500.0))))))

(event `JumpscareCall`
  ;[1 1 1] Jumpscare
  (if (`self.CanMove`)
    (`/Engine/EditorBlueprintResources/StandardMacros.DoOnce` false
      (:`Completed`
        (`SceneComponent.SetRelativeScale3D` (`self.SkeletalMesh`) (0.75 0.75 0.75))
        (`self.K2_TeleportTo` :`self` self :`DestLocation` (-100.68499 -66.185059 20.0))
        (`/Engine/EditorBlueprintResources/StandardMacros.DoOnce` false
          (:`Completed`
            (`GameplayStatics.PlaySound2D` "/Game/Core/Player/XSCREAM.XSCREAM" 1.0 1.0 0.0 null null)
            (`SkeletalMeshComponent.PlayAnimation` (`self.SkeletalMesh`) "/Game/Core/Assets/Characters/Bonnie/Animations/Bonnie_jumpy__1__RIG_Bonnie_ao_Action.Bonnie_jumpy__1__RIG_Bonnie_ao_Action" false)
            (`SkeletalMeshComponent.PlayAnimation` (`self.CameraLink`) "/Game/Core/Assets/Characters/Bonnie/Animations/Bonnie_jumpyCUBE_Anim_Cube_002_Cube_002Action_001.Bonnie_jumpyCUBE_Anim_Cube_002_Cube_002Action_001" false)))))))

(event `self.ReceiveBeginPlay`
  ;[1 1 1] Init
  (`self.StageMove`)
  (`KismetSystemLibrary.Delay` 2.0)
  (`self.Difficulty Define`))

(event `SpookyBonnieEnd`
  ;[1 1 1] Bonnie Spooky Activities
  (`AudioComponent.Stop` (`self.DemonWhisper`))
  (set `self.SpookyMode` false))

(event `MoveTrigger`
  (bind _arrivallocation (`self.ArrivalLocation`))
  ;[1 1 1] Teleport And Animation
  (`|ExecutionSequence`
    (:`then_0`
      (if (not (`KismetStringLibrary.EqualEqual_StrStr` "LeftCorner" _arrivallocation))
        (`self.SpookyBonnieEnd`)
        (`KismetSystemLibrary.Delay` 0.4))
      (switch `string` _arrivallocation
        (:`Default`
          (`self.BeginCycle`))
        (:`Stage`
          (goto _label_2))
        (:`Dining1`
          (if (`KismetMathLibrary.RandomBool`)
            (`self.K2_TeleportTo` (2299.399518 -52.554298 37.839706) (struct :`Yaw` -89.999999))
            (`SkeletalMeshComponent.PlayAnimation` (`self.SkeletalMesh`) "/Game/Core/Assets/Characters/Bonnie/Animations/ANIM_Showroom1.ANIM_Showroom1" true)
            (else
              (`self.K2_TeleportTo` (1804.205067 -88.690543 19.999938) (struct :`Yaw` -89.999999))
              (`SkeletalMeshComponent.PlayAnimation` (`self.SkeletalMesh`) "/Game/Core/Assets/Characters/Bonnie/Animations/ANIM_Showroom1.ANIM_Showroom1" true))))
        (:`Dining2`
          (`self.K2_TeleportTo` (2520.590238 -88.132883 90.480693) (struct :`Pitch` 8.043651 :`Yaw` -43.2691 :`Roll` 19.599914))
          (`SkeletalMeshComponent.PlayAnimation` (`self.SkeletalMesh`) "/Game/Core/Assets/Characters/Bonnie/Animations/HallwayNEW.HallwayNEW" true))
        (:`EmployeeOnly1`
          (if (`KismetMathLibrary.RandomBool`)
            (`self.K2_TeleportTo` (2997.185507 -1250.160755 37.847937) (struct :`Pitch` 9.91906 :`Yaw` -205.989107 :`Roll` -2.227658))
            (`SkeletalMeshComponent.PlayAnimation` (`self.SkeletalMesh`) "/Game/Core/Assets/Characters/Bonnie/Animations/Backstage02.Backstage02" true)
            (else
              (`self.K2_TeleportTo` (3023.637574 -1013.867927 25.070257) (struct :`Yaw` 169.999999))
              (`SkeletalMeshComponent.PlayAnimation` (`self.SkeletalMesh`) "/Game/Core/Assets/Characters/Bonnie/Animations/ANIM_Backstage1.ANIM_Backstage1" true))))
        (:`LeftHallway`
          (if (`KismetMathLibrary.RandomBool`)
            (`self.K2_TeleportTo` (850.0 -300.740874 19.355199) (struct :`Yaw` 109.344772))
            (`SkeletalMeshComponent.PlayAnimation` (`self.SkeletalMesh`) "/Game/Core/Assets/Characters/Bonnie/Animations/HallwayNEW.HallwayNEW" true)
            (else
              (`self.K2_TeleportTo` (521.594702 -300.74079 51.376583) (struct :`Yaw` 109.344772))
              (`SkeletalMeshComponent.PlayAnimation` (`self.SkeletalMesh`) "/Game/Core/Assets/Characters/Bonnie/Animations/HallwayNEW.HallwayNEW" true))))
        (:`Closet`
          (`self.K2_TeleportTo` (582.944309 -518.37402 101.936589) (struct :`Pitch` -15.149823 :`Yaw` 57.278664 :`Roll` -31.70068))
          (`SkeletalMeshComponent.PlayAnimation` (`self.SkeletalMesh`) "/Game/Core/Assets/Characters/Bonnie/Animations/ANIM_Closet.ANIM_Closet" true))
        (:`LeftCorner`
          (`self.K2_TeleportTo` (-389.739769 -248.596075 81.315548) (struct :`Pitch` -3.397737 :`Yaw` 319.929328 :`Roll` -3.207978))
          (`SkeletalMeshComponent.PlayAnimation` (`self.SkeletalMesh`) "/Game/Core/Assets/Characters/Bonnie/Animations/Hallway/A_HallwayCornerV2.A_HallwayCornerV2" true)
          (if (>= (`self.AIDifficulty`) 14)
            (set `self.SpookyMode` true)
            (`self.SpookyBonnie`)
            (else
              (`self.SpookyBonnieEnd`))))
        (:`LeftDoor`
          (`self.K2_TeleportTo` (-213.68802 -261.349571 19.999998))
          (`SkeletalMeshComponent.PlayAnimation` (`self.SkeletalMesh`) "/Game/Core/Assets/Characters/Bonnie/Animations/BonnieDoorAnimation.BonnieDoorAnimation" true))))
    (:`then_1`
      (if (`KismetStringLibrary.EqualEqual_StrStr` (`self.ArrivalLocation`) "LeftDoor")
        (`self.Door Sequence`)
        (`self.BeginCycle`)
        (else
          (`self.BeginCycle`)
          (set `self.AtDoor` false))))))

(event `self.ReceiveTick`
  (params (DeltaSeconds :type "Float (single-precision)"))
  ;[1 1 1] ugh
  (`self.Door Sequence`))

(event `SpookyBonnie`
  ;[1 1 1] Bonnie Spooky Activities
  (if (`self.SpookyMode`)
    (`|ExecutionSequence`
      (:`then_0`
        (`/Engine/EditorBlueprintResources/StandardMacros.DoOnce` false :!label _label_3
          (:`Completed`
            (`AudioComponent.Play` (`self.DemonWhisper`) 0.0)
            (`KismetSystemLibrary.Delay` 15.0)
            (if (`self.SpookyMode`)
              (goto _label_3 :!via `Reset`)
              (else
                (`AudioComponent.Stop` (`self.DemonWhisper`))
                (goto _label_3 :!via `Reset`))))))
      (:`then_1`
        (`self.CreepyPoseLogic`)))))

(event `TryAgain`
  (bind _returnvalue (`KismetMathLibrary.RandomIntegerInRange` 0 2))
  (bind _returnvalue_2 (!= _returnvalue (`self.RNGMove`)))
  ;[1 1 1] Random Movement
  (switch `string` (`self.CurrentLocation`) :!label _label_4
    (:`Stage`
      (switch `int` _returnvalue
        (:`0`
          (if _returnvalue_2
            (`self.Dining1`)
            (set `self.RNGMove` 0)))
        (:`1`
          (if _returnvalue_2
            (`self.Dining2`)
            (set `self.RNGMove` 1)))
        (:`2`
          (if _returnvalue_2
            (`self.EmployeeOnly1`)
            (set `self.RNGMove` 2)))))
    (:`Dining1`
      (if (or (> (`self.AIDifficulty`) 10) (>= (`self.Time`) 2))
        (`self.Hallway`)
        (elif (`KismetMathLibrary.RandomBool`)
          (`self.EmployeeOnly1`)
          (else
            (`self.Hallway`)))))
    (:`Dining2`
      (if (`KismetMathLibrary.RandomBool`)
        (`self.Closet`)
        (else
          (`self.Hallway`))))
    (:`EmployeeOnly1`
      (if (`KismetMathLibrary.RandomBool`)
        (`self.Dining1`)
        (else
          (`self.Dining2`))))
    (:`LeftHallway`
      (if (or (>= (`self.AIDifficulty`) (`KismetMathLibrary.RandomIntegerInRange` 0 20)) (>= 2 (`self.Time`)))
        (if (`KismetMathLibrary.RandomBool`)
          (`self.Corner`)
          (else
            (`self.Closet`)))
        (else
          (`self.Dining1`))))
    (:`Closet`
      (if (or (>= (`self.AIDifficulty`) (`KismetMathLibrary.RandomIntegerInRange` 0 20)) (>= 3 (`self.Time`)))
        (`self.Corner`)
        (else
          (`self.Hallway`))))
    (:`LeftCorner`
      (if (or (>= (`self.AIDifficulty`) (`KismetMathLibrary.RandomIntegerInRange` 0 20)) (>= 2 (`self.Time`)))
        (`self.Door`)
        (elif (`KismetMathLibrary.RandomBool`)
          (`self.Hallway`)
          (else
            (`self.Corner`)))))
    (:`LeftDoor`
      (if (`self.LeftDoorClosed`)
        (if (`KismetMathLibrary.RandomBool`)
          (`self.Dining1`)
          (elif (>= (`self.Time`) 4)
            (`self.Hallway`)
            (else
              (`self.EmployeeOnly1`))))
        (`self.BonnieFromDoor`)
        (else
          (set `self.InOffice` true)
          (`self.InOfficeLogic`))))))

(event `CreepyPoseLogic`
  ;[1 1 1] SpookyAnimations
  (`self.K2_TeleportTo` (-482.702524 -270.600276 33.445133))
  (if (`self.SpookyMode`)
    (`KismetSystemLibrary.Delay` 0.2)
    (`SkeletalMeshComponent.PlayAnimation` (`self.SkeletalMesh`) "/Game/Core/Assets/Characters/Bonnie/Animations/BonnieCorner_RIG_Bonnie_ao_RIG_Bonnie_aoAction.BonnieCorner_RIG_Bonnie_ao_RIG_Bonnie_aoAction" false)))

(event `MovementCycle`
  ;[1 1 1] Random Movement
  (goto _label_4))

(event `Difficulty Define`
  ;[1 1 1] Difficulty
  (switch `string` (`self.Night`)
    (:`Night1`
      (set `self.AIDifficulty` 4)
      (set `self.WaitTime` (`KismetMathLibrary.RandomFloatInRange` 7.0 12.0))
      (`KismetSystemLibrary.Delay` 30.0)
      (set `self.CanMove` true)
      (`self.BeginCycle`))
    (:`Night2`
      (set `self.AIDifficulty` 8)
      (set `self.WaitTime` (`KismetMathLibrary.RandomFloatInRange` 6.0 10.0))
      (`KismetSystemLibrary.Delay` 36.0)
      (set `self.CanMove` true)
      (`self.BeginCycle`))
    (:`Night3`
      (set `self.AIDifficulty` 12)
      (set `self.WaitTime` (`KismetMathLibrary.RandomFloatInRange` 8.0 11.0))
      (`KismetSystemLibrary.Delay` 24.0)
      (set `self.CanMove` true)
      (`self.BeginCycle`))
    (:`Night4`
      (set `self.AIDifficulty` 14)
      (set `self.WaitTime` (`KismetMathLibrary.RandomFloatInRange` 7.0 10.0))
      (`KismetSystemLibrary.Delay` 12.0)
      (set `self.CanMove` true)
      (`self.BeginCycle`))
    (:`Night5`
      (set `self.AIDifficulty` 15)
      (set `self.WaitTime` (`KismetMathLibrary.RandomFloatInRange` 6.0 8.0))
      (`KismetSystemLibrary.Delay` 6.0)
      (set `self.CanMove` true)
      (`self.BeginCycle`))
    (:`Night6`
      (set `self.AIDifficulty` 20)
      (set `self.WaitTime` (`KismetMathLibrary.RandomFloatInRange` 0.1 1.0))
      (`KismetSystemLibrary.Delay` 1.0)
      (set `self.CanMove` true)
      (`self.BeginCycle`))
    (:`CustomNight`
      (set `self.AIDifficulty` 20)
      (set `self.WaitTime` (`KismetMathLibrary.RandomFloatInRange` 10.0 12.0))
      (`KismetSystemLibrary.Delay` 5.0)
      (set `self.CanMove` true)
      (`self.BeginCycle`))))

(event `Dining1`
  ;[1 1 1] Movement Action
  (if (`self.HoldingPosition`)
    (`self.BeginCycle`)
    (else
      (bind _output_get (set `self.ArrivalLocation` "Dining1"))
      (`self.CameraBlur`)
      (set `self.CurrentLocation` _output_get)
      (`self.MoveTrigger`)
      (`self.BonnieMoved`))))

(event `Dining2`
  ;[1 1 1] Movement Action
  (if (`self.HoldingPosition`)
    (`self.BeginCycle`)
    (else
      (bind _output_get (set `self.ArrivalLocation` "Dining2"))
      (`self.CameraBlur`)
      (set `self.CurrentLocation` _output_get)
      (`self.MoveTrigger`)
      (`self.BonnieMoved`))))

(event `EmployeeOnly1`
  ;[1 1 1] Movement Action
  (if (`self.HoldingPosition`)
    (`self.BeginCycle`)
    (else
      (bind _output_get (set `self.ArrivalLocation` "EmployeeOnly1"))
      (`self.CameraBlur`)
      (set `self.CurrentLocation` _output_get)
      (`self.MoveTrigger`)
      (`self.BonnieMoved`))))

(event `Hallway`
  ;[1 1 1] Movement Action
  (bind _returnvalue (`GameplayStatics.GetActorOfClass` "/Game/Core/Assets/Characters/Foxy/Blueprint/FoxyStageBP.FoxyStageBP_C"))
  (if (or (== (`/Game/Core/Assets/Characters/Foxy/Blueprint/FoxyStageBP.ArrivalStage` _returnvalue) 3) (`/Game/Core/Assets/Characters/Foxy/Blueprint/FoxyStageBP.Running` _returnvalue))
    (set `self.HoldingPosition` true)
    (else
      (set `self.HoldingPosition` false)))
  (if (`self.HoldingPosition`)
    (`self.BeginCycle`)
    (else
      (bind _output_get (set `self.ArrivalLocation` "LeftHallway"))
      (`self.CameraBlur`)
      (set `self.CurrentLocation` _output_get)
      (`self.MoveTrigger`)
      (`self.BonnieMoved`))))

(event `Closet`
  ;[1 1 1] Movement Action
  (bind _returnvalue (`GameplayStatics.GetActorOfClass` "/Game/Core/Assets/Characters/Foxy/Blueprint/FoxyStageBP.FoxyStageBP_C"))
  (if (or (== (`/Game/Core/Assets/Characters/Foxy/Blueprint/FoxyStageBP.ArrivalStage` _returnvalue) 3) (`/Game/Core/Assets/Characters/Foxy/Blueprint/FoxyStageBP.Running` _returnvalue))
    (set `self.HoldingPosition` true)
    (else
      (set `self.HoldingPosition` false)))
  (if (`self.HoldingPosition`)
    (`self.BeginCycle`)
    (else
      (bind _output_get (set `self.ArrivalLocation` "Closet"))
      (`self.CameraBlur`)
      (set `self.CurrentLocation` _output_get)
      (`self.MoveTrigger`)
      (`self.BonnieMoved`))))

(event `StageSpookMoment`
  ;[1 1 1] Stage Scare
  (if (and (`KismetStringLibrary.EqualEqual_StrStr` (`self.CurrentLocation`) "Stage") (`KismetMathLibrary.RandomBool`))
    (`SkeletalMeshComponent.PlayAnimation` (`self.SkeletalMesh`) "/Game/Core/Assets/Characters/Bonnie/Animations/BonnieStageSpookAnim.BonnieStageSpookAnim" false)))

(event `Corner`
  ;[1 1 1] Movement Action
  (bind _returnvalue (`GameplayStatics.GetActorOfClass` "/Game/Core/Assets/Characters/Foxy/Blueprint/FoxyStageBP.FoxyStageBP_C"))
  (if (or (== (`/Game/Core/Assets/Characters/Foxy/Blueprint/FoxyStageBP.ArrivalStage` _returnvalue) 3) (`/Game/Core/Assets/Characters/Foxy/Blueprint/FoxyStageBP.Running` _returnvalue))
    (set `self.HoldingPosition` true)
    (else
      (set `self.HoldingPosition` false)))
  (if (`self.HoldingPosition`)
    (`self.BeginCycle`)
    (else
      (bind _output_get (set `self.ArrivalLocation` "LeftCorner"))
      (`self.CameraBlur`)
      (set `self.CurrentLocation` _output_get)
      (`self.MoveTrigger`)
      (`self.BonnieMoved`))))

(event `StageSpookOff`
  ;[1 1 1] Stage Scare
  (if (`KismetStringLibrary.EqualEqual_StrStr` (`self.CurrentLocation`) "Stage")
    (`SkeletalMeshComponent.PlayAnimation` (`self.SkeletalMesh`) "/Game/Core/Assets/Characters/Bonnie/Animations/BonnieStagePose.BonnieStagePose" true)))

(event `Door`
  ;[1 1 1] Movement Action
  (bind _returnvalue (`GameplayStatics.GetActorOfClass` "/Game/Core/Assets/Characters/Foxy/Blueprint/FoxyStageBP.FoxyStageBP_C"))
  (if (or (== (`/Game/Core/Assets/Characters/Foxy/Blueprint/FoxyStageBP.ArrivalStage` _returnvalue) 3) (`/Game/Core/Assets/Characters/Foxy/Blueprint/FoxyStageBP.Running` _returnvalue))
    (set `self.HoldingPosition` true)
    (else
      (set `self.HoldingPosition` false)))
  (if (`self.HoldingPosition`)
    (`self.BeginCycle`)
    (else
      (`self.BonnieToDoor`)
      (bind _output_get (set `self.ArrivalLocation` "LeftDoor"))
      (`self.CameraBlur`)
      (set `self.CurrentLocation` _output_get)
      (`self.MoveTrigger`)
      (set `self.AtDoor` true)
      (`self.BonnieMoved`))))

(fn `UserConstructionScript`)