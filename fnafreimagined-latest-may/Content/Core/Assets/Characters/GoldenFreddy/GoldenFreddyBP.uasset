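; Golden Freddy character Blueprint that handles his scripted start pose, breaker-scene appearance and office haunting.
; Once ready, raising the monitor or triggering the office scene with it active teleports him into the office once and notifies PlayerBP.
; A self-retriggering delay loop then polls whether the player sees him, playing or reversing the AngerScale timeline.
; That timeline drives the anim Blueprint's twitch scale and the eye material's emissive glow.
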(event `Start Primary`
  (`self.K2_TeleportTo` (-547.56496 -62.026626 81.150558) (struct :`Pitch` 21.886114 :`Yaw` -94.557988 :`Roll` 29.383958))
  (`SkeletalMeshComponent.PlayAnimation` (`self.GoldenFreddy`) null true))

(event `Teleport For Breaker Scene`
  (`SceneComponent.SetVisibility` (`self.GoldenFreddy`) false false)
  (`self.K2_TeleportTo` (199.66953 845.176996 21.887672))
  (`SkeletalMeshComponent.PlayAnimation` (`self.GoldenFreddy`) "/Game/Core/Assets/Characters/GoldenFreddy/Animations/GoldenFreddyCreepyPose_RIG_Freddy_ao_RIG_Freddy_aoAction.GoldenFreddyCreepyPose_RIG_Freddy_ao_RIG_Freddy_aoAction" true))

(event `Play Breaker Scene`
  (`SceneComponent.SetVisibility` (`self.GoldenFreddy`) true false))

(event `MonitorUp`
  (if (`self.Ready`)
    (`self.OfficeSpookyTime`)))

(event `OfficeScene`
  (if (`self.Ready`)
    (`self.CameraCheckGF`)
    (if (`self.MonitorActive`)
      (`self.OfficeSpookyTime`))
    (else
      (`KismetSystemLibrary.PrintString` "GF READY ERROR" true true (struct :`R` 1.0 :`B` 0.556642 :`A` 1.0) 15.0))))

(event `OfficeSpookyTime`
  (`/Engine/EditorBlueprintResources/StandardMacros.DoOnce` false
    (:`Completed`
      (`self.K2_TeleportTo` (-295.263952 -52.543351 -2.499309))
      (bind _returnvalue (`PrimitiveComponent.CreateDynamicMaterialInstance` (`self.GoldenFreddy`) 2 null "None"))
      (bind _output_get (set `self.EyeBrightness` _returnvalue))
      (`MaterialInstanceDynamic.SetScalarParameterValue` _output_get "Emissive" 0.0)
      (set `self.IsActiveInOffice` true)
      (`self.AngerTimer`)
      (bind _asplayer_bp (cast `/Game/Core/Player/PlayerBP` (`GameplayStatics.GetPlayerCharacter` 0)))
      (set `/Game/Core/Player/PlayerBP.GFActive` true _asplayer_bp)
      (`/Game/Core/Player/PlayerBP.GFreddyActive` _asplayer_bp))))

(event `AngerPlus`
  (bind (_direction _twitch _eyes) (`Timeline|AngerScale` :!label _label)
    (:`Update`
      (bind _asgfanim_bp (cast `/Game/Core/Assets/Characters/GoldenFreddy/Animations/GFAnimBP` (`SkeletalMeshComponent.GetAnimInstance` (`self.GoldenFreddy`))))
      (set `/Game/Core/Assets/Characters/GoldenFreddy/Animations/GFAnimBP.Scale` _twitch _asgfanim_bp)
      (bind _returnvalue (`PrimitiveComponent.CreateDynamicMaterialInstance` (`self.GoldenFreddy`) 2 null "None"))
      (bind _output_get (set `self.EyeBrightness` _returnvalue))
      (`MaterialInstanceDynamic.SetScalarParameterValue` _output_get "Emissive" _eyes))))

(event `AngerTimer`
  (if (`self.IsActiveInOffice`)
    (`|ExecutionSequence`
      (:`then_0`
        (`KismetSystemLibrary.Delay` 0.05)
        (`self.AngerTimer`))
      (:`then_1`
        (bind _asplayer_bp (cast `/Game/Core/Player/PlayerBP` (`GameplayStatics.GetPlayerCharacter` 0)))
        (if (`/Game/Core/Player/PlayerBP.SeeGf` _asplayer_bp)
          (`self.AngerPlus`)
          (else
            (`self.AngerMinus`)))))))

(event `AngerMinus`
  (goto _label :!via `Reverse`))

(fn `UserConstructionScript`)