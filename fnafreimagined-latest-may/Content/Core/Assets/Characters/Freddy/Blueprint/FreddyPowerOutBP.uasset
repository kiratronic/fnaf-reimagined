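; Freddy actor for the power-out sequence, exposing events for peeking in, the music show, its end and the jumpscare.
; The show plays the Toreador cue at the actor and flickers two point lights at random.
; Ending it kills lights and music, then calls JumpscareReady after a random delay.
; The one-shot jumpscare teleports the actor, plays the scream and animations on Freddy and a cube, and loops light flicker.
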(event `PeekIn`
  (`/Engine/EditorBlueprintResources/StandardMacros.DoOnce` false
    (:`Completed`
      (`SkeletalMeshComponent.PlayAnimation` (`self.Freddy`) "/Game/Core/Assets/Characters/Freddy/Animations/FreddyLeanIn.FreddyLeanIn" false))))

(event `StartShow`
  (set `self.IsActive` true)
  (`|ExecutionSequence`
    (:`then_0`
      (`/Engine/EditorBlueprintResources/StandardMacros.DoOnce` false
        (:`Completed`
          (bind _returnvalue (`GameplayStatics.SpawnSoundAtLocation` "/Game/Core/Assets/Sounds/Toreador_Cover_Cue.Toreador_Cover_Cue" (`self.K2_GetActorLocation`) (struct) 1.0 1.0 0.0 "/Game/Core/Assets/Sounds/NewSoundAttenuation.NewSoundAttenuation" null)))))
    (:`then_1`
      (if (`self.IsActive`) :!label _label
        (`KismetSystemLibrary.Delay` (`KismetMathLibrary.RandomFloatInRange` 0.02 0.2))
        (`LightComponent.SetIntensity` (`self.PointLight`) (`KismetMathLibrary.RandomFloatInRange` 0.0 2.0))
        (`LightComponent.SetIntensity` (`self.PointLight1`) (`KismetMathLibrary.RandomFloatInRange` 0.0 2.0))
        (goto _label)))))

(event `EndShow`
  (set `self.IsActive` false)
  (`KismetSystemLibrary.Delay` 0.3)
  (`LightComponent.SetIntensity` (`self.PointLight`) 0.0)
  (`LightComponent.SetIntensity` (`self.PointLight1`) 0.0)
  (`AudioComponent.Stop` (stale `StartShow` _returnvalue))
  (`ActorComponent.K2_DestroyComponent` (stale `StartShow` _returnvalue))
  (`KismetSystemLibrary.Delay` (`KismetMathLibrary.RandomFloatInRange` 3.0 7.0))
  (`self.JumpscareReady`))

(event `Jumpscare`
  (`/Engine/EditorBlueprintResources/StandardMacros.DoOnce` false
    (:`Completed`
      (`GameplayStatics.PlaySound2D` "/Game/Core/Player/XSCREAM.XSCREAM" 1.0 1.0 0.0 null null)
      (`self.K2_TeleportTo` (-226.510587 -411.661766 0.6) (struct))
      (`SkeletalMeshComponent.PlayAnimation` (`self.Freddy`) "/Game/Core/Assets/Characters/Freddy/Animations/FreddyJUMPSCARTE.FreddyJUMPSCARTE" false)
      (`SkeletalMeshComponent.PlayAnimation` (`self.Cube`) "/Game/Core/Assets/Characters/Freddy/Animations/FreddyPowerOutJumpscareBOX_Anim_Cube_CameraAction.FreddyPowerOutJumpscareBOX_Anim_Cube_CameraAction" false)
      ;[1 1 1] Lights
      (`KismetSystemLibrary.Delay` 0.05 :!label _label_2)
      (`LightComponent.SetIntensity` (`self.PointLight`) (`KismetMathLibrary.RandomFloatInRange` 0.1 2.0))
      (`LightComponent.SetIntensity` (`self.PointLight1`) (`KismetMathLibrary.RandomFloatInRange` 0.1 2.0))
      (`|ExecutionSequence`
        (:`then_0`
          (goto _label_2))
        (:`then_1`
          (`KismetSystemLibrary.Delay` 0.05 :!label _label_3)
          (`LightComponent.SetIntensity` (`self.SpotLight`) (`KismetMathLibrary.RandomFloatInRange` 0.0 5000.0))
          (goto _label_3))))))

(fn `UserConstructionScript`)