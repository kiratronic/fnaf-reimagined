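; Roaming animatronic enemy (foxyroam) that wanders the level, chases the player on sight and delivers a jumpscare.
; After a startup delay it loops AI moves to random reachable points until PawnSensing spots BP_PlayerFPS, which raises its speed and starts a chase.
; Reaching the player shows the GFjumpscare widget, reduces player health and restarts roaming.
; A delayed PassiveMode call resumes wandering only if the spotted flag has cleared.
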(event `Key|Q`
  (params (Key :type "Key Structure")))

(event `tick`
  (set `self.PlayerSpotted` false)
  (`|AIMoveTo` self (`NavigationSystemV1.K2_GetRandomReachablePointInRadius` (`self.K2_GetActorLocation`) 5000.0 null null) null :!label _label
    (:`OnSuccess`
      (`|ExecutionSequence`
        (:`then_0`
          (`KismetSystemLibrary.Delay` 2.0 :!label _label_2)
          (if (not (`self.PlayerSpotted`)) :!label _label_3
            (goto _label)))
        (:`then_1`
          (`KismetSystemLibrary.Delay` 2.0)
          (`TypedElementListLibrary.Reset` (struct)))))
    (:`OnFail`
      (goto _label_2))))

(event `Passive Mode`
  (goto _label_3))

(event `self.ReceiveBeginPlay`
  (`KismetSystemLibrary.Delay` 5.0)
  (goto _label))

(event `reset`
  (`/Engine/EditorBlueprintResources/StandardMacros.DoOnce` false :!via `Reset`))

(event `self.PawnSensing.OnSeePawn`
  (params (Pawn :type "Pawn Object Reference"))
  (bind _asbp_player_fps (cast `/Game/Core/Player/FPS/BP_PlayerFPS` Pawn)
    (:`then`
      (`/Engine/EditorBlueprintResources/StandardMacros.IsValid` _asbp_player_fps
        (:`Is Valid`
          (set `self.PlayerSpotted` true)
          (set `CharacterMovementComponent.MaxWalkSpeed` 450.0 (`self.CharacterMovement`))
          (`|AIMoveTo` self (0.0 0.0 0.0) _asbp_player_fps
            (:`then`
              (`KismetSystemLibrary.Delay` 10.0)
              (`self.Passive Mode`))
            (:`OnSuccess`
              (`KismetSystemLibrary.PrintString` "SCARE")
              (`self.tick`)
              (bind _returnvalue (`|CreateWidget` "/Game/Core/Assets/ahscary/GFjumpscare.GFjumpscare_C"))
              (`UserWidget.AddToViewport` _returnvalue 0)
              (bind _outactors (`GameplayStatics.GetAllActorsOfClass` "/Game/Core/Player/FPS/BP_PlayerFPS.BP_PlayerFPS_C"))
              (bind _output (`|GetArrayItem` _outactors))
              (set `/Game/Core/Player/FPS/BP_PlayerFPS.Health` (`KismetMathLibrary.FClamp` (- (`/Game/Core/Player/FPS/BP_PlayerFPS.Health` _output) 0.25)) _output))))
        (:`Is Not Valid`
          (set `self.PlayerSpotted` false :!label _label_4)
          (set `CharacterMovementComponent.MaxWalkSpeed` 300.0 (`self.CharacterMovement`)))))
    (:`CastFailed`
      (goto _label_4))))

(fn `UserConstructionScript`)