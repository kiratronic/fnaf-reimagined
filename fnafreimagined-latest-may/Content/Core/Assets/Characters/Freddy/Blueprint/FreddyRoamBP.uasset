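; Roaming Freddy enemy character that wanders the level and chases the player on sight.
; After a start delay it loops AI moves to random reachable points, pausing between each.
; Pawn sensing a player sets PlayerSpotted, raises walk speed and starts a chase, with a placeholder "SCARE" print on arrival.
; A delayed PassiveMode call resumes roaming only if PlayerSpotted is false, which happens only when another pawn is sensed.
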(event `Passive Mode`
  (if (not (`self.PlayerSpotted`)) :!label _label
    (`|AIMoveTo` self (`NavigationSystemV1.K2_GetRandomReachablePointInRadius` (`self.K2_GetActorLocation`) 5000.0 null null) null :!label _label_2
      (:`OnSuccess`
        _)
      (:`OnFail`
        _))
    (`KismetSystemLibrary.Delay` 2.0)
    (goto _label)))

(event `self.ReceiveBeginPlay`
  (`KismetSystemLibrary.Delay` 5.0)
  (goto _label_2))

(event `self.PawnSensing.OnSeePawn`
  (params (Pawn :type "Pawn Object Reference"))
  (bind _asbp_player_fps (cast `/Game/Core/Player/FPS/BP_PlayerFPS` Pawn)
    (:`then`
      (`/Engine/EditorBlueprintResources/StandardMacros.IsValid` _asbp_player_fps
        (:`Is Valid`
          (set `self.PlayerSpotted` true)
          (set `CharacterMovementComponent.MaxWalkSpeed` 350.0 (`self.CharacterMovement`))
          (`|AIMoveTo` self (0.0 0.0 0.0) _asbp_player_fps
            (:`then`
              (`KismetSystemLibrary.Delay` 10.0)
              (`self.Passive Mode`))
            (:`OnSuccess`
              (`KismetSystemLibrary.PrintString` "SCARE"))))
        (:`Is Not Valid`
          (set `self.PlayerSpotted` false :!label _label_3)
          (set `CharacterMovementComponent.MaxWalkSpeed` 120.0 (`self.CharacterMovement`)))))
    (:`CastFailed`
      (goto _label_3))))

(fn `UserConstructionScript`)