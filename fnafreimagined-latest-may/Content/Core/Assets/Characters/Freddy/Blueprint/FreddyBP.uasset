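; Freddy animatronic AI for a Five Nights at Freddy's-style game, advancing from the stage through fixed rooms to the office's right door.
; Night sets difficulty and timing for a looping random roll that advances him by teleport, pose animation and sound.
; Active cameras stall him, as does Chica occupying his kitchen, hallway or corner destination.
; Tick polls the door sequence, which checks door, monitor and cameras before triggering the one-shot office jumpscare.
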(event `InOfficeLogic`
  ;[1 1 1] Scare
  (`/Engine/EditorBlueprintResources/StandardMacros.DoOnce` false
    (:`Completed`
      (`SceneComponent.SetWorldScale3D` (`self.SkeletalMesh`) (0.75 0.75 0.75))
      (`self.FreddyInOffice`)
      (`self.K2_TeleportTo` (-97.056076 33.566071 20.0))
      (`SkeletalMeshComponent.PlayAnimation` (`self.SkeletalMesh`) "/Game/Core/Assets/Characters/Freddy/Animations/freddywalk3_RIG_Freddy_ao_Action.freddywalk3_RIG_Freddy_ao_Action" false)
      (`KismetSystemLibrary.Delay` 1.75)
      (`SkeletalMeshComponent.Stop` (`self.SkeletalMesh`))
      (set `self.JumpscareNow` true)
      (`|ExecutionSequence`
        (:`then_0`
          (`SkeletalMeshComponent.PlayAnimation` (`self.SkeletalMesh`) "/Game/Core/Assets/Characters/Freddy/Animations/FreddyActualJumpscare3_RIG_Freddy_ao_Action_002.FreddyActualJumpscare3_RIG_Freddy_ao_Action_002" false))
        (:`then_1`
          (`SkeletalMeshComponent.PlayAnimation` (`self.CameraMount`) "/Game/Core/Assets/Characters/Freddy/Animations/FreddyActualJumpscare3CUBE_Anim_Cube_001_Action_001.FreddyActualJumpscare3CUBE_Anim_Cube_001_Action_001" false))))))

(event `Door Sequence`
  ;[1 1 1] Door Logic
  (if (`self.AtDoor`)
    (if (not (`self.RightDoorClosed`))
      (bind _asplayer_bp (cast `/Game/Core/Player/PlayerBP` (`GameplayStatics.GetPlayerCharacter` 0)))
      (if (`/Game/Core/Player/PlayerBP.MonitorUp` _asplayer_bp)
        (if (not (`self.CamerasActive`))
          (`KismetSystemLibrary.Delay` 5.5)
          (if (`self.RightDoorClosed`) :!label _label
            _
            (elif (not (`self.CamerasActive`))
              (set `self.InOffice` true)
              (`self.InOfficeLogic`)
              (`KismetSystemLibrary.PrintString` "InOffice"))))
        (else
          (`KismetSystemLibrary.Delay` 3.25)
          (goto _label))))))

(event `StageMove`
  ;[1 1 1] Teleport And Animation
  (`self.K2_TeleportTo` (2872.343018 0.0 90.0) (struct :`Yaw` 90.0) :!label _label_2)
  (`SkeletalMeshComponent.PlayAnimation` (`self.SkeletalMesh`) "/Game/Core/Assets/Characters/Freddy/Animations/FreddyStage.FreddyStage" true)
  (`SceneComponent.SetVisibility` (`self.GlowingLeftEye`) false false)
  (`SceneComponent.SetVisibility` (`self.GlowingLeftEye1`) false false))

(event `BeginCycle`
  ;[1 1 1] MovementChance
  (`KismetSystemLibrary.Delay` (`self.WaitTime`))
  (if (`self.CanMove`)
    (if (and (`self.InOffice`) (`self.HoldingPosition`))
      (`self.BeginCycle`)
      (elif (<= (`KismetMathLibrary.RandomIntegerInRange` 0 20) (`self.AIDifficulty`))
        (`self.CameraCheck`)
        (`KismetSystemLibrary.Delay` 1.0)
        (if (`self.CamerasActive`)
          (`self.BeginCycle`)
          (else
            (`self.MovementCycle`)))
        (else
          (`self.BeginCycle`))))
    (else
      (`self.BeginCycle`))))

(event `MoveTrigger`
  ;[1 1 1] Teleport And Animation
  (`GameplayStatics.PlaySoundAtLocation` "/Game/Core/Assets/Sounds/FreddyLaugh_Cue.FreddyLaugh_Cue" (`self.K2_GetActorLocation`) (struct) 1.0 1.0 0.0 null null null null)
  (`|ExecutionSequence`
    (:`then_0`
      (switch `string` (`self.ArrivalLocation`)
        (:`Default`
          (`self.BeginCycle`)
          (`KismetSystemLibrary.PrintString` (`self.ArrivalLocation`) true true (struct :`R` 0.650518 :`G` 1.0 :`A` 1.0)))
        (:`Stage`
          (goto _label_2))
        (:`DiningRoom`
          (`self.K2_TeleportTo` (1631.671143 238.461166 20.0) (struct :`Yaw` -105.0))
          (`SkeletalMeshComponent.PlayAnimation` (`self.SkeletalMesh`) "/Game/Core/Assets/Characters/Freddy/Animations/FreddyDining1.FreddyDining1" true)
          (`SceneComponent.SetVisibility` (`self.GlowingLeftEye`) true false)
          (`SceneComponent.SetVisibility` (`self.GlowingLeftEye1`) true false))
        (:`Bathroom`
          (`self.K2_TeleportTo` (2622.318359 1276.225098 -7.542852) (struct :`Pitch` -24.092936 :`Yaw` 206.470276 :`Roll` -6.881703))
          (`SkeletalMeshComponent.PlayAnimation` (`self.SkeletalMesh`) "/Game/Core/Assets/Characters/Freddy/Animations/FreddyBathrooms.FreddyBathrooms" true)
          (`SceneComponent.SetVisibility` (`self.GlowingLeftEye`) false false)
          (`SceneComponent.SetVisibility` (`self.GlowingLeftEye1`) false false))
        (:`Kitchen`
          (`self.K2_TeleportTo` (0.0 0.0 500.0))
          (`SkeletalMeshComponent.PlayAnimation` (`self.SkeletalMesh`) null true)
          (bind _returnvalue (`GameplayStatics.SpawnSoundAtLocation` "/Game/Core/Assets/Sounds/Toreador_Cover_Cue.Toreador_Cover_Cue" (942.42395 965.457825 129.266678) (struct) 0.5 1.0 (`KismetMathLibrary.RandomFloatInRange` 0.0 7.0) "/Game/Core/Assets/Sounds/NewSoundAttenuation.NewSoundAttenuation" null)))
        (:`Hallway`
          (`self.K2_TeleportTo` (775.276001 323.311249 20.0) (struct :`Yaw` 88.0))
          (`SkeletalMeshComponent.PlayAnimation` (`self.SkeletalMesh`) "/Game/Core/Assets/Characters/Freddy/Animations/FreddyHallway.FreddyHallway" true)
          (`AudioComponent.Stop` _returnvalue)
          (`ActorComponent.K2_DestroyComponent` _returnvalue))
        (:`RightCorner`
          (`self.K2_TeleportTo` (-318.143868 233.315278 131.282487) (struct :`Pitch` -7.398512 :`Yaw` -99.17024 :`Roll` -33.144232))
          (`SkeletalMeshComponent.PlayAnimation` (`self.SkeletalMesh`) "/Game/Core/Assets/Characters/Freddy/HallCorner.HallCorner" true))))
    (:`then_1`
      (if (`KismetStringLibrary.EqualEqual_StrStr` (`self.ArrivalLocation`) "RightCorner")
        (`self.Door Sequence`)
        (`self.BeginCycle`)
        (set `self.AtDoor` true)
        (else
          (`self.BeginCycle`)
          (set `self.AtDoor` false))))))

(event `self.ReceiveBeginPlay`
  (`self.StageMove`)
  (`KismetSystemLibrary.Delay` 2.0)
  (`self.Difficulty Define`))

(event `self.ReceiveTick`
  (params (DeltaSeconds :type "Float (single-precision)"))
  (`self.Door Sequence`))

(event `TryAgain`
  ;[1 1 1] Random Movement
  (switch `string` (`self.CurrentLocation`) :!label _label_3
    (:`Stage`
      (set `self.ArrivalLocation` "")
      (`self.DiningRoom`))
    (:`DiningRoom`
      (set `self.ArrivalLocation` "Bathroom")
      (`self.Bathroom`))
    (:`Bathroom`
      (set `self.ArrivalLocation` "Kitchen")
      (`self.Kitchen`))
    (:`Kitchen`
      (set `self.ArrivalLocation` "Hallway")
      (`self.RightHallway`))
    (:`Hallway`
      (set `self.ArrivalLocation` "RightCorner")
      (`self.RightCorner`))
    (:`RightCorner`
      (if (`self.RightDoorClosed`)
        (`self.DiningRoom`)
        (`self.FreddyFromDoor`)
        (else
          (set `self.InOffice` true)
          (`self.InOfficeLogic`))))))

(event `MovementCycle`
  ;[1 1 1] Random Movement
  (goto _label_3))

(event `Difficulty Define`
  ;[1 1 1] Difficulty
  (switch `string` (`self.Night`)
    (:`NightTemplate`
      (set `self.AIDifficulty` 10)
      (set `self.WaitTime` (`KismetMathLibrary.RandomFloatInRange` 6.0 10.0))
      (`KismetSystemLibrary.Delay` 0.0)
      (set `self.CanMove` true)
      (`self.BeginCycle`))
    (:`Night1`
      (set `self.AIDifficulty` 20)
      (set `self.WaitTime` 4.0)
      (`KismetSystemLibrary.Delay` 0.0)
      (set `self.CanMove` false)
      (`self.BeginCycle`))
    (:`Night2`
      (set `self.AIDifficulty` 5)
      (set `self.WaitTime` (`KismetMathLibrary.RandomFloatInRange` 15.0 25.0))
      (`KismetSystemLibrary.Delay` 60.0)
      (set `self.CanMove` false)
      (`self.BeginCycle`))
    (:`Night3`
      (set `self.AIDifficulty` 5)
      (set `self.WaitTime` (`KismetMathLibrary.RandomFloatInRange` 15.0 25.0))
      (`KismetSystemLibrary.Delay` 60.0)
      (set `self.CanMove` true)
      (`self.BeginCycle`))
    (:`Night4`
      (set `self.AIDifficulty` 8)
      (set `self.WaitTime` (`KismetMathLibrary.RandomFloatInRange` 15.0 25.0))
      (`KismetSystemLibrary.Delay` 60.0)
      (set `self.CanMove` true)
      (`self.BeginCycle`))
    (:`Night5`
      (set `self.AIDifficulty` 13 :!label _label_4)
      (set `self.WaitTime` (`KismetMathLibrary.RandomFloatInRange` 15.0 25.0))
      (`KismetSystemLibrary.Delay` 60.0)
      (set `self.CanMove` true)
      (`self.BeginCycle`))
    (:`Night6`
      (goto _label_4))))

(event `DiningRoom`
  ;[1 1 1] Movement Action
  (`self.CameraCheck`)
  (`KismetSystemLibrary.Delay` 1.0)
  (if (`self.CamerasActive`)
    (`self.BeginCycle` :!label _label_5)
    (elif (`self.HoldingPosition`)
      (goto _label_5)
      (else
        (bind _output_get (set `self.ArrivalLocation` "DiningRoom"))
        (set `self.CurrentLocation` _output_get)
        (`self.MoveTrigger`)))))

(event `Bathroom`
  ;[1 1 1] Movement Action
  (`self.CameraCheck`)
  (`KismetSystemLibrary.Delay` 1.0)
  (if (`self.CamerasActive`)
    (`self.BeginCycle` :!label _label_6)
    (elif (`self.HoldingPosition`)
      (goto _label_6)
      (else
        (bind _output_get (set `self.ArrivalLocation` "Bathroom"))
        (set `self.CurrentLocation` _output_get)
        (`self.MoveTrigger`)))))

(event `Kitchen`
  ;[1 1 1] Movement Action
  (`self.CameraCheck`)
  (`KismetSystemLibrary.Delay` 1.0)
  (if (`self.CamerasActive`)
    (`self.BeginCycle` :!label _label_7)
    (else
      (bind _returnvalue (`GameplayStatics.GetActorOfClass` "/Game/Core/Assets/Characters/Chica/Blueprint/ChicaBP.ChicaBP_C"))
      (if (`KismetStringLibrary.EqualEqual_StrStr` (`/Game/Core/Assets/Characters/Chica/Blueprint/ChicaBP.CurrentLocation` _returnvalue) "Kitchen")
        (set `self.HoldingPosition` true)
        (elif (`self.CamerasActive`)
          (goto _label_7)
          (else
            (set `self.HoldingPosition` false))))
      (if (`self.HoldingPosition`)
        (goto _label_7)
        (else
          (bind _output_get (set `self.ArrivalLocation` "Kitchen"))
          (set `self.CurrentLocation` _output_get)
          (`self.MoveTrigger`))))))

(event `RightHallway`
  ;[1 1 1] Movement Action
  (`self.CameraCheck`)
  (`KismetSystemLibrary.Delay` 1.0)
  (if (`self.CamerasActive`)
    (`self.BeginCycle` :!label _label_8)
    (else
      (bind _returnvalue (`GameplayStatics.GetActorOfClass` "/Game/Core/Assets/Characters/Chica/Blueprint/ChicaBP.ChicaBP_C"))
      (if (`KismetStringLibrary.EqualEqual_StrStr` (`/Game/Core/Assets/Characters/Chica/Blueprint/ChicaBP.CurrentLocation` _returnvalue) "RightHallway1")
        (set `self.HoldingPosition` true)
        (elif (`self.CamerasActive`)
          (goto _label_8)
          (else
            (set `self.HoldingPosition` false))))
      (if (`self.HoldingPosition`)
        (goto _label_8)
        (else
          (bind _output_get (set `self.ArrivalLocation` "Hallway"))
          (set `self.CurrentLocation` _output_get)
          (`self.MoveTrigger`))))))

(event `RightCorner`
  ;[1 1 1] Movement Action
  (`self.CameraCheck`)
  (`KismetSystemLibrary.Delay` 1.0)
  (if (`self.CamerasActive`)
    (`self.BeginCycle` :!label _label_9)
    (else
      (bind _returnvalue (`GameplayStatics.GetActorOfClass` "/Game/Core/Assets/Characters/Chica/Blueprint/ChicaBP.ChicaBP_C"))
      (if (`KismetStringLibrary.EqualEqual_StrStr` (`/Game/Core/Assets/Characters/Chica/Blueprint/ChicaBP.CurrentLocation` _returnvalue) "RightCorner")
        (set `self.HoldingPosition` true)
        (elif (`self.CamerasActive`)
          (goto _label_9)
          (else
            (set `self.HoldingPosition` false))))
      (if (`self.HoldingPosition`)
        (goto _label_9)
        (else
          (bind _output_get (set `self.ArrivalLocation` "RightCorner"))
          (set `self.CurrentLocation` _output_get)
          (`self.MoveTrigger`)
          (set `self.AtDoor` true))))))

(event `StageSpookMoment`
  (if (`KismetStringLibrary.EqualEqual_StrStr` (`self.CurrentLocation`) "Stage")
    (`SkeletalMeshComponent.PlayAnimation` (`self.SkeletalMesh`) "/Game/Core/Assets/Characters/Freddy/Animations/FreddyStageSpook.FreddyStageSpook" true)))

(event `StageSpookOff`
  (if (`KismetStringLibrary.EqualEqual_StrStr` (`self.CurrentLocation`) "Stage")
    (`SkeletalMeshComponent.PlayAnimation` (`self.SkeletalMesh`) "/Game/Core/Assets/Characters/Freddy/Animations/FreddyStage.FreddyStage" true)))

(fn `UserConstructionScript`)