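; Chica animatronic AI for a FNAF-style night game, roaming from the stage toward the right office door and jumpscare.
; Night number sets difficulty, wait time and start delay; a timed loop rolls against difficulty to pick the next room.
; Each move checks holding, sometimes set by Freddy's location, then teleports with pose and camera blur.
; Tick checks the door for office entry; high difficulty adds twitching, whispering poses at the corner.
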(event `Door Sequence`
  ;[1 1 1] Door Logic
  (if (`self.AtDoor`)
    (if (`self.RightDoorClosed`)
      (`KismetSystemLibrary.Delay` 0.05)
      (if (not (`self.RightDoorClosed`))
        (`KismetSystemLibrary.Delay` 1.0)
        (if (not (`self.RightDoorClosed`)) :!label _label
          (set `self.InOffice` true)
          (`self.InOfficeLogic`)
          (`KismetSystemLibrary.PrintString` "InOffice")))
      (elif (`self.LightOn`)
        (`KismetSystemLibrary.Delay` 3.0)
        (goto _label)))))

(event `SpookyChicaEnd`
  ;[1 1 1] Creepy Stuff
  (`AudioComponent.Stop` (`self.DemonWhisper`))
  (set `self.SpookyMode` false))

(event `SpookyChica`
  ;[1 1 1] Creepy Stuff
  (if (`self.SpookyMode`)
    (`|ExecutionSequence`
      (:`then_0`
        (`/Engine/EditorBlueprintResources/StandardMacros.DoOnce` false :!label _label_2
          (:`Completed`
            (`AudioComponent.Play` (`self.DemonWhisper`) 0.0)
            (`KismetSystemLibrary.Delay` 15.0)
            (if (`self.SpookyMode`)
              (goto _label_2 :!via `Reset`)
              (else
                (`AudioComponent.Stop` (`self.DemonWhisper`))
                (goto _label_2 :!via `Reset`))))))
      (:`then_1`
        (`self.Creepy Poses`)))))

(event `BeginCycle`
  ;[1 1 1] Movement Chance
  (`KismetSystemLibrary.Delay` (`self.WaitTime`))
  (if (`self.CanMove`)
    (if (and (`self.InOffice`) (`self.HoldingPosition`))
      (`self.BeginCycle`)
      (elif (<= (`KismetMathLibrary.RandomIntegerInRange` 0 20) (`self.AIDifficulty`))
        (`self.MovementCycle`)
        (else
          (`self.BeginCycle`))))
    (else
      (`self.BeginCycle`))))

(event `Creepy Poses`
  (if (`self.SpookyMode`)
    (`KismetSystemLibrary.Delay` (`KismetMathLibrary.RandomFloatInRange` 0.0 0.1))
    (switch `int` (`KismetMathLibrary.RandomIntegerInRange` 0 2)
      (:`0`
        (`SkeletalMeshComponent.PlayAnimation` (`self.SkeletalMesh`) "/Game/Core/Assets/Characters/Chica/Animations/ANIM_RightHallCorner.ANIM_RightHallCorner" true))
      (:`1`
        (`SkeletalMeshComponent.PlayAnimation` (`self.SkeletalMesh`) "/Game/Core/Assets/Characters/Chica/Animations/ChicaCorner.ChicaCorner" true))
      (:`2`
        (`SkeletalMeshComponent.PlayAnimation` (`self.SkeletalMesh`) "/Game/Core/Assets/Characters/Chica/Animations/ChicaCorner02.ChicaCorner02" true)))
    (`self.Creepy Poses`)))

(event `StageMove`
  ;[1 1 1] Teleport And Animation
  (`self.K2_TeleportTo` (2978.659946 -87.0 90.0) (struct :`Yaw` 104.400002) :!label _label_3)
  (`SkeletalMeshComponent.PlayAnimation` (`self.SkeletalMesh`) "/Game/Core/Assets/Characters/Chica/Animations/chica_pose.chica_pose" true))

(event `InOfficeLogic`
  (bind _skeletalmesh (`self.SkeletalMesh`))
  (`self.ChicaInOffice`)
  (`self.K2_TeleportTo` (-357.035309 -10.0 500.0) (struct :`Yaw` -90.0))
  (`SkeletalMeshComponent.PlayAnimation` _skeletalmesh "/Game/Core/Assets/Characters/Chica/Animations/ChicaPreJumpscare.ChicaPreJumpscare" true)
  (`PrimitiveComponent.SetMaterial` _skeletalmesh 1 "/Game/Core/Assets/Characters/Shared/Material/EmmissiveEye_MI.EmmissiveEye_MI")
  (`KismetSystemLibrary.PrintString` "InOffice"))

(event `self.ReceiveBeginPlay`
  (`self.StageMove`)
  (`KismetSystemLibrary.Delay` 2.0)
  (`self.Difficulty Define`))

(event `self.ReceiveTick`
  (params (DeltaSeconds :type "Float (single-precision)"))
  (`self.Door Sequence`))

(event `Jumpscare`
  (`self.ChicaJumpscare`)
  (`SkeletalMeshComponent.PlayAnimation` (`self.SkeletalMesh`) "/Game/Core/Assets/Characters/Chica/Animations/chica_jumpscare_1.chica_jumpscare_1" true)
  (`SceneComponent.SetVisibility` (`self.PointLight`) true false))

(event `MoveTrigger`
  (bind _arrivallocation (`self.ArrivalLocation`))
  ;[1 1 1] Teleport And Animation
  (`|ExecutionSequence`
    (:`then_0`
      (if (not (`KismetStringLibrary.EqualEqual_StrStr` "RightCorner" _arrivallocation))
        (`self.SpookyChicaEnd`)
        (`KismetSystemLibrary.Delay` 0.4))
      (switch `string` _arrivallocation
        (:`Stage`
          (goto _label_3))
        (:`Dining1`
          (`self.K2_TeleportTo` (1898.229505 210.247903 41.050667) (struct :`Yaw` -170.0))
          (`SkeletalMeshComponent.PlayAnimation` (`self.SkeletalMesh`) "/Game/Core/Assets/Characters/Chica/Animations/ChicaDining2.ChicaDining2" true))
        (:`Dining2`
          (`self.K2_TeleportTo` (2578.454984 149.550051 76.62842) (struct :`Pitch` 344.425789 :`Yaw` 201.612855 :`Roll` 14.035497))
          (`SkeletalMeshComponent.PlayAnimation` (`self.SkeletalMesh`) "/Game/Core/Assets/Characters/Chica/Animations/ChicaDining2.ChicaDining2" true))
        (:`Bathroom1`
          (`self.K2_TeleportTo` (2158.252441 1008.845764 74.631096) (struct :`Yaw` -85.0))
          (`SkeletalMeshComponent.PlayAnimation` (`self.SkeletalMesh`) "/Game/Core/Assets/Characters/Chica/Animations/ChicaBathroom1v2.ChicaBathroom1v2" true))
        (:`Bathroom2`
          (`self.K2_TeleportTo` (2628.255165 978.24276 93.220834) (struct :`Pitch` -5.078546 :`Yaw` -104.132723 :`Roll` -19.370055))
          (`SkeletalMeshComponent.PlayAnimation` (`self.SkeletalMesh`) "/Game/Core/Assets/Characters/Chica/Animations/ChicaBathroom1v2.ChicaBathroom1v2" true))
        (:`Kitchen`
          (`self.K2_TeleportTo` (0.0 0.0 500.0))
          (`SkeletalMeshComponent.PlayAnimation` (`self.SkeletalMesh`) null true)
          (bind _returnvalue (`GameplayStatics.SpawnSoundAtLocation` "/Game/Core/Assets/Sounds/ChicaKitchen_Cue.ChicaKitchen_Cue" (942.42395 965.457825 129.266678) (struct) 0.25 1.0 0.0 "/Game/Core/Assets/Sounds/NewSoundAttenuation.NewSoundAttenuation" null false :!label _label_4))
          (`KismetSystemLibrary.Delay` 8.0)
          (if (`KismetStringLibrary.EqualEqual_StrStr` (`self.CurrentLocation`) "Kitchen")
            (`ActorComponent.K2_DestroyComponent` _returnvalue)
            (goto _label_4)
            (else
              (`ActorComponent.K2_DestroyComponent` _returnvalue))))
        (:`RightHallway1`
          (`self.K2_TeleportTo` (782.735107 314.217865 20.0) (struct :`Yaw` 90.0))
          (`SkeletalMeshComponent.PlayAnimation` (`self.SkeletalMesh`) "/Game/Core/Assets/Characters/Chica/Animations/ChicaHallway1.ChicaHallway1" true))
        (:`RightHallway2`
          (`self.K2_TeleportTo` (229.623734 353.649516 38.062604) (struct :`Pitch` 12.183114 :`Yaw` 87.092759 :`Roll` -2.230779))
          (`SkeletalMeshComponent.PlayAnimation` (`self.SkeletalMesh`) "/Game/Core/Assets/Characters/Chica/Animations/ChicaHallway2.ChicaHallway2" true))
        (:`RightCorner`
          (`self.K2_TeleportTo` (-487.881125 230.498539 93.786293) (struct :`Yaw` -53.391406))
          (`SkeletalMeshComponent.PlayAnimation` (`self.SkeletalMesh`) "/Game/Core/Assets/Characters/Chica/Animations/ChicaCorner02.ChicaCorner02" true)
          (if (>= (`self.AIDifficulty`) 14)
            (set `self.SpookyMode` true)
            (`self.SpookyChica`)
            (else
              (`self.SpookyChicaEnd`))))
        (:`RightDoor`
          (`self.K2_TeleportTo` (-48.774742 222.027725 20.0) (struct :`Yaw` -207.244293))
          (`SkeletalMeshComponent.PlayAnimation` (`self.SkeletalMesh`) "/Game/Core/Assets/Characters/Chica/Animations/ChicaAtDoor.ChicaAtDoor" true))))
    (:`then_1`
      (if (`KismetStringLibrary.EqualEqual_StrStr` (`self.ArrivalLocation`) "LeftDoor")
        (`self.Door Sequence`)
        (`self.BeginCycle`)
        (else
          (`self.BeginCycle`)
          (set `self.AtDoor` false))))))

(event `JumpscareCall`
  (`SkeletalMeshComponent.PlayAnimation` (`self.SkeletalMesh`) "/Game/Core/Assets/Characters/Chica/Animations/chica_jumpscare_1.chica_jumpscare_1" true)
  (`SceneComponent.SetVisibility` (`self.PointLight`) true false))

(event `TryAgain`
  (bind _returnvalue (`KismetMathLibrary.RandomIntegerInRange` 0 3))
  (bind _returnvalue_2 (!= _returnvalue (`self.RNGMove`)))
  ;[1 1 1] Random Movement
  (switch `string` (`self.CurrentLocation`) :!label _label_5
    (:`Stage`
      (switch `int` _returnvalue :!label _label_6
        (:`0`
          (if _returnvalue_2
            (`self.Bathroom1`)
            (set `self.RNGMove` 0)
            (else
              (`KismetSystemLibrary.PrintString` "ChicaTryAgain" true true (struct :`R` 1.0 :`G` 0.133929 :`A` 1.0) :!label _label_7)
              (goto _label_6))))
        (:`1`
          (if _returnvalue_2
            (`self.Dining1`)
            (set `self.RNGMove` 1)
            (else
              (goto _label_7))))
        (:`2`
          (if _returnvalue_2
            (`self.Bathroom2`)
            (set `self.RNGMove` 2)
            (else
              (goto _label_7))))
        (:`3`
          (if _returnvalue_2
            (`self.Dining2`)
            (set `self.RNGMove` 3)
            (else
              (goto _label_7))))))
    (:`Dining1`
      (if (`KismetMathLibrary.RandomBool`)
        (goto _label_6)
        (elif (> (`KismetMathLibrary.RandomIntegerInRange` 0 20) (`self.AIDifficulty`))
          (`self.Dining2`)
          (else
            (`self.Bathroom1`)))))
    (:`Dining2`
      (if (> (`KismetMathLibrary.RandomIntegerInRange` 0 20) (`self.AIDifficulty`))
        (goto _label_6)
        (elif (`KismetMathLibrary.RandomBool`)
          (`self.Kitchen`)
          (else
            (`self.RightHallway1`)))))
    (:`Bathroom1`
      (if (> (`KismetMathLibrary.RandomIntegerInRange` 0 20) (`self.AIDifficulty`))
        (goto _label_6)
        (elif (`KismetMathLibrary.RandomBool`)
          (`self.Bathroom2`)
          (else
            (`self.Dining2`)))))
    (:`Bathroom2`
      (if (`KismetMathLibrary.RandomBool`)
        (`self.Kitchen`)
        (else
          (`self.Dining2`))))
    (:`Kitchen`
      (if (> (`KismetMathLibrary.RandomIntegerInRange` 0 20) (`self.AIDifficulty`))
        (`self.Dining2`)
        (elif (`KismetMathLibrary.RandomBool`)
          (`self.RightHallway1`)
          (else
            (`self.RightHallway2`)))))
    (:`RightHallway1`
      (if (> (`KismetMathLibrary.RandomIntegerInRange` 0 20) (`self.AIDifficulty`))
        (`self.Dining2`)
        (elif (`KismetMathLibrary.RandomBool`)
          (`self.RightHallway2`)
          (else
            (`self.RightCorner`)))))
    (:`RightHallway2`
      (if (> (`KismetMathLibrary.RandomIntegerInRange` 0 20) (`self.AIDifficulty`))
        (`self.Kitchen`)
        (else
          (`self.RightCorner`))))
    (:`RightCorner`
      (if (> (`KismetMathLibrary.RandomIntegerInRange` 0 20) (`self.AIDifficulty`))
        (`self.RightHallway1`)
        (else
          (`self.RightDoor`))))
    (:`RightDoor`
      (if (`self.RightDoorClosed`)
        (if (`KismetMathLibrary.RandomBool`)
          (`self.Dining1`)
          (elif (`KismetMathLibrary.RandomBool`)
            (`self.Dining2`)
            (else
              (`self.RightHallway2`))))
        (`self.ChicaFromDoor`)
        (else
          (set `self.InOffice` true)
          (`self.InOfficeLogic`))))))

(event `MovementCycle`
  ;[1 1 1] Random Movement
  (goto _label_5))

(event `Dining1`
  ;[1 1 1] MovementAction
  (if (`self.HoldingPosition`)
    (`self.BeginCycle`)
    (else
      (bind _output_get (set `self.ArrivalLocation` "Dining1"))
      (`self.CameraBlur`)
      (set `self.CurrentLocation` _output_get)
      (`self.MoveTrigger`))))

(event `Difficulty Define`
  ;[1 1 1] Difficulty
  (switch `string` (`self.Night`)
    (:`Night1`
      (set `self.AIDifficulty` (`KismetMathLibrary.RandomIntegerInRange` 4 6))
      (set `self.WaitTime` (`KismetMathLibrary.RandomFloatInRange` 9.0 12.0))
      (`KismetSystemLibrary.Delay` 60.0)
      (set `self.CanMove` true)
      (`self.BeginCycle`))
    (:`Night2`
      (set `self.AIDifficulty` 8)
      (set `self.WaitTime` (`KismetMathLibrary.RandomFloatInRange` 15.0 25.0))
      (`KismetSystemLibrary.Delay` 30.0)
      (set `self.CanMove` true)
      (`self.BeginCycle`))
    (:`Night3`
      (set `self.AIDifficulty` 9)
      (set `self.WaitTime` (`KismetMathLibrary.RandomFloatInRange` 15.0 25.0))
      (`KismetSystemLibrary.Delay` 20.0)
      (set `self.CanMove` true)
      (`self.BeginCycle`))
    (:`Night4`
      (set `self.AIDifficulty` 10)
      (set `self.WaitTime` (`KismetMathLibrary.RandomFloatInRange` 15.0 25.0))
      (`KismetSystemLibrary.Delay` 10.0)
      (set `self.CanMove` true)
      (`self.BeginCycle`))
    (:`Night5`
      (set `self.AIDifficulty` 13)
      (set `self.WaitTime` (`KismetMathLibrary.RandomFloatInRange` 15.0 25.0))
      (`KismetSystemLibrary.Delay` 8.0)
      (set `self.CanMove` true)
      (`self.BeginCycle`))
    (:`Night6`
      (set `self.AIDifficulty` 20 :!label _label_8)
      (set `self.WaitTime` (`KismetMathLibrary.RandomFloatInRange` 7.0 11.0))
      (`KismetSystemLibrary.Delay` 5.0)
      (set `self.CanMove` true)
      (`self.BeginCycle`))
    (:`CustomNight`
      (goto _label_8))))

(event `Dining2`
  ;[1 1 1] MovementAction
  (if (`self.HoldingPosition`)
    (`self.BeginCycle`)
    (else
      (bind _output_get (set `self.ArrivalLocation` "Dining2"))
      (`self.CameraBlur`)
      (set `self.CurrentLocation` _output_get)
      (`self.MoveTrigger`))))

(event `Bathroom1`
  ;[1 1 1] MovementAction
  (if (`self.HoldingPosition`)
    (`self.BeginCycle`)
    (else
      (bind _output_get (set `self.ArrivalLocation` "Bathroom1"))
      (`self.CameraBlur`)
      (set `self.CurrentLocation` _output_get)
      (`self.MoveTrigger`))))

(event `Bathroom2`
  ;[1 1 1] MovementAction
  (if (`self.HoldingPosition`)
    (`self.BeginCycle`)
    (else
      (bind _output_get (set `self.ArrivalLocation` "Bathroom2"))
      (`self.CameraBlur`)
      (set `self.CurrentLocation` _output_get)
      (`self.MoveTrigger`))))

(event `Kitchen`
  ;[1 1 1] MovementAction
  (bind _returnvalue (`GameplayStatics.GetActorOfClass` "/Game/Core/Assets/Characters/Freddy/Blueprint/FreddyBP.FreddyBP_C"))
  (if (`KismetStringLibrary.EqualEqual_StrStr` (`/Game/Core/Assets/Characters/Freddy/Blueprint/FreddyBP.CurrentLocation` _returnvalue) "Kitchen")
    (set `self.HoldingPosition` true)
    (else
      (set `self.HoldingPosition` false)))
  (if (`self.HoldingPosition`)
    (`self.BeginCycle`)
    (else
      (bind _output_get (set `self.ArrivalLocation` "Kitchen"))
      (`self.CameraBlur`)
      (set `self.CurrentLocation` _output_get)
      (`self.MoveTrigger`))))

(event `RightHallway1`
  ;[1 1 1] MovementAction
  (bind _returnvalue (`GameplayStatics.GetActorOfClass` "/Game/Core/Assets/Characters/Freddy/Blueprint/FreddyBP.FreddyBP_C"))
  (if (`KismetStringLibrary.EqualEqual_StrStr` (`/Game/Core/Assets/Characters/Freddy/Blueprint/FreddyBP.CurrentLocation` _returnvalue) "Hallway")
    (set `self.HoldingPosition` true)
    (else
      (set `self.HoldingPosition` false)))
  (if (`self.HoldingPosition`)
    (`self.BeginCycle`)
    (else
      (bind _output_get (set `self.ArrivalLocation` "RightHallway1"))
      (`self.CameraBlur`)
      (set `self.CurrentLocation` _output_get)
      (`self.MoveTrigger`))))

(event `RightHallway2`
  ;[1 1 1] MovementAction
  (if (`self.HoldingPosition`)
    (`self.BeginCycle`)
    (else
      (bind _output_get (set `self.ArrivalLocation` "RightHallway2"))
      (`self.CameraBlur`)
      (set `self.CurrentLocation` _output_get)
      (`self.MoveTrigger`))))

(event `RightCorner`
  ;[1 1 1] MovementAction
  (bind _returnvalue (`GameplayStatics.GetActorOfClass` "/Game/Core/Assets/Characters/Freddy/Blueprint/FreddyBP.FreddyBP_C"))
  (if (`KismetStringLibrary.EqualEqual_StrStr` (`/Game/Core/Assets/Characters/Freddy/Blueprint/FreddyBP.CurrentLocation` _returnvalue) "RightCorner")
    (set `self.HoldingPosition` true)
    (else
      (set `self.HoldingPosition` false)))
  (if (`self.HoldingPosition`)
    (`self.BeginCycle`)
    (else
      (bind _output_get (set `self.ArrivalLocation` "RightCorner"))
      (`self.CameraBlur`)
      (set `self.CurrentLocation` _output_get)
      (`self.MoveTrigger`))))

(event `RightDoor`
  ;[1 1 1] MovementAction
  (bind _returnvalue (`GameplayStatics.GetActorOfClass` "/Game/Core/Assets/Characters/Freddy/Blueprint/FreddyBP.FreddyBP_C"))
  (if (`KismetStringLibrary.EqualEqual_StrStr` (`/Game/Core/Assets/Characters/Freddy/Blueprint/FreddyBP.CurrentLocation` _returnvalue) "Corner")
    (set `self.HoldingPosition` true)
    (else
      (set `self.HoldingPosition` false)))
  (if (`self.HoldingPosition`)
    (`self.BeginCycle`)
    (else
      (`self.ChicaToDoor`)
      (bind _output_get (set `self.ArrivalLocation` "RightDoor"))
      (`self.CameraBlur`)
      (set `self.CurrentLocation` _output_get)
      (`self.MoveTrigger`)
      (set `self.AtDoor` true))))

(event `StageSpookMoment`
  (if (`KismetStringLibrary.EqualEqual_StrStr` (`self.CurrentLocation`) "Stage")
    (`SkeletalMeshComponent.PlayAnimation` (`self.SkeletalMesh`) "/Game/Core/Assets/Characters/Chica/Animations/ChicaStageScare.ChicaStageScare" true)))

(event `StageSpookOff`
  (if (`KismetStringLibrary.EqualEqual_StrStr` (`self.CurrentLocation`) "Stage")
    (`SkeletalMeshComponent.PlayAnimation` (`self.SkeletalMesh`) "/Game/Core/Assets/Characters/Chica/Animations/chica_pose.chica_pose" true)))

(fn `UserConstructionScript`)