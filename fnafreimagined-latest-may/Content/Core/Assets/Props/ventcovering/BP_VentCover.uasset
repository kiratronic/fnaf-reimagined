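; BP_VentCover is a vent cover prop that can fall and makes banging noises when hit.
; DropVent turns on physics simulation for the VentPrimary component so the cover drops.
; Hit plays the VentBangs sound at the impact location, using a DoOnce reset after a 0.9 second delay to space out bangs and a NoiseCount check to stop them after two.
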(event `DropVent`
  (`PrimitiveComponent.SetSimulatePhysics` (`self.VentPrimary`) true))

(event `self.ReceiveHit`
  (params (MyComp :type "PrimitiveComponent Object Reference") (Other :type "Actor Object Reference") (OtherComp :type "PrimitiveComponent Object Reference") (bSelfMoved :type Boolean) (HitLocation :type "Vector Structure") (HitNormal :type "Vector Structure") (NormalImpulse :type "Vector Structure") (Hit :type "HitResult Structure (by ref)"))
  (if (not (== (`self.Noise Count`) 2))
    (`/Engine/EditorBlueprintResources/StandardMacros.DoOnce` false :!label _label
      (:`Completed`
        (set `self.Noise Count` (+ (`self.Noise Count`) 1))
        (`GameplayStatics.PlaySoundAtLocation` "/Game/Core/Assets/Sounds/VentBangs.VentBangs" HitLocation (struct) 1.0 1.0 0.0 null null null null)
        (`KismetSystemLibrary.Delay` 0.9)
        (goto _label :!via `Reset`)))))

(fn `UserConstructionScript`)