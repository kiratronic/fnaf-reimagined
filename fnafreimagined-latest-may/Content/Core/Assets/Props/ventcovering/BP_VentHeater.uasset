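; BP_VentHeater is a vent heater prop that fades a point light on and off through its VentOn and VentOff events.
; A Light timeline drives the light intensity, playing forward for on and reversing for off.
; Both paths look up BP_Usage and write its Usage value back unchanged, as the -1 adjustment nodes are left unconnected.
; That lookup repeats on every timeline update.
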(event `VentOn`
  (bind (_direction _intensity) (`Timeline|Light` :!label _label)
    (:`Update`
      (`LightComponent.SetIntensity` (`self.PointLight`) _intensity)
      (bind _returnvalue (`GameplayStatics.GetActorOfClass` "/Game/Core/Assets/Interactables/BP_Usage.BP_Usage_C"))
      (set `/Game/Core/Assets/Interactables/BP_Usage.Usage` (`/Game/Core/Assets/Interactables/BP_Usage.Usage` _returnvalue) _returnvalue))))

(event `VentOff`
  (bind _returnvalue (`GameplayStatics.GetActorOfClass` "/Game/Core/Assets/Interactables/BP_Usage.BP_Usage_C"))
  (set `/Game/Core/Assets/Interactables/BP_Usage.Usage` (`/Game/Core/Assets/Interactables/BP_Usage.Usage` _returnvalue) _returnvalue)
  (goto _label :!via `Reverse`))

(fn `UserConstructionScript`)