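; Ceiling light prop that flickers continuously from BeginPlay for as long as it exists.
; A self-calling Flash event waits briefly, picks a random intensity, and applies it to the RectLight and to the mesh material's Bloom-Strength.
; Each flicker creates a new dynamic material instance.
; The construction script applies the Intensity variable the same way, but with a much larger bloom divisor than the runtime loop.
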(event `Flash`
  (bind _intensity (`self.Intensity`))
  (`KismetSystemLibrary.Delay` 0.05 :!label _label)
  (set `self.Intensity` (`KismetMathLibrary.RandomFloatInRange` 900.0 1500.0))
  (bind _returnvalue (`PrimitiveComponent.CreateDynamicMaterialInstance` (`self.SM_CeilingLight02`) 0 "/Game/Core/Assets/Props/CeilingLight/M_CeilingLight02_Inst.M_CeilingLight02_Inst" "None"))
  (`LightComponent.SetIntensity` (`self.RectLight`) _intensity)
  (`MaterialInstanceDynamic.SetScalarParameterValue` _returnvalue "Bloom-Strength" (/ _intensity 32.0))
  (`self.Flash`))

(event `self.ReceiveBeginPlay`
  (goto _label))

(fn `Again`)

(fn `UserConstructionScript`
  (bind _intensity (`self.Intensity`))
  (bind _returnvalue (`PrimitiveComponent.CreateDynamicMaterialInstance` (`self.SM_CeilingLight02`) 0 "/Game/Core/Assets/Props/CeilingLight/M_CeilingLight02_Inst.M_CeilingLight02_Inst" "None"))
  (`LightComponent.SetIntensity` (`self.RectLight`) _intensity)
  (`MaterialInstanceDynamic.SetScalarParameterValue` _returnvalue "Bloom-Strength" (/ _intensity 400.0)))