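; Security camera prop with configurable height, pitch and FOV, viewed through the player's monitor in a game with animatronics.
; Rotary cameras pan back and forth on a ping-pong timeline from a random start, pausing at each end.
; Blur events briefly swap the main camera for a blur camera, using resettable DoOnce gates against retriggering.
; Poor-connection cameras use a dedicated camera component and ignore blurs; a separate event loops the turning sound at random intervals.
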(event `TurningSound`
  (`/Engine/EditorBlueprintResources/StandardMacros.DoOnce` false :!label _label
    (:`Completed`
      (`AudioComponent.Play` (`self.SC_Camera`) 0.0)
      (`KismetSystemLibrary.Delay` (`KismetMathLibrary.RandomFloatInRange` 22.0 60.0))
      (`self.Sound Again`))))

(event `Sound Again`
  (`|ExecutionSequence`
    (:`then_0`
      (goto _label :!via `Reset`))
    (:`then_1`
      (goto _label))))

(event `self.ReceiveBeginPlay`
  (`|ExecutionSequence`
    (:`then_0`
      (if (`self.IsRotary`)
        (`|ExecutionSequence`
          (:`then_0`
            (bind (_direction _rotation) (`Timeline|CameraMovement` :`NewTime` (`KismetMathLibrary.RandomFloatInRange` 0.0 6.8) :!via `SetNewTime` :!label _label_2)
              (:`Update`
                (`SceneComponent.K2_SetRelativeRotation` (`self.Sphere`) (`KismetMathLibrary.MakeRotator` 0.0 0.0 _rotation) false false))
              (:`Finished`
                (`KismetSystemLibrary.Delay` 2.0)
                (`/Engine/EditorBlueprintResources/StandardMacros.FlipFlop`
                  (:`A`
                    (goto _label_2 :!via `Reverse`))
                  (:`B`
                    (goto _label_2))))))
          (:`then_1`
            (goto _label_2)))))
    (:`then_1`
      (if (`self.PoorConnection`)
        (`ActorComponent.Deactivate` (`self.Camera`))
        (`ActorComponent.Activate` (`self.PoorConnectionCamera`) false)))))

(event `CameraBlurEvent`
  (if (not (`self.PoorConnection`))
    (bind _asplayer_bp (cast `/Game/Core/Player/PlayerBP` (`GameplayStatics.GetPlayerCharacter` 0)))
    (if (`/Game/Core/Player/PlayerBP.MonitorUp` _asplayer_bp)
      _
      (else
        _))
    (`/Engine/EditorBlueprintResources/StandardMacros.DoOnce` false :!label _label_3
      (:`Completed`
        (set `self.IsBlurEvent` true)
        (`AudioComponent.Play` (`self.SC_Garble`) 0.0)
        (`ActorComponent.Deactivate` (`self.Camera`))
        (`ActorComponent.Activate` (`self.BlurCamera`) false)
        (`KismetSystemLibrary.Delay` 4.0)
        (`self.GarbleReset`)
        (`ActorComponent.Deactivate` (`self.BlurCamera`))
        (`ActorComponent.Activate` (`self.Camera`) false)))))

(event `GarbleReset`
  (set `self.IsBlurEvent` false)
  (goto _label_3 :!via `Reset`))

(event `ShortBlur`
  (if (`self.PoorConnection`)
    _
    (elif (not (`self.IsBlurEvent`))
      (`/Engine/EditorBlueprintResources/StandardMacros.DoOnce` false :!label _label_4
        (:`Completed`
          (`|ExecutionSequence`
            (:`then_0`
              (`ActorComponent.Deactivate` (`self.Camera`))
              (`ActorComponent.Activate` (`self.BlurCamera`) false)
              (`KismetSystemLibrary.Delay` 0.17)
              (if (not (`self.AnimatronicBlurring?`))
                (`ActorComponent.Deactivate` (`self.BlurCamera`))
                (`ActorComponent.Activate` (`self.Camera`) false)))
            (:`then_1`
              (if (`self.CameraUp`)
                _))
            (:`then_2`
              (`KismetSystemLibrary.Delay` 0.15)
              (`self.BlipReset`))))))))

(event `BlipReset`
  (goto _label_4 :!via `Reset`))

(event `AnimatronicBlur`
  (if (not (`self.PoorConnection`))
    (set `self.AnimatronicBlurring?` true)
    (if (not (`self.IsBlurEvent`))
      (`/Engine/EditorBlueprintResources/StandardMacros.DoOnce` false :!label _label_5
        (:`Completed`
          (`|ExecutionSequence`
            (:`then_0`
              (`ActorComponent.Deactivate` (`self.Camera`))
              (`ActorComponent.Activate` (`self.BlurCamera`) false)
              (`KismetSystemLibrary.Delay` 0.5)
              (set `self.AnimatronicBlurring?` false)
              (`ActorComponent.Deactivate` (`self.BlurCamera`))
              (`ActorComponent.Activate` (`self.Camera`) false))
            (:`then_1`
              (if (`self.CameraUp`)
                (`GameplayStatics.PlaySound2D` "/Game/Core/Assets/Sounds/Blip_Cue.Blip_Cue" 1.0 1.0 0.0 null null)))
            (:`then_2`
              (`KismetSystemLibrary.Delay` 1.5)
              (`self.AnimatronicReset`))))))))

(event `AnimatronicReset`
  (goto _label_5 :!via `Reset`))

(fn `UserConstructionScript`
  (`SceneComponent.K2_SetRelativeLocation` (`self.Camera`) (`KismetMathLibrary.MakeVector` 0.0 0.0 (`self.Z-Drop`)) false false)
  (`SceneComponent.K2_SetRelativeRotation` (`self.Camera`) (`KismetMathLibrary.MakeRotator` 0.0 (`self.Pitch`)) false false)
  (`CameraComponent.SetFieldOfView` (`self.Camera`) (`self.FOV`))
  (`CameraComponent.SetFieldOfView` (`self.BlurCamera`) (`self.FOV`)))