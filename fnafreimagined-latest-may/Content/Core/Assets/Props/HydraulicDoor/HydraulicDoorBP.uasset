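; Hydraulic door prop Blueprint with Open and Close events that slide the Door component vertically along timelines, each with its own sound.
; Open plays a sound and drives the door's relative Z from the OpenDoor timeline.
; Close plays a fast sound, drives Z from the CloseDoor timeline, and shakes the first player's camera when it finishes.
; Alongside closing, four spark components briefly become visible after a short delay.
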(event `Open`
  (`GameplayStatics.PlaySound2D` "/Game/Core/Assets/Sounds/ElevatorOpen3.ElevatorOpen3" 1.0 1.0 0.0 null null)
  (bind (_direction _wow) (`Timeline|OpenDoor` :!via `PlayFromStart`)
    (:`Update`
      (`SceneComponent.K2_SetRelativeLocation` (`self.Door`) (`KismetMathLibrary.MakeVector` 0.0 0.0 (.z _wow)) false false))))

(event `Close`
  (`GameplayStatics.PlaySound2D` "/Game/Core/Assets/Sounds/DoorOpenFast.DoorOpenFast" 1.0 1.0 0.0 null null)
  (`|ExecutionSequence`
    (:`then_0`
      (bind (_direction _location) (`Timeline|CloseDoor` :!via `PlayFromStart`)
        (:`Update`
          (`SceneComponent.K2_SetRelativeLocation` (`self.Door`) (`KismetMathLibrary.MakeVector` 0.0 0.0 (.z _location)) false false))
        (:`Finished`
          (`PlayerCameraManager.StartCameraShake` :`self` (`GameplayStatics.GetPlayerCameraManager` 0) :`ShakeClass` "/Game/Core/Player/CameraShake/DoorCameraShakeBP.DoorCameraShakeBP_C"))))
    (:`then_1`
      (`KismetSystemLibrary.Delay` 0.1)
      (`SceneComponent.SetVisibility` (`self.P_Sparks1`) true false)
      (`SceneComponent.SetVisibility` (`self.P_Sparks`) true false)
      (`SceneComponent.SetVisibility` (`self.P_Sparks3`) true false)
      (`SceneComponent.SetVisibility` (`self.P_Sparks2`) true false)
      (`KismetSystemLibrary.Delay` 0.8)
      (`SceneComponent.SetVisibility` (`self.P_Sparks1`) false false)
      (`SceneComponent.SetVisibility` (`self.P_Sparks`) false false)
      (`SceneComponent.SetVisibility` (`self.P_Sparks3`) false false)
      (`SceneComponent.SetVisibility` (`self.P_Sparks2`) false false))))

(fn `UserConstructionScript`)