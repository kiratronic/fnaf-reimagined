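; Hall light prop Blueprint that flickers its spotlight while Active is true.
; From BeginPlay, a self-calling event loop waits briefly, then picks a random intensity for the SpotLight.
; The same value, scaled down, drives the Bloom parameter of the mesh's emissive material, keeping glow in step with the light.
; Each flicker creates a new dynamic material instance rather than reusing a cached one.
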(event `Again`
  (bind _intensity (`self.Intensity`))
  (if (`self.Active`) :!label _label
    (`KismetSystemLibrary.Delay` 0.1)
    (set `self.Intensity` (`KismetMathLibrary.RandomFloatInRange` 1.0 5.0))
    (bind _returnvalue (`PrimitiveComponent.CreateDynamicMaterialInstance` (`self.StaticMesh`) 0 "/Game/Core/Assets/Props/HallLight/M_Emmisve.M_Emmisve" "None"))
    (`LightComponent.SetIntensity` (`self.SpotLight`) _intensity)
    (`MaterialInstanceDynamic.SetScalarParameterValue` _returnvalue "Bloom" (/ _intensity 32.0))
    (`self.Again`)))

(event `self.ReceiveBeginPlay`
  (goto _label))

(fn `UserConstructionScript`)