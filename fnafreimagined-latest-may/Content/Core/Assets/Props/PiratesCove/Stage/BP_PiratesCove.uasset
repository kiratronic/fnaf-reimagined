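; Pirate's Cove stage prop whose two curtain meshes show staged states named Hidden, Peek, AboutToRun and Run.
; Hidden plays the Curtain timeline from the start to animate the yaw of both curtains.
; Peek, AboutToRun and Run snap both curtains to fixed relative rotations.
; The Blueprint holds no state or trigger logic, so the events rely on outside callers.
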(event `self.ReceiveBeginPlay`)

(event `Hidden`
  (bind (_direction _curtainrotation001 _curtainrotation) (`Timeline|Curtain` :!via `PlayFromStart`)
    (:`Update`
      (`SceneComponent.K2_SetRelativeRotation` (`self.SM_PiratesCove_Curtains_Curtain_001`) (`KismetMathLibrary.MakeRotator` 0.0 0.0 _curtainrotation001) false false)
      (`SceneComponent.K2_SetRelativeRotation` (`self.SM_PiratesCove_Curtains_Curtain`) (`KismetMathLibrary.MakeRotator` 0.0 0.0 _curtainrotation) false false))))

(event `Peek`
  (`SceneComponent.K2_SetRelativeRotation` (`self.SM_PiratesCove_Curtains_Curtain_001`) (struct :`Yaw` -0.3) false false)
  (`SceneComponent.K2_SetRelativeRotation` (`self.SM_PiratesCove_Curtains_Curtain`) (struct :`Yaw` -15.0) false false))

(event `AboutToRun`
  (`SceneComponent.K2_SetRelativeRotation` (`self.SM_PiratesCove_Curtains_Curtain_001`) (struct :`Yaw` -15.3) false false)
  (`SceneComponent.K2_SetRelativeRotation` (`self.SM_PiratesCove_Curtains_Curtain`) (struct :`Yaw` -0.6) false false))

(event `Run`
  (`SceneComponent.K2_SetRelativeRotation` (`self.SM_PiratesCove_Curtains_Curtain_001`) (struct :`Yaw` -19.5) false false)
  (`SceneComponent.K2_SetRelativeRotation` (`self.SM_PiratesCove_Curtains_Curtain`) (struct :`Yaw` 4.1) false false))

(fn `UserConstructionScript`)