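; First-person player character with walk, sprint, crouch, mouse look and a hold-to-show spotlight.
; Timelines drive Q/E SpringArm2 yaw, crouch height and a drink animation, with DoOnce gates guarding crouch and drinking.
; Drinking the held item restores Health, adds Score and clears the Inventory flag.
; Tick line-traces from the camera for autofocus depth of field, toggles the item mesh by Inventory and quits the game at zero Health.
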(event `Key|Q`
  (params (Key :type "Key Structure"))
  (:`Pressed`
    (bind (_direction _newtrack_0) (`Timeline|Timeline_0` :!label _label)
      (:`Update`
        (`SceneComponent.K2_SetRelativeRotation` (`self.SpringArm2`) (`KismetMathLibrary.MakeRotator` 0.0 0.0 _newtrack_0) false false))))
  (:`Released`
    (goto _label :!via `Reverse`)))

(event `Key|E`
  (params (Key :type "Key Structure"))
  (:`Pressed`
    (bind (_direction _newtrack_0) (`Timeline|Timeline` :!label _label_2)
      (:`Update`
        (`SceneComponent.K2_SetRelativeRotation` (`self.SpringArm2`) (`KismetMathLibrary.MakeRotator` 0.0 0.0 _newtrack_0) false false))))
  (:`Released`
    (goto _label_2 :!via `Reverse`)))

(event `Key|LeftShift`
  (params (Key :type "Key Structure"))
  (bind _charactermovement (`self.CharacterMovement`))
  (:`Pressed`
    (set `CharacterMovementComponent.MaxWalkSpeed` 400.0 _charactermovement))
  (:`Released`
    (set `CharacterMovementComponent.MaxWalkSpeed` 150.0 _charactermovement)))

(event `Key|LeftControl`
  (params (Key :type "Key Structure"))
  (bind _charactermovement (`self.CharacterMovement`))
  (:`Pressed`
    (`/Engine/EditorBlueprintResources/StandardMacros.DoOnce` false :!label _label_3
      (:`Completed`
        (`/Engine/EditorBlueprintResources/StandardMacros.FlipFlop`
          (:`A`
            (set `CharacterMovementComponent.MaxWalkSpeed` 50.0 _charactermovement)
            (bind (_direction _newtrack_0) (`Timeline|Crouch Graph` :!via `PlayFromStart` :!label _label_4)
              (:`Update`
                (`SceneComponent.K2_SetRelativeLocation` (`self.SpringArm`) (`KismetMathLibrary.MakeVector` 0.0 0.0 _newtrack_0) false false))
              (:`Finished`
                (`self.CrouchAgain`))))
          (:`B`
            (set `CharacterMovementComponent.MaxWalkSpeed` 150.0 _charactermovement)
            (goto _label_4 :!via `ReverseFromEnd`)))))))

(event `Key|C`
  (params (Key :type "Key Structure"))
  (:`Pressed`
    (goto _label_3)))

(event `CrouchAgain`
  (goto _label_3 :!via `Reset`))

(event `self.ReceiveBeginPlay`
  (bind _returnvalue (`GameplayStatics.GetPlayerCameraManager` 0))
  (set `PlayerCameraManager.ViewPitchMin` -40.0 _returnvalue)
  (set `PlayerCameraManager.ViewPitchMax` 30.0 _returnvalue)
  (set `self.Mouse Sensitivy` 20.0)
  (set `self.Health` 0.5)
  (set `self.inventory` false)
  (`self.beginplaything`)
  (set `self.score` 0))

(event `Key|F`
  (params (Key :type "Key Structure"))
  (:`Pressed`
    (set `self.fkeypres` true))
  (:`Released`
    (set `self.fkeypres` false)))

(event `Key|RightMouseButton`
  (params (Key :type "Key Structure"))
  (bind _spotlight (`self.SpotLight`))
  (:`Pressed`
    (`SceneComponent.SetVisibility` _spotlight true false))
  (:`Released`
    (`SceneComponent.SetVisibility` _spotlight false false)))

(event `InputAxis|LookX`
  (params (AxisValue :type "Float (single-precision)"))
  (`self.AddControllerYawInput` (/ (* AxisValue (`self.Mouse Sensitivy`)) 100.0)))

(event `InputAxis|LookY`
  (params (AxisValue :type "Float (single-precision)"))
  (`self.AddControllerPitchInput` (/ (* (`self.Mouse Sensitivy`) (* AxisValue -1.0)) 110.0)))

(event `InputAxis|MOVEMENTX`
  (params (AxisValue :type "Float (single-precision)"))
  (bind _returnvalue (`GameplayStatics.GetPlayerCameraManager` 0))
  (`self.AddMovementInput` (`KismetMathLibrary.GetForwardVector` (`KismetMathLibrary.MakeRotator` 0.0 0.0 (.yaw (`self.GetControlRotation`)))) AxisValue)
  (if (!= AxisValue 0.0)
    (`LegacyCameraShake.StartLegacyCameraShake` _returnvalue "/Game/Headbob/Walk.Walk_C")
    (else
      (`LegacyCameraShake.StartLegacyCameraShake` _returnvalue))))

(event `InputAxis|MOVEMENTY`
  (params (AxisValue :type "Float (single-precision)"))
  (`self.AddMovementInput` (`KismetMathLibrary.GetRightVector` (`KismetMathLibrary.MakeRotator` 0.0 0.0 (.yaw (`self.GetControlRotation`)))) AxisValue))

(event `resetthing`
  (bind _staticmesh (`self.StaticMesh`))
  (goto _label_6 :!via `Reset`))

(event `resetanim`
  (bind _staticmesh (`self.StaticMesh`))
  (bind (_direction _newtrack_0 _z) (`Timeline|drink` :!via `PlayFromStart` :!label _label_5)
    (:`Update`
      (`SceneComponent.K2_SetRelativeRotation` _staticmesh (`KismetMathLibrary.MakeRotator` _newtrack_0) false false)
      (`SceneComponent.K2_SetRelativeLocation` _staticmesh (`KismetMathLibrary.MakeVector` 76.283777 12.074851 _z) false false))
    (:`Finished`
      (set `self.inventory` false)
      (`self.resetthing`))))

(event `Key|LeftMouseButton`
  (params (Key :type "Key Structure"))
  (:`Pressed`
    (if (`self.inventory`)
      (`/Engine/EditorBlueprintResources/StandardMacros.DoOnce` false :!label _label_6
        (:`Completed`
          (set `self.Health` (`KismetMathLibrary.FClamp` (+ (`self.Health`) 0.05)))
          (`|ExecutionSequence`
            (:`then_0`
              (goto _label_5 :!via `PlayFromStart`))
            (:`then_1`
              (set `self.score` (+ (`self.score`) 25)))))))))

(event `beginplaything`
  (goto _label_5 :!via `ReverseFromEnd`))

(event `resetthingy`
  (bind _staticmesh (`self.StaticMesh`))
  (goto _label_7 :!via `Reset`))

(event `self.ReceiveTick`
  (params (DeltaSeconds :type "Float (single-precision)"))
  (bind _staticmesh (`self.StaticMesh`))
  (bind _staticmesh_2 (`self.StaticMesh`))
  (bind _returnvalue (`SceneComponent.K2_GetComponentLocation` (`self.Camera`)))
  (`|ExecutionSequence`
    (:`then_0`
      (bind (_outhit _returnvalue_2) (`KismetSystemLibrary.LineTraceSingle` _returnvalue (+ (* (`SceneComponent.GetForwardVector` (`self.Camera`)) 10000.0) _returnvalue) "TraceTypeQuery1"))
      (if _returnvalue_2
        (bind _returnvalue_3 (`KismetMathLibrary.VSize` (- (`.Location` (`GameplayStatics.BreakHitResult` _outhit)) (`SceneComponent.K2_GetComponentLocation` (`self.Camera`)))))
        (set `self.Focal Length` _returnvalue_3)
        (set `CameraComponent.PostProcessSettings` (make `PostProcessSettings` :`DepthOfFieldFstop` 1.2 :`DepthOfFieldFocalDistance` (`self.Focal Length`)) (`self.Camera`))
        (else
          (set `self.Focal Length` _returnvalue_3))))
    (:`then_1`
      (if (== (`self.Health`) 0.0)
        (`KismetSystemLibrary.QuitGame` null "Quit")))
    (:`then_2`
      (if (`self.inventory`)
        (`SceneComponent.SetVisibility` _staticmesh true false)
        (`/Engine/EditorBlueprintResources/StandardMacros.DoOnce` true :!label _label_7
          (:`Completed`
            (`SceneComponent.K2_SetRelativeLocation` _staticmesh_2 (76.283777 12.074851 -25.0) false false)
            (`SceneComponent.K2_SetRelativeRotation` _staticmesh_2 (`KismetMathLibrary.MakeRotator` 0.0 0.0 -25.0) false false)))
        (else
          (`SceneComponent.SetVisibility` _staticmesh false false)
          (`self.resetthingy`))))))

(event `UpdateDoF`)

(fn `UserConstructionScript`)