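; Player Blueprint for a Five Nights at Freddy's-style office game, with pitch-clamped mouse look.
; An Interact line trace toggles door lights, honks the Freddy poster or clicks the desk phone.
; Mouse wheel or Space flips a timeline-animated monitor, swapping HUD and camera state and updating BP_Usage.
; Looping timers drive trace-based autofocus and idle or spooked camera sway, while events handle power-out, jumpscare shake and the 6AM screen.
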(event `0Off`
  (if (stale _isa)
    (bind _isa (`/Engine/EditorBlueprintResources/StandardMacros.FlipFlop` :!label _label)
      (:`A`
        (`/Game/Core/Assets/Interactables/DoorButtonBP.LightOn` (`self.Door Button BP`)))
      (:`B`
        (if (== (`/Game/Core/Assets/Interactables/DoorButtonBP.Door` (`self.Door Button BP`)) 0)
          (`/Game/Core/Assets/Interactables/DoorButtonBP.LightOff` (`self.Door Button BP`)))))))

(event `1Off`
  (if (stale _isa)
    (bind _isa (`/Engine/EditorBlueprintResources/StandardMacros.FlipFlop` :!label _label_2)
      (:`A`
        (`/Game/Core/Assets/Interactables/DoorButtonBP.LightOn` (`self.Door Button BP`)))
      (:`B`
        (if (== (`/Game/Core/Assets/Interactables/DoorButtonBP.Door` (`self.Door Button BP`)) 1)
          (`/Game/Core/Assets/Interactables/DoorButtonBP.LightOff` (`self.Door Button BP`)))))))

(event `LeftDoorReset`
  (bind _door_button_bp (`self.Door Button BP`))
  (`/Engine/EditorBlueprintResources/StandardMacros.DoOnce` false :!via `Reset`
    (:`Completed`
      (`/Engine/EditorBlueprintResources/StandardMacros.FlipFlop`
        (:`A`
          (`/Game/Core/Assets/Interactables/DoorButtonBP.DoorClose` _door_button_bp))
        (:`B`
          (`/Game/Core/Assets/Interactables/DoorButtonBP.DoorOpen` _door_button_bp)))
      (`KismetSystemLibrary.Delay` 1.75)
      (`self.LeftDoorReset`))))

(event `RightDoorReset`
  (bind _door_button_bp (`self.Door Button BP`))
  (`/Engine/EditorBlueprintResources/StandardMacros.DoOnce` false :!via `Reset`
    (:`Completed`
      (`/Engine/EditorBlueprintResources/StandardMacros.FlipFlop`
        (:`A`
          (`/Game/Core/Assets/Interactables/DoorButtonBP.DoorClose` _door_button_bp))
        (:`B`
          (`/Game/Core/Assets/Interactables/DoorButtonBP.DoorOpen` _door_button_bp)))
      (`KismetSystemLibrary.Delay` 1.75)
      (`self.RightDoorReset`))))

(event `Key|F`
  (params (Key :type "Key Structure")))

(event `InputAction|Interact`
  (params (Key :type "Key Structure"))
  (bind _camera (`self.Camera`))
  (bind _returnvalue (`SceneComponent.K2_GetComponentLocation` _camera))
  (:`Pressed`
    (if (`self.CanInteract`)
      (if (not (`self.MonitorUp`))
        (bind _outhit (`KismetSystemLibrary.LineTraceSingle` _returnvalue (+ _returnvalue (* (`SceneComponent.GetForwardVector` _camera) 250.0)) "TraceTypeQuery2"))
        (bind (_bblockinghit _binitialoverlap _time _distance _location _impactpoint _normal _impactnormal _physmat _hitactor _hitcomponent) (`GameplayStatics.BreakHitResult` _outhit))
        (bind _asdoor_button_bp (cast `/Game/Core/Assets/Interactables/DoorButtonBP` _hitactor)
          (:`then`
            (set `self.Door Button BP` _asdoor_button_bp)
            (if (== (`/Game/Core/Assets/Interactables/DoorButtonBP.LightCollision` (`self.Door Button BP`)) _hitcomponent)
              (switch `int` (`/Game/Core/Assets/Interactables/DoorButtonBP.Door` (`self.Door Button BP`))
                (:`0`
                  (goto _label))
                (:`1`
                  (goto _label_2)))
              (elif true
                _)))
          (:`CastFailed`
            (bind _asfreddy_poster (cast `/Game/Core/Assets/Props/Posters/FreddyPoster` _hitactor)
              (:`then`
                (if (== (`/Game/Core/Assets/Props/Posters/FreddyPoster.BoxCollision` _asfreddy_poster) _hitcomponent)
                  (if (> (`self.noseclick`) 71)
                    (`/Engine/EditorBlueprintResources/StandardMacros.DoOnce` false :!label _label_3
                      (:`Completed`
                        (`GameplayStatics.PlaySound2D` "/Game/Core/Assets/Sounds/Honk_Cue.Honk_Cue" 1.0 1.0 0.0 null null)
                        (set `self.noseclick` 0)
                        (`KismetSystemLibrary.Delay` 60.0)
                        (goto _label_3 :!via `Reset`)))
                    (else
                      (`/Engine/EditorBlueprintResources/StandardMacros.DoOnce` false :!label _label_4
                        (:`Completed`
                          (`GameplayStatics.PlaySound2D` "/Game/Core/Assets/Sounds/Honk_Cue1.Honk_Cue1" 1.0 1.0 0.0 null null)
                          (set `self.noseclick` (+ (`self.noseclick`) 2))
                          (`KismetSystemLibrary.Delay` 0.5)
                          (goto _label_4 :!via `Reset`)))))))
              (:`CastFailed`
                (bind _asdesk_phone (cast `/Game/Core/Assets/Props/DeskPhone/DeskPhone` _hitactor))
                (if (== (`/Game/Core/Assets/Props/DeskPhone/DeskPhone.Box` _asdesk_phone) _hitcomponent)
                  (`/Game/Core/Assets/Props/DeskPhone/DeskPhone.ClickedPhone` _asdesk_phone))))))))))

(event `self.ReceiveBeginPlay`
  (bind _returnvalue (`GameplayStatics.GetPlayerCameraManager` 0))
  ;[1 1 1] Player Look
  (`self.UIActivation`)
  (set `PlayerCameraManager.ViewPitchMin` 5.0 _returnvalue)
  (set `PlayerCameraManager.ViewPitchMax` 40.0 _returnvalue)
  (`self.StartUp`)
  (set `self.MouseSensitivy` 18.0))

(event `MonitorOn`
  ;[1 1 1] Monitor On / Off
  (`Widget.RemoveFromParent` (stale `MonitorOff` _returnvalue))
  (`self.CamerasActive`)
  (bind _returnvalue (`GameplayStatics.GetActorOfClass` "/Game/Core/Assets/Interactables/BP_Usage.BP_Usage_C"))
  (set `/Game/Core/Assets/Interactables/BP_Usage.Usage` (+ (`/Game/Core/Assets/Interactables/BP_Usage.Usage` _returnvalue) 1) _returnvalue)
  (`/Game/Core/Assets/Interactables/BP_Usage.Update` _returnvalue))

(event `InputAxis|LookX`
  (params (AxisValue :type "Float (single-precision)"))
  ;[1 1 1] Player Look
  (if (not (`self.MonitorUp`))
    (`self.AddControllerYawInput` (/ (* AxisValue (`self.MouseSensitivy`)) 128.0))))

(event `InputAxis|LookY`
  (params (AxisValue :type "Float (single-precision)"))
  ;[1 1 1] Player Look
  (if (not (`self.MonitorUp`))
    (set `self.Pitch Rate` AxisValue)
    (`self.AddControllerPitchInput` (/ (* (`self.MouseSensitivy`) (* AxisValue -1.0)) 200.0))))

(event `MonitorOff`
  ;[1 1 1] Monitor On / Off
  (`self.CamerasInactive`)
  (bind _returnvalue (`|CreateWidget` "/Game/Core/Assets/Widgets/PlayerUI.PlayerUI_C" :!label _label_5))
  (`UserWidget.AddToViewport` _returnvalue 0)
  (bind _returnvalue_2 (`GameplayStatics.GetActorOfClass` "/Game/Core/Assets/Interactables/BP_Usage.BP_Usage_C"))
  (set `/Game/Core/Assets/Interactables/BP_Usage.Usage` (- (`/Game/Core/Assets/Interactables/BP_Usage.Usage` _returnvalue_2) 1) _returnvalue_2)
  (`/Game/Core/Assets/Interactables/BP_Usage.Update` _returnvalue_2))

(event `Key|MouseScrollDown`
  (params (Key :type "Key Structure"))
  (:`Pressed`
    (if (`self.CanInteract`) :!label _label_6
      (`/Engine/EditorBlueprintResources/StandardMacros.FlipFlop`
        (:`A`
          _)
        (:`B`
          _))
      (`/Engine/EditorBlueprintResources/StandardMacros.DoOnce` false :!label _label_7
        (:`Completed`
          (if (`self.CanMonitor?`)
            (`/Engine/EditorBlueprintResources/StandardMacros.FlipFlop`
              (:`A`
                (`GameplayStatics.PlaySound2D` "/Game/Core/Assets/Sounds/panel_in.panel_in" 1.0 1.0 0.0 null null)
                (set `self.MonitorUp` true)
                (bind (_direction _movement_z _movementforward) (`Timeline|MonitorMove` :!via `PlayFromStart` :!label _label_8)
                  (:`Update`
                    (`SceneComponent.K2_SetRelativeLocationAndRotation` (`self.Monitor`) (`KismetMathLibrary.MakeVector` _movementforward 0.0 _movement_z) (`KismetMathLibrary.MakeRotator` 0.0 0.0 90.0) false false))
                  (:`Finished`
                    (if (`self.MonitorUp`)
                      (`self.MonitorOn`))
                    (`KismetSystemLibrary.Delay` 0.05)
                    (`self.MonitorAgain`))))
              (:`B`
                (`GameplayStatics.PlaySound2D` "/Game/Core/Assets/Sounds/panel_out.panel_out" 1.0 1.0 0.0 null null :!label _label_9)
                (set `self.MonitorUp` false)
                (`self.MonitorOff`)
                (goto _label_8 :!via `Reverse`)))))))))

(event `UIActivation`
  ;[1 1 1] Monitor On / Off
  (`/Engine/EditorBlueprintResources/StandardMacros.DoOnce` false
    (:`Completed`
      (set `self.CanMonitor?` true)
      (set `self.CanInteract` true)
      (goto _label_5))))

(event `Key|MouseScrollUp`
  (params (Key :type "Key Structure"))
  (:`Pressed`
    (goto _label_6)))

(event `6 AM`
  (`|ExecutionSequence`
    (:`then_0`
      (`Widget.RemoveFromParent` (stale `MonitorOff` _returnvalue))
      (bind _returnvalue (`|CreateWidget` "/Game/Cinematics/VideoWidget/VideoPlayer.VideoPlayer_C"))
      (set `/Game/Cinematics/VideoWidget/VideoPlayer.SceneType` "6AM" _returnvalue)
      (`UserWidget.AddToViewport` _returnvalue 0))
    (:`then_1`
      (`GameplayStatics.PlaySound2D` "/Game/Cinematics/Cinematics/6AM_Assets/BETA-6am-AUDIO.BETA-6am-AUDIO" 1.0 1.0 0.0 null null))))

(event `Key|SpaceBar`
  (params (Key :type "Key Structure"))
  (:`Pressed`
    (goto _label_6)))

(event `Key|F`
  (params (Key :type "Key Structure"))
  ;[1 1 1] Bob
)

(event `MonitorAgain`
  (goto _label_7 :!via `Reset`))

(event `StartUp`
  ;[1 1 1] Bob
  (`KismetSystemLibrary.K2_SetTimerDelegate` (delegate `UpdateDoF`) 0.1 true)
  (`KismetSystemLibrary.K2_SetTimerDelegate` (delegate `CameraIdleShake`) 1.0 true))

(event `MonitorForceDown`
  (goto _label_9))

(event `CameraIdleShake`
  (bind _springarm1 (`self.SpringArm1`))
  ;[1 1 1] Bob
  (if (`self.Spooked`)
    (bind (_direction _shake) (`Timeline|IdleSpooked` :!via `PlayFromStart`)
      (:`Update`
        (`SceneComponent.K2_SetRelativeLocation` _springarm1 (`KismetMathLibrary.MakeVector` (* _shake 2.0) (* _shake 2.0) (* _shake 2.0)) false false)
        (`SceneComponent.K2_SetRelativeRotation` _springarm1 (`KismetMathLibrary.MakeRotator` (* _shake 2.0) (* _shake 2.0) (* _shake 2.0)) false false)
        (`KismetSystemLibrary.Delay` 1.0)
        (`GameplayStatics.PlaySound2D` "/Game/Core/Assets/Sounds/Heartbeat_Fast__patobottos_.Heartbeat_Fast__patobottos_" 1.0 1.0 0.0 null null)))
    (else
      (bind (_direction_2 _x) (`Timeline|Idle` :!via `PlayFromStart`)
        (:`Update`
          (`SceneComponent.K2_SetRelativeLocation` _springarm1 (`KismetMathLibrary.MakeVector` (* _x 0.5) (* _x 0.5) (* _x 0.5)) false false)
          (`SceneComponent.K2_SetRelativeRotation` _springarm1 (`KismetMathLibrary.MakeRotator` (* _x 0.5) (* _x 0.5) (* _x 0.5)) false false)
          (bind _returnvalue (* _x 0.4))
          (`SceneComponent.K2_SetRelativeRotation` (`self.Camera`) (`KismetMathLibrary.MakeRotator` _returnvalue _returnvalue) false false))))))

(event `Key|A`
  (params (Key :type "Key Structure"))
  (bind _returnvalue (`GameplayStatics.GetPlayerCameraManager` 0))
  (:`Pressed`
    (`PlayerCameraManager.StopCameraShake` _returnvalue null true :!label _label_10)
    (set `self.JumpscareAboutToHappen` true)
    (`LegacyCameraShake.StartLegacyCameraShake` _returnvalue "/Game/Core/Player/CameraShake/JumpscareShakeBP.JumpscareShakeBP_C")))

(event `PowerOff`
  ;[1 1 1] PowerOut
  (set `self.CanInteract` false)
  (`PrimitiveComponent.SetMaterial` (`self.SM_Tablet_Cube_004`) 0 "/Game/Core/Assets/Props/Pizzas/Pizza02/Black.Black")
  (`Widget.RemoveFromParent` (stale `MonitorOff` _returnvalue)))

(event `UpdateDoF`
  (bind _returnvalue (`SceneComponent.K2_GetComponentLocation` (`self.Camera`)))
  ;[1 1 1] Bob
  (bind (_outhit _returnvalue_2) (`KismetSystemLibrary.LineTraceSingle` _returnvalue (+ (* (`SceneComponent.GetForwardVector` (`self.Camera`)) 10000.0) _returnvalue) "TraceTypeQuery1"))
  (if _returnvalue_2
    (bind _returnvalue_3 (`KismetMathLibrary.VSize` (- (`.Location` (`GameplayStatics.BreakHitResult` _outhit)) (`SceneComponent.K2_GetComponentLocation` (`self.Camera`)))))
    (set `self.Focal Length` _returnvalue_3)
    (set `CameraComponent.PostProcessSettings` (make `PostProcessSettings` :`DepthOfFieldFstop` 1.2 :`DepthOfFieldMinFstop` 22.0 :`DepthOfFieldFocalDistance` (`self.Focal Length`)) (`self.Camera`))
    (else
      (set `self.Focal Length` _returnvalue_3))))

(event `JumpscareShakeTrigger`
  (goto _label_10))

(event `SpookMovement`
  (bind _camera (`self.Camera`))
  ;[1 1 1] Spook
  (set `self.Spooked` true)
  (`|ExecutionSequence`
    (:`then_0`
      (bind (_direction _fov) (`Timeline|Spook` :!via `PlayFromStart`)
        (:`Update`
          (`CameraComponent.SetFieldOfView` _camera _fov))))
    (:`then_1`
      (bind (_direction_2 _rot) (`Timeline|RotationalCameraSpook` :!via `PlayFromStart`)
        (:`Update`
          (`SceneComponent.K2_SetRelativeRotation` _camera (`KismetMathLibrary.MakeRotator` (* _rot 0.5) _rot) false false))))
    (:`then_2`
      (`KismetSystemLibrary.Delay` (`KismetMathLibrary.RandomFloatInRange` 8.0 15.0))
      (set `self.Spooked` false))))

(event `Blink`
  ;[1 1 1] My Eyes
  (`KismetSystemLibrary.PrintString` "PlayerBP Cannot Blink!" true true (struct :`R` 1.0 :`G` 0.566729 :`A` 1.0)))

(event `InputAction|Interact`
  (params (Key :type "Key Structure"))
  (:`Pressed`
    (`self.ClickOn`))
  (:`Released`
    (`self.ClickOff`)))

(event `JumpscareOver`
  (`PlayerCameraManager.StopCameraShake` (`GameplayStatics.GetPlayerCameraManager` 0) null true)
  (set `self.JumpscareAboutToHappen` true))

(fn `UserConstructionScript`)