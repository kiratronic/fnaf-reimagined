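; Rain actor that drives a Niagara rain system with optional splashes and box-shaped ambient sound.
; One init routine, run on construction, BeginPlay and UpdateGoodRain, pushes color, spawn, wind, collision, bounds and quality-based material settings into Niagara.
; Splashes take a percentage of the total spawn rate, and sound volume follows rain density.
; Debug mode previews spawn area, bounds and sound falloff; disabling the system hides and deactivates it.
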(event `self.ReceiveTick`
  (params (DeltaSeconds :type "Float (single-precision)")))

(event `self.ReceiveBeginPlay`
  ;[1 1 1] Init
  (`self.Init Good Rain System`))

(event `Update Good Rain`
  ;[1 1 1] update event
  (`self.Init Good Rain System`))

(fn `Init Good Rain System`
  ;[1 1 1] Refresh (alway false)
  (if (`self.Refresh`)
    _
    (else
      _))
  (set `self.Refresh` false)
  (if (`self.Enable Rain System`)
    (`self.Init Base Variable Settings`)
    (`self.Init Sound`)
    ;[0.5997 0.5625 1] Debug mode let you easy to see some function in game.
    ; ------------------------------------------------------------
    ; If you see....... (in editor or game mode).
    ;
    ; Green Box : Rain Influence Area
    ; Purple Box ( Wire ) : Bound Box
    ; Big Yellow Box ( Wire )  : Out of Sound Influence Area = 0
    ; Small Yellow Box ( Wire ) : In Sound Influence Area = 1
    ;
    ; Blue rain : GPU particle ( don't generate splash )
    ; Red rain : CPU particle ( generate splash )
    (`self.Init Debug Mode`)
    (`self.Init Quality`)
    (else
      ;[1 1 1] Hide and Deactivate
      (`SceneComponent.SetVisibility` (`self.Scene`) false true)
      (`ActorComponent.Deactivate` (`self.Debug Box`))
      (`ActorComponent.Deactivate` (`self.Sound TEXT 02`))
      (`ActorComponent.Deactivate` (`self.Ambient Rain Sound`))
      (`ActorComponent.Deactivate` (`self.Sound TEXT 01`))
      (`ActorComponent.Deactivate` (`self.Bound Box`))
      (`ActorComponent.Deactivate` (`self.NS_Good Rain`)))))

(fn `UserConstructionScript`
  (`self.Init Good Rain System`))