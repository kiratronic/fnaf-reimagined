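; Cutscene character Blueprint for Chica, driven by custom events that pose her and toggle her visible details.
; Night6 plays a non-looping stage pose animation and teleports the actor to a hardcoded location and rotation.
; ShowChicaDetails and HideChicaDetails swap the mesh's mech and eye materials with a transparent one while toggling a Cube's visibility inversely.
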(event `Night6`
  (`SkeletalMeshComponent.PlayAnimation` (`self.Chica`) "/Game/Core/Assets/Characters/Chica/Animations/ChicaStagePose.ChicaStagePose" false)
  (`self.K2_TeleportTo` (-24178.118272 164.283205 84.067292) (struct :`Yaw` 90.0)))

(event `ShowChicaDetails`
  (`PrimitiveComponent.SetMaterial` (`self.Chica`) 2 "/Game/Core/Assets/Characters/Mech/Materials/M_Mech.M_Mech")
  (`PrimitiveComponent.SetMaterial` (`self.Chica`) 1 "/Game/Core/Assets/Characters/Chica/Materials/M_Eye.M_Eye")
  (`SceneComponent.SetVisibility` (`self.Cube`) false false))

(event `HideChicaDetails`
  (`PrimitiveComponent.SetMaterial` (`self.Chica`) 2 "/Game/Core/Assets/Characters/Mech/Materials/M_transparent.M_transparent")
  (`PrimitiveComponent.SetMaterial` (`self.Chica`) 1 "/Game/Core/Assets/Characters/Mech/Materials/M_transparent.M_transparent")
  (`SceneComponent.SetVisibility` (`self.Cube`) true false))

(fn `UserConstructionScript`)