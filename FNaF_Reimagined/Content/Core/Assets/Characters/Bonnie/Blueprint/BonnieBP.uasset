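; Bonnie animatronic AI for a night-based office survival game, roaming from the stage toward the left office door.
; DifficultyDefine sets aggression and wait time per night, then BeginCycle repeatedly rolls against aggression to pick neighboring rooms.
; MoveTrigger teleports Bonnie into looping poses, and moves toward the hallway side hold while Foxy is at stage 3 or running.
; Tick polls door state for office entry; JumpscareCall plays the scare.
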(event `Door Sequence`
  ;[1 1 1] Door Logic
  (if (`self.AtDoor`)
    (if (`self.LeftDoorClosed`)
      (`KismetSystemLibrary.Delay` 0.05)
      (if (not (`self.LeftDoorClosed`))
        (`KismetSystemLibrary.Delay` 1.0)
        (if (not (`self.LeftDoorClosed`)) :!label _label
          (set `self.InOffice` true)
          (`self.InOfficeLogic`)
          (`KismetSystemLibrary.PrintString` "InOffice")))
      (elif (`self.LightOn`)
        (`KismetSystemLibrary.Delay` 3.0)
        (goto _label)))))

(event `InOfficeLogic`
  (`self.BonnieInOffice`)
  (`self.K2_TeleportTo` (0.0 0.0 500.0))
  (`KismetSystemLibrary.PrintString` "InOffice"))

(event `BeginCycle`
  ;[1 1 1] MovementChance
  (`KismetSystemLibrary.Delay` (`self.WaitTime`))
  (if (`self.CanMove`)
    (if (and (`self.InOffice`) (`self.HoldingPosition`))
      (`self.BeginCycle`)
      (elif (<= (`KismetMathLibrary.RandomIntegerInRange` 0 20) (`self.AIDifficulty`))
        (`self.MovementCycle`)
        (else
          (`self.BeginCycle`))))
    (else
      (`self.BeginCycle`))))

(event `JumpscareCall`
  (`SceneComponent.SetRelativeScale3D` (`self.SkeletalMesh`) (0.75 0.75 0.75))
  (`self.K2_TeleportTo` :`self` self :`DestLocation` (-100.68499 -66.185059 20.0))
  (`SkeletalMeshComponent.PlayAnimation` (`self.SkeletalMesh`) "/Game/Core/Assets/Characters/Bonnie/Animations/Bonnie_jumpy__1__RIG_Bonnie_ao_Action.Bonnie_jumpy__1__RIG_Bonnie_ao_Action" false)
  (`SkeletalMeshComponent.PlayAnimation` (`self.CameraLink`) "/Game/Core/Assets/Characters/Bonnie/Animations/Bonnie_jumpyCUBE_Anim_Cube_002_Cube_002Action_001.Bonnie_jumpyCUBE_Anim_Cube_002_Cube_002Action_001" false))

(event `self.ReceiveBeginPlay`
  (`self.StageMove`)
  (`KismetSystemLibrary.Delay` 2.0)
  (`self.Difficulty Define`))

(event `self.ReceiveTick`
  (params (DeltaSeconds :type "Float (single-precision)"))
  (`self.Door Sequence`))

(event `StageMove`
  ;[1 1 1] Teleport And Animation
  (`self.K2_TeleportTo` (2972.123535 -182.529968 90.0) (struct :`Yaw` 90.0) :!label _label_2)
  (`SkeletalMeshComponent.PlayAnimation` (`self.SkeletalMesh`) "/Game/Core/Assets/Characters/Bonnie/Animations/bonnie_pose1.bonnie_pose1" true))

(event `MoveTrigger`
  ;[1 1 1] Teleport And Animation
  (`|ExecutionSequence`
    (:`then_0`
      (switch `string` (`self.ArrivalLocation`)
        (:`Default`
          (`self.BeginCycle`)
          (`KismetSystemLibrary.PrintString` (`self.ArrivalLocation`) true true (struct :`R` 0.650518 :`G` 1.0 :`A` 1.0)))
        (:`Stage`
          (goto _label_2))
        (:`Dining1`
          (`self.K2_TeleportTo` (2518.854248 -24.444901 56.459915) (struct :`Yaw` -70.0))
          (`SkeletalMeshComponent.PlayAnimation` (`self.SkeletalMesh`) "/Game/Core/Assets/Characters/Bonnie/Animations/DiningRoom01/S_Bonnie_Sequence1.S_Bonnie_Sequence1" true))
        (:`Dining2`
          (`self.K2_TeleportTo` (1833.505371 -98.677132 20.0) (struct :`Yaw` -90.0))
          (`SkeletalMeshComponent.PlayAnimation` (`self.SkeletalMesh`) "/Game/Core/Assets/Characters/Bonnie/Animations/ANIM_Closet.ANIM_Closet" true))
        (:`EmployeeOnly1`
          (if (`KismetMathLibrary.RandomBool`)
            (`self.K2_TeleportTo` (3030.417969 -1169.113525 20.0) (struct :`Yaw` 150.0))
            (`SkeletalMeshComponent.PlayAnimation` (`self.SkeletalMesh`) "/Game/Core/Assets/Characters/Bonnie/Animations/BonnieCorner_v1.BonnieCorner_v1" true)
            (else
              (`self.K2_TeleportTo` (3041.948486 -1236.466797 20.0) (struct :`Yaw` -205.0))
              (`SkeletalMeshComponent.PlayAnimation` (`self.SkeletalMesh`) "/Game/Core/Assets/Characters/Bonnie/Animations/Backstage02.Backstage02" true))))
        (:`LeftHallway`
          (`self.K2_TeleportTo` (929.89032 -300.740875 24.145002) (struct :`Yaw` 109.344772))
          (`SkeletalMeshComponent.PlayAnimation` (`self.SkeletalMesh`) "/Game/Core/Assets/Characters/Bonnie/Animations/HallwayNEW.HallwayNEW" true))
        (:`Closet`
          (`self.K2_TeleportTo` (735.728394 -618.101135 20.0) (struct :`Yaw` 10.0))
          (`SkeletalMeshComponent.PlayAnimation` (`self.SkeletalMesh`) "/Game/Core/Assets/Characters/Bonnie/Animations/ANIM_Closet.ANIM_Closet" true))
        (:`LeftCorner`
          (`self.K2_TeleportTo` (-528.0 -249.0 18.0) (struct :`Yaw` 259.19928))
          (`SkeletalMeshComponent.PlayAnimation` (`self.SkeletalMesh`) "/Game/Core/Assets/Characters/Bonnie/Animations/Hallway/A_HallwayCornerV2.A_HallwayCornerV2" true))
        (:`LeftDoor`
          (`self.K2_TeleportTo` (-269.123688 -254.594757 20.0) (struct :`Yaw` -20.0))
          (`SkeletalMeshComponent.PlayAnimation` (`self.SkeletalMesh`) "/Game/Core/Assets/Characters/Bonnie/Animations/bonnie_Door.bonnie_Door" true))))
    (:`then_1`
      (if (`KismetStringLibrary.EqualEqual_StrStr` (`self.ArrivalLocation`) "LeftDoor")
        (`self.Door Sequence`)
        (`self.BeginCycle`)
        (else
          (`self.BeginCycle`)
          (set `self.AtDoor` false))))))

(event `TryAgain`
  (bind _returnvalue (`KismetMathLibrary.RandomIntegerInRange` 0 2))
  (bind _returnvalue_2 (!= _returnvalue (`self.RNGMove`)))
  ;[1 1 1] Random Movement
  (switch `string` (`self.CurrentLocation`) :!label _label_3
    (:`Stage`
      (switch `int` _returnvalue :!label _label_4
        (:`0`
          (if _returnvalue_2
            (`self.Dining1`)
            (set `self.RNGMove` 0)
            (else
              (`self.TryAgain` :!label _label_5)
              (`KismetSystemLibrary.PrintString` "BonnieTryAgain" true true (struct :`R` 1.0 :`G` 0.133929 :`A` 1.0)))))
        (:`1`
          (if _returnvalue_2
            (`self.Dining2`)
            (set `self.RNGMove` 1)
            (else
              (goto _label_5))))
        (:`2`
          (if _returnvalue_2
            (`self.EmployeeOnly1`)
            (set `self.RNGMove` 2)
            (else
              (goto _label_5))))))
    (:`Dining1`
      (goto _label_4))
    (:`Dining2`
      (if (> (`KismetMathLibrary.RandomIntegerInRange` 0 20) (`self.AIDifficulty`))
        (goto _label_4)
        (else
          (`self.Hallway`))))
    (:`EmployeeOnly1`
      (goto _label_4))
    (:`LeftHallway`
      (if (> (`KismetMathLibrary.RandomIntegerInRange` 0 20) (`self.AIDifficulty`))
        (`self.Dining2`)
        (elif (`KismetMathLibrary.RandomBool`)
          (`self.Corner`)
          (else
            (`self.Closet`)))))
    (:`Closet`
      (if (> (`KismetMathLibrary.RandomIntegerInRange` 0 20) (`self.AIDifficulty`))
        (`self.Hallway`)
        (else
          (`self.Corner`))))
    (:`LeftCorner`
      (if (> (`KismetMathLibrary.RandomIntegerInRange` 0 20) (`self.AIDifficulty`))
        (if (`KismetMathLibrary.RandomBool`)
          (`self.Hallway`)
          (else
            (`self.Corner`)))
        (else
          (`self.Door`))))
    (:`LeftDoor`
      (if (`self.LeftDoorClosed`)
        (if (`KismetMathLibrary.RandomBool`)
          (`self.Dining1`)
          (elif (`KismetMathLibrary.RandomBool`)
            (`self.Hallway`)
            (else
              (`self.Dining2`))))
        (`self.BonnieFromDoor`)
        (else
          (set `self.InOffice` true)
          (`self.InOfficeLogic`))))))

(event `MovementCycle`
  ;[1 1 1] Random Movement
  (goto _label_3))

(event `Difficulty Define`
  ;[1 1 1] Difficulty
  (switch `string` (`self.Night`)
    (:`Night1`
      (`KismetSystemLibrary.PrintString` "222")
      (set `self.AIDifficulty` 10)
      (set `self.WaitTime` (`KismetMathLibrary.RandomFloatInRange` 7.0 10.0))
      (`KismetSystemLibrary.Delay` 0.0)
      (set `self.CanMove` false)
      (`self.BeginCycle`))
    (:`Night2`
      (set `self.AIDifficulty` 5)
      (set `self.WaitTime` (`KismetMathLibrary.RandomFloatInRange` 15.0 25.0))
      (`KismetSystemLibrary.Delay` 60.0)
      (set `self.CanMove` true)
      (`self.BeginCycle`))
    (:`Night3`
      (set `self.AIDifficulty` 5)
      (set `self.WaitTime` (`KismetMathLibrary.RandomFloatInRange` 15.0 25.0))
      (`KismetSystemLibrary.Delay` 60.0)
      (set `self.CanMove` true)
      (`self.BeginCycle`))
    (:`Night4`
      (set `self.AIDifficulty` 8)
      (set `self.WaitTime` (`KismetMathLibrary.RandomFloatInRange` 15.0 25.0))
      (`KismetSystemLibrary.Delay` 60.0)
      (set `self.CanMove` true)
      (`self.BeginCycle`))
    (:`Night5`
      (set `self.AIDifficulty` 12)
      (set `self.WaitTime` (`KismetMathLibrary.RandomFloatInRange` 15.0 25.0))
      (`KismetSystemLibrary.Delay` 60.0)
      (set `self.CanMove` true)
      (`self.BeginCycle`))
    (:`Night6`
      (set `self.AIDifficulty` 14)
      (set `self.WaitTime` (`KismetMathLibrary.RandomFloatInRange` 5.0 17.0))
      (`KismetSystemLibrary.Delay` 7.0)
      (set `self.CanMove` true)
      (`self.BeginCycle`))))

(event `Dining1`
  ;[1 1 1] Movement Action
  (if (`self.HoldingPosition`)
    (`self.BeginCycle`)
    (else
      (bind _output_get (set `self.ArrivalLocation` "Dining1"))
      (`self.CameraBlur`)
      (set `self.CurrentLocation` _output_get)
      (`self.MoveTrigger`))))

(event `Dining2`
  ;[1 1 1] Movement Action
  (if (`self.HoldingPosition`)
    (`self.BeginCycle`)
    (else
      (bind _output_get (set `self.ArrivalLocation` "Dining2"))
      (`self.CameraBlur`)
      (set `self.CurrentLocation` _output_get)
      (`self.MoveTrigger`))))

(event `EmployeeOnly1`
  ;[1 1 1] Movement Action
  (if (`self.HoldingPosition`)
    (`self.BeginCycle`)
    (else
      (bind _output_get (set `self.ArrivalLocation` "EmployeeOnly1"))
      (`self.CameraBlur`)
      (set `self.CurrentLocation` _output_get)
      (`self.MoveTrigger`))))

(event `StageSpookMoment`
  (if (`KismetStringLibrary.EqualEqual_StrStr` (`self.CurrentLocation`) "Stage")
    (`SkeletalMeshComponent.PlayAnimation` (`self.SkeletalMesh`) "/Game/Core/Assets/Characters/Bonnie/Animations/BonnieStageSpook.BonnieStageSpook" true)))

(event `Hallway`
  ;[1 1 1] Movement Action
  (bind _returnvalue (`GameplayStatics.GetActorOfClass` "/Game/Core/Assets/Characters/Foxy/Blueprint/FoxyStageBP.FoxyStageBP_C"))
  (if (or (== (`/Game/Core/Assets/Characters/Foxy/Blueprint/FoxyStageBP.ArrivalStage` _returnvalue) 3) (`/Game/Core/Assets/Characters/Foxy/Blueprint/FoxyStageBP.Running` _returnvalue))
    (set `self.HoldingPosition` true)
    (else
      (set `self.HoldingPosition` false)))
  (if (`self.HoldingPosition`)
    (`self.BeginCycle`)
    (else
      (bind _output_get (set `self.ArrivalLocation` "LeftHallway"))
      (`self.CameraBlur`)
      (set `self.CurrentLocation` _output_get)
      (`self.MoveTrigger`))))

(event `StageSpookOff`
  (if (`KismetStringLibrary.EqualEqual_StrStr` (`self.CurrentLocation`) "Stage")
    (`SkeletalMeshComponent.PlayAnimation` (`self.SkeletalMesh`) "/Game/Core/Assets/Characters/Bonnie/Animations/bonnie_pose1.bonnie_pose1" true)))

(event `Closet`
  ;[1 1 1] Movement Action
  (bind _returnvalue (`GameplayStatics.GetActorOfClass` "/Game/Core/Assets/Characters/Foxy/Blueprint/FoxyStageBP.FoxyStageBP_C"))
  (if (or (== (`/Game/Core/Assets/Characters/Foxy/Blueprint/FoxyStageBP.ArrivalStage` _returnvalue) 3) (`/Game/Core/Assets/Characters/Foxy/Blueprint/FoxyStageBP.Running` _returnvalue))
    (set `self.HoldingPosition` true)
    (else
      (set `self.HoldingPosition` false)))
  (if (`self.HoldingPosition`)
    (`self.BeginCycle`)
    (else
      (bind _output_get (set `self.ArrivalLocation` "Closet"))
      (`self.CameraBlur`)
      (set `self.CurrentLocation` _output_get)
      (`self.MoveTrigger`))))

(event `Corner`
  ;[1 1 1] Movement Action
  (bind _returnvalue (`GameplayStatics.GetActorOfClass` "/Game/Core/Assets/Characters/Foxy/Blueprint/FoxyStageBP.FoxyStageBP_C"))
  (if (or (== (`/Game/Core/Assets/Characters/Foxy/Blueprint/FoxyStageBP.ArrivalStage` _returnvalue) 3) (`/Game/Core/Assets/Characters/Foxy/Blueprint/FoxyStageBP.Running` _returnvalue))
    (set `self.HoldingPosition` true)
    (else
      (set `self.HoldingPosition` false)))
  (if (`self.HoldingPosition`)
    (`self.BeginCycle`)
    (else
      (bind _output_get (set `self.ArrivalLocation` "LeftCorner"))
      (`self.CameraBlur`)
      (set `self.CurrentLocation` _output_get)
      (`self.MoveTrigger`))))

(event `Door`
  ;[1 1 1] Movement Action
  (bind _returnvalue (`GameplayStatics.GetActorOfClass` "/Game/Core/Assets/Characters/Foxy/Blueprint/FoxyStageBP.FoxyStageBP_C"))
  (if (or (== (`/Game/Core/Assets/Characters/Foxy/Blueprint/FoxyStageBP.ArrivalStage` _returnvalue) 3) (`/Game/Core/Assets/Characters/Foxy/Blueprint/FoxyStageBP.Running` _returnvalue))
    (set `self.HoldingPosition` true)
    (else
      (set `self.HoldingPosition` false)))
  (if (`self.HoldingPosition`)
    (`self.BeginCycle`)
    (else
      (`self.BonnieToDoor`)
      (bind _output_get (set `self.ArrivalLocation` "LeftDoor"))
      (`self.CameraBlur`)
      (set `self.CurrentLocation` _output_get)
      (`self.MoveTrigger`)
      (set `self.AtDoor` true))))

(fn `UserConstructionScript`)