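; Freddy Fazbear's power-out show actor, which plays the Toreador cover tune with flickering lights once StartShow is triggered.
; StartShow sets the active flag and plays the music at the actor's location, guarded by a DoOnce.
; A self-looping Delay with a random interval then keeps setting three point lights to random intensities while the flag stays true, producing an irregular flicker.
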(event `StartShow`
  (set `self.IsActive` true)
  (`|ExecutionSequence`
    (:`then_0`
      (`/Engine/EditorBlueprintResources/StandardMacros.DoOnce` false
        (:`Completed`
          (`GameplayStatics.PlaySoundAtLocation` "/Game/Core/Assets/Sounds/Toreador_Cover_Cue.Toreador_Cover_Cue" (`self.K2_GetActorLocation`) (struct) 1.0 1.0 0.0 null null null null))))
    (:`then_1`
      (if (`self.IsActive`) :!label _label
        (`KismetSystemLibrary.Delay` (`KismetMathLibrary.RandomFloatInRange` 0.02 0.2))
        (`LightComponent.SetIntensity` (`self.PointLight`) (`KismetMathLibrary.RandomFloatInRange` 100.0 500.0))
        (`LightComponent.SetIntensity` (`self.PointLight1`) (`KismetMathLibrary.RandomFloatInRange` 100.0 500.0))
        (`LightComponent.SetIntensity` (`self.PointLight2`) (`KismetMathLibrary.RandomFloatInRange` 100.0 500.0))
        (goto _label)))))

(fn `UserConstructionScript`)