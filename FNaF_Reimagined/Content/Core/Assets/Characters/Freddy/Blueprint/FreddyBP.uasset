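; Freddy animatronic AI for a Five Nights at Freddy's-style game, stalking the player from stage to office.
; The level name sets AI difficulty and wait time for a looping random roll that advances him room by room, stalling while cameras are active or Chica occupies certain destinations.
; Each move teleports him and swaps his looping animation.
; At the right corner, a closed door sends him back; otherwise he enters the office, with separate jumpscare events.
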(event `Door Sequence`
  ;[1 1 1] Door Logic
  (if (`self.AtDoor`)
    (if (`self.RightDoorClosed`)
      (`KismetSystemLibrary.Delay` 0.05)
      (if (not (`self.RightDoorClosed`))
        (`KismetSystemLibrary.Delay` 1.0)
        (if (not (`self.RightDoorClosed`)) :!label _label
          (set `self.InOffice` true)
          (`self.InOfficeLogic`)
          (`KismetSystemLibrary.PrintString` "InOffice")))
      (elif (`self.LightOn`)
        (`KismetSystemLibrary.Delay` 3.0)
        (goto _label)))))

(event `InOfficeLogic`
  (bind _skeletalmesh (`self.SkeletalMesh`))
  (`self.FreddyInOffice`)
  (`self.K2_TeleportTo` (-357.035309 -10.0 20.0) (struct :`Yaw` -90.0))
  (`SkeletalMeshComponent.PlayAnimation` _skeletalmesh "/Game/Core/Assets/Characters/Bonnie/Animations/bonnie_prejumpscare.bonnie_prejumpscare" true)
  (`PrimitiveComponent.SetMaterial` _skeletalmesh 2 "/Game/Core/Assets/Characters/Shared/Material/EmmissiveEye_MI.EmmissiveEye_MI")
  (`KismetSystemLibrary.PrintString` "InOffice"))

(event `StageMove`
  ;[1 1 1] Teleport And Animation
  (`self.K2_TeleportTo` (2872.343018 0.0 90.0) (struct :`Yaw` 90.0) :!label _label_2)
  (`SkeletalMeshComponent.PlayAnimation` (`self.SkeletalMesh`) "/Game/Core/Assets/Characters/Freddy/Animations/FreddyStage.FreddyStage" true)
  (`SceneComponent.SetVisibility` (`self.GlowingLeftEye`) false false)
  (`SceneComponent.SetVisibility` (`self.GlowingLeftEye1`) false false))

(event `BeginCycle`
  ;[1 1 1] MovementChance
  (`KismetSystemLibrary.Delay` (`self.WaitTime`))
  (if (`self.CanMove`)
    (if (and (`self.InOffice`) (`self.HoldingPosition`))
      (`self.BeginCycle`)
      (elif (<= (`KismetMathLibrary.RandomIntegerInRange` 0 20) (`self.AIDifficulty`))
        (if (`self.CamerasActive`)
          (`self.BeginCycle`)
          (else
            (`self.MovementCycle`)))
        (else
          (`self.BeginCycle`))))
    (else
      (`self.BeginCycle`))))

(event `Jumpscare`
  (`self.FreddyJumpscare`)
  (`SkeletalMeshComponent.PlayAnimation` (`self.SkeletalMesh`) "/Game/Core/Assets/Characters/Bonnie/Animations/bonnie_jumpscare.bonnie_jumpscare" true)
  (`SceneComponent.SetVisibility` (`self.PointLight`) true false))

(event `MoveTrigger`
  (bind _arrivallocation (`self.ArrivalLocation`))
  ;[1 1 1] Teleport And Animation
  (`KismetSystemLibrary.PrintString` _arrivallocation true true (struct :`R` 1.0 :`G` 0.554034 :`A` 1.0))
  (`|ExecutionSequence`
    (:`then_0`
      (switch `string` (`self.ArrivalLocation`)
        (:`Default`
          (`self.BeginCycle`)
          (`KismetSystemLibrary.PrintString` (`self.ArrivalLocation`) true true (struct :`R` 0.650518 :`G` 1.0 :`A` 1.0)))
        (:`Stage`
          (goto _label_2))
        (:`DiningRoom`
          (`self.K2_TeleportTo` (1631.671143 238.461166 20.0) (struct :`Yaw` -105.0))
          (`SkeletalMeshComponent.PlayAnimation` (`self.SkeletalMesh`) "/Game/Core/Assets/Characters/Freddy/Animations/FreddyDining1.FreddyDining1" true)
          (`SceneComponent.SetVisibility` (`self.GlowingLeftEye`) true false)
          (`SceneComponent.SetVisibility` (`self.GlowingLeftEye1`) true false))
        (:`Bathroom`
          (`self.K2_TeleportTo` (2622.318359 1276.225098 -7.542852) (struct :`Pitch` -24.092936 :`Yaw` 206.470276 :`Roll` -6.881703))
          (`SkeletalMeshComponent.PlayAnimation` (`self.SkeletalMesh`) "/Game/Core/Assets/Characters/Freddy/Animations/FreddyBathrooms.FreddyBathrooms" true)
          (`SceneComponent.SetVisibility` (`self.GlowingLeftEye`) false false)
          (`SceneComponent.SetVisibility` (`self.GlowingLeftEye1`) false false))
        (:`Kitchen`
          (`self.K2_TeleportTo` (0.0 0.0 500.0))
          (`SkeletalMeshComponent.PlayAnimation` (`self.SkeletalMesh`) null true)
          (`GameplayStatics.PlaySoundAtLocation` null (974.232117 968.572815 20.0) (struct) 1.0 1.0 0.0 null null null null))
        (:`Hallway`
          (`self.K2_TeleportTo` (775.276001 323.311249 20.0) (struct :`Yaw` 88.0))
          (`SkeletalMeshComponent.PlayAnimation` (`self.SkeletalMesh`) "/Game/Core/Assets/Characters/Freddy/Animations/FreddyHallway.FreddyHallway" true))
        (:`RightCorner`
          (`self.K2_TeleportTo` (-453.318512 270.23584 81.349312) (struct :`Yaw` -128.0))
          (`SkeletalMeshComponent.PlayAnimation` (`self.SkeletalMesh`) "/Game/Core/Assets/Characters/Freddy/Animations/FreddyCorner.FreddyCorner" true))
        (:`RightDoor`
          (`self.K2_TeleportTo` (0.0 0.0 400.0))
          (`SkeletalMeshComponent.PlayAnimation` (`self.SkeletalMesh`) null true))))
    (:`then_1`
      (if (`KismetStringLibrary.EqualEqual_StrStr` _arrivallocation "LeftDoor")
        (`self.Door Sequence`)
        (`self.BeginCycle`)
        (else
          (`self.BeginCycle`)
          (set `self.AtDoor` false))))))

(event `self.ReceiveBeginPlay`
  (`self.StageMove`)
  (`self.Difficulty Define`))

(event `JumpscareCall`
  (`SkeletalMeshComponent.PlayAnimation` (`self.SkeletalMesh`) "/Game/Core/Assets/Characters/Bonnie/Animations/bonnie_jumpscare.bonnie_jumpscare" true)
  (`SceneComponent.SetVisibility` (`self.PointLight`) true false))

(event `self.ReceiveTick`
  (params (DeltaSeconds :type "Float (single-precision)"))
  (`self.Door Sequence`))

(event `TryAgain`
  ;[1 1 1] Random Movement
  (switch `string` (`self.CurrentLocation`) :!label _label_3
    (:`Stage`
      (`self.DiningRoom`))
    (:`DiningRoom`
      (`self.Bathroom`))
    (:`Bathroom`
      (`self.Kitchen`))
    (:`Kitchen`
      (`self.RightHallway`))
    (:`Hallway`
      (`self.RightCorner`))
    (:`RightCorner`
      (if (`self.RightDoorClosed`)
        (if (`KismetMathLibrary.RandomBool`)
          (`self.DiningRoom`)
          (else
            (`self.Bathroom`)))
        (`self.FreddyFromDoor`)
        (else
          (set `self.InOffice` true)
          (`self.InOfficeLogic`))))))

(event `MovementCycle`
  ;[1 1 1] Random Movement
  (goto _label_3))

(event `Difficulty Define`
  ;[1 1 1] Difficulty
  (bind _returnvalue (`GameplayStatics.GetCurrentLevelName` true))
  (switch `string` _returnvalue
    (:`LVL_Night1`
      (set `self.AIDifficulty` 0)
      (set `self.WaitTime` (`KismetMathLibrary.RandomFloatInRange` 20.0 30.0))
      (`KismetSystemLibrary.Delay` 60.0)
      (set `self.CanMove` true)
      (`self.BeginCycle`))
    (:`LVL_Night2`
      (set `self.AIDifficulty` 5)
      (set `self.WaitTime` (`KismetMathLibrary.RandomFloatInRange` 15.0 25.0))
      (`KismetSystemLibrary.Delay` 60.0)
      (set `self.CanMove` true)
      (`self.BeginCycle`))
    (:`LVL_Night3`
      (set `self.AIDifficulty` 5)
      (set `self.WaitTime` (`KismetMathLibrary.RandomFloatInRange` 15.0 25.0))
      (`KismetSystemLibrary.Delay` 60.0)
      (set `self.CanMove` true)
      (`self.BeginCycle`))
    (:`LVL_Night4`
      (set `self.AIDifficulty` 8)
      (set `self.WaitTime` (`KismetMathLibrary.RandomFloatInRange` 15.0 25.0))
      (`KismetSystemLibrary.Delay` 60.0)
      (set `self.CanMove` true)
      (`self.BeginCycle`))
    (:`LVL_Night5`
      (set `self.AIDifficulty` 12)
      (set `self.WaitTime` (`KismetMathLibrary.RandomFloatInRange` 15.0 25.0))
      (`KismetSystemLibrary.Delay` 60.0)
      (set `self.CanMove` true)
      (`self.BeginCycle`))
    (:`LVL_Night6`
      (set `self.AIDifficulty` 13)
      (set `self.WaitTime` (`KismetMathLibrary.RandomFloatInRange` 15.0 25.0))
      (`KismetSystemLibrary.Delay` 60.0)
      (set `self.CanMove` true)
      (`self.BeginCycle`))))

(event `DiningRoom`
  ;[1 1 1] Movement Action
  (if (`self.CamerasActive`)
    (`self.BeginCycle` :!label _label_4)
    (elif (`self.HoldingPosition`)
      (goto _label_4)
      (else
        (bind _output_get (set `self.ArrivalLocation` "DiningRoom"))
        (`self.CameraCheck`)
        (set `self.CurrentLocation` _output_get)
        (`self.MoveTrigger`)))))

(event `Bathroom`
  ;[1 1 1] Movement Action
  (if (`self.CamerasActive`)
    (`self.BeginCycle` :!label _label_5)
    (elif (`self.HoldingPosition`)
      (goto _label_5)
      (else
        (bind _output_get (set `self.ArrivalLocation` "Bathroom"))
        (`self.CameraCheck`)
        (set `self.CurrentLocation` _output_get)
        (`self.MoveTrigger`)))))

(event `Kitchen`
  ;[1 1 1] Movement Action
  (if (`self.CamerasActive`)
    (`self.BeginCycle` :!label _label_6)
    (else
      (bind _returnvalue (`GameplayStatics.GetActorOfClass` "/Game/Core/Assets/Characters/Chica/Blueprint/ChicaBP.ChicaBP_C"))
      (if (`KismetStringLibrary.EqualEqual_StrStr` (`/Game/Core/Assets/Characters/Chica/Blueprint/ChicaBP.CurrentLocation` _returnvalue) "Kitchen")
        (set `self.HoldingPosition` true)
        (else
          (set `self.HoldingPosition` false)))
      (if (`self.HoldingPosition`)
        (goto _label_6)
        (else
          (bind _output_get (set `self.ArrivalLocation` "Kitchen"))
          (`self.CameraCheck`)
          (set `self.CurrentLocation` _output_get)
          (`self.MoveTrigger`))))))

(event `RightHallway`
  ;[1 1 1] Movement Action
  (if (`self.CamerasActive`)
    (`self.BeginCycle` :!label _label_7)
    (else
      (bind _returnvalue (`GameplayStatics.GetActorOfClass` "/Game/Core/Assets/Characters/Chica/Blueprint/ChicaBP.ChicaBP_C"))
      (if (`KismetStringLibrary.EqualEqual_StrStr` (`/Game/Core/Assets/Characters/Chica/Blueprint/ChicaBP.CurrentLocation` _returnvalue) "RightHallway1")
        (set `self.HoldingPosition` true)
        (else
          (set `self.HoldingPosition` false)))
      (if (`self.HoldingPosition`)
        (goto _label_7)
        (else
          (bind _output_get (set `self.ArrivalLocation` "Hallway"))
          (`self.CameraCheck`)
          (set `self.CurrentLocation` _output_get)
          (`self.MoveTrigger`))))))

(event `RightCorner`
  ;[1 1 1] Movement Action
  (if (`self.CamerasActive`)
    (`self.BeginCycle` :!label _label_8)
    (else
      (bind _returnvalue (`GameplayStatics.GetActorOfClass` "/Game/Core/Assets/Characters/Chica/Blueprint/ChicaBP.ChicaBP_C"))
      (if true
        (if (`KismetStringLibrary.EqualEqual_StrStr` (`/Game/Core/Assets/Characters/Chica/Blueprint/ChicaBP.CurrentLocation` _returnvalue) "RightCorner")
          (set `self.HoldingPosition` true)
          (else
            (set `self.HoldingPosition` false)))
        (if (`self.HoldingPosition`)
          (goto _label_8)
          (else
            (bind _output_get (set `self.ArrivalLocation` "RightCorner"))
            (`self.CameraCheck`)
            (set `self.CurrentLocation` _output_get)
            (`self.MoveTrigger`)))))))

(fn `UserConstructionScript`)