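; Foxy's staged AI for Pirate's Cove, advancing from behind the curtain through peeking and about-to-run to a run.
; A delayed loop rolls against AIDifficulty, set with wait time by night level name, and stalls while cameras are active.
; Later stages also require Bonnie to be off the left hallway, corner and door.
; PositionUpdate teleports and animates Foxy, updates BP_PiratesCove, and finally activates FoxyRunBP.
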(event `BeginCycle`
  (`KismetSystemLibrary.Delay` (`self.WaitTime`))
  (if (`self.CanMove`)
    (if (and (`self.Running`) (`self.HoldingPosition`))
      (`self.BeginCycle`)
      (elif (<= (`KismetMathLibrary.RandomIntegerInRange` 1 20) (`self.AIDifficulty`))
        (`self.CameraCheck`)
        (`KismetSystemLibrary.Delay` 0.2)
        (if (`self.CamerasActive`)
          (`self.BeginCycle`)
          (`KismetSystemLibrary.PrintString` "FOXY CAM FAIL")
          (else
            (`self.MovementCycle`)
            (`KismetSystemLibrary.PrintString` "FOXY CYCLE" true true (struct :`R` 1.0 :`G` 0.087795 :`A` 1.0))))
        (else
          (`self.BeginCycle`))))
    (else
      (`self.BeginCycle`))))

(event `MovementCycle`
  (switch `int` (`self.CurrentStage`)
    (:`0`
      (`self.Peeking`))
    (:`1`
      (`self.AboutToRun`))
    (:`2`
      (`self.Run`))))

(event `PositionUpdate`
  (`|ExecutionSequence`
    (:`then_0`
      (switch `int` (`self.CurrentStage`)
        (:`0`
          (`self.K2_TeleportTo` (0.0 0.0 500.0))
          (bind _returnvalue (`GameplayStatics.GetActorOfClass` "/Game/Core/Assets/Props/PiratesCove/Stage/BP_PiratesCove.BP_PiratesCove_C"))
          (`/Game/Core/Assets/Props/PiratesCove/Stage/BP_PiratesCove.Hidden` _returnvalue))
        (:`1`
          (`self.K2_TeleportTo` (1562.089966 -726.630798 71.740067))
          (`SkeletalMeshComponent.PlayAnimation` (`self.SkeletalMesh`) "/Game/Core/Assets/Characters/Foxy/Animations/Stage01.Stage01" true)
          (bind _returnvalue_2 (`GameplayStatics.GetActorOfClass` "/Game/Core/Assets/Props/PiratesCove/Stage/BP_PiratesCove.BP_PiratesCove_C"))
          (`/Game/Core/Assets/Props/PiratesCove/Stage/BP_PiratesCove.Peek` _returnvalue_2))
        (:`2`
          (`self.K2_TeleportTo` (1542.871704 -562.744446 20.0))
          (`SkeletalMeshComponent.PlayAnimation` (`self.SkeletalMesh`) "/Game/Core/Assets/Characters/Foxy/Animations/Stage02.Stage02" true)
          (bind _returnvalue_3 (`GameplayStatics.GetActorOfClass` "/Game/Core/Assets/Props/PiratesCove/Stage/BP_PiratesCove.BP_PiratesCove_C"))
          (`/Game/Core/Assets/Props/PiratesCove/Stage/BP_PiratesCove.AboutToRun` _returnvalue_3))
        (:`3`
          (`self.K2_TeleportTo` (0.0 0.0 500.0))
          (bind _returnvalue_4 (`GameplayStatics.GetActorOfClass` "/Game/Core/Assets/Props/PiratesCove/Stage/BP_PiratesCove.BP_PiratesCove_C"))
          (`/Game/Core/Assets/Props/PiratesCove/Stage/BP_PiratesCove.Run` _returnvalue_4)
          (bind _returnvalue_5 (`GameplayStatics.GetActorOfClass` "/Game/Core/Assets/Characters/Foxy/Blueprint/FoxyRunBP.FoxyRunBP_C"))
          (`/Game/Core/Assets/Characters/Foxy/Blueprint/FoxyRunBP.Activate` _returnvalue_5)
          (set `self.Running` true))))
    (:`then_1`
      (`KismetSystemLibrary.Delay` 3.0)
      (`self.BeginCycle`))))

(event `BehindCurtain`
  (`self.CameraCheck`)
  (if (`self.CamerasActive`)
    (`self.BeginCycle`)
    (else
      (bind _output_get (set `self.ArrivalStage` 0))
      (set `self.CurrentStage` _output_get)
      (`self.PositionUpdate`))))

(event `Peeking`
  (`self.CameraCheck`)
  (if (`self.CamerasActive`)
    (`self.BeginCycle`)
    (else
      (bind _output_get (set `self.ArrivalStage` 1))
      (set `self.CurrentStage` _output_get)
      (`self.PositionUpdate`))))

(event `AboutToRun`
  (`self.CameraCheck`)
  (if (`self.CamerasActive`)
    (`self.BeginCycle` :!label _label)
    (else
      (bind _returnvalue (`GameplayStatics.GetActorOfClass` "/Game/Core/Assets/Characters/Bonnie/Blueprint/BonnieBP.BonnieBP_C"))
      (bind _currentlocation (`/Game/Core/Assets/Characters/Bonnie/Blueprint/BonnieBP.CurrentLocation` _returnvalue))
      (if (or (`KismetStringLibrary.EqualEqual_StrStr` _currentlocation "LeftHallway") (`KismetStringLibrary.EqualEqual_StrStr` _currentlocation "LeftCorner") (`KismetStringLibrary.EqualEqual_StrStr` _currentlocation "LeftDoor"))
        (goto _label)
        (elif (`self.CamerasActive`)
          (goto _label)
          (else
            (bind _output_get (set `self.ArrivalStage` 2))
            (set `self.CurrentStage` _output_get)
            (`self.PositionUpdate`)))))))

(event `self.ReceiveBeginPlay`
  (`self.Difficulty Define`))

(event `Run`
  (`self.CameraCheck`)
  (if (not (`self.CamerasActive`))
    (bind _returnvalue (`GameplayStatics.GetActorOfClass` "/Game/Core/Assets/Characters/Bonnie/Blueprint/BonnieBP.BonnieBP_C"))
    (bind _currentlocation (`/Game/Core/Assets/Characters/Bonnie/Blueprint/BonnieBP.CurrentLocation` _returnvalue))
    (if (or (`KismetStringLibrary.EqualEqual_StrStr` _currentlocation "LeftHallway") (`KismetStringLibrary.EqualEqual_StrStr` _currentlocation "LeftCorner") (`KismetStringLibrary.EqualEqual_StrStr` _currentlocation "LeftDoor"))
      (`self.BeginCycle` :!label _label_2)
      (elif (`self.CamerasActive`)
        (goto _label_2)
        (else
          (bind _output_get (set `self.ArrivalStage` 3))
          (set `self.CurrentStage` _output_get)
          (`self.PositionUpdate`))))))

(event `Difficulty Define`
  ;[1 1 1] Difficulty
  (bind _returnvalue (`GameplayStatics.GetCurrentLevelName` true))
  (switch `string` _returnvalue
    (:`LVL_NightTemplate`
      (set `self.AIDifficulty` 20)
      (set `self.WaitTime` (`KismetMathLibrary.RandomFloatInRange` 1.0 3.0))
      (`KismetSystemLibrary.Delay` 0.0)
      (set `self.CanMove` true)
      (`self.BeginCycle`))
    (:`LVL_Night1`
      (set `self.AIDifficulty` 0)
      (set `self.WaitTime` (`KismetMathLibrary.RandomFloatInRange` 20.0 30.0))
      (`KismetSystemLibrary.Delay` 60.0)
      (set `self.CanMove` true)
      (`self.BeginCycle`))
    (:`LVL_Night2`
      (set `self.AIDifficulty` 5)
      (set `self.WaitTime` (`KismetMathLibrary.RandomFloatInRange` 15.0 25.0))
      (`KismetSystemLibrary.Delay` 60.0)
      (set `self.CanMove` true)
      (`self.BeginCycle`))
    (:`LVL_Night3`
      (set `self.AIDifficulty` 5)
      (set `self.WaitTime` (`KismetMathLibrary.RandomFloatInRange` 15.0 25.0))
      (`KismetSystemLibrary.Delay` 60.0)
      (set `self.CanMove` true)
      (`self.BeginCycle`))
    (:`LVL_Night4`
      (set `self.AIDifficulty` 8)
      (set `self.WaitTime` (`KismetMathLibrary.RandomFloatInRange` 15.0 25.0))
      (`KismetSystemLibrary.Delay` 60.0)
      (set `self.CanMove` true)
      (`self.BeginCycle`))
    (:`LVL_Night5`
      (set `self.AIDifficulty` 12)
      (set `self.WaitTime` (`KismetMathLibrary.RandomFloatInRange` 15.0 25.0))
      (`KismetSystemLibrary.Delay` 60.0)
      (set `self.CanMove` true)
      (`self.BeginCycle`))
    (:`LVL_Night6`
      (set `self.AIDifficulty` 13)
      (set `self.WaitTime` (`KismetMathLibrary.RandomFloatInRange` 15.0 25.0))
      (`KismetSystemLibrary.Delay` 60.0)
      (set `self.CanMove` true)
      (`self.BeginCycle`))))

(fn `UserConstructionScript`)