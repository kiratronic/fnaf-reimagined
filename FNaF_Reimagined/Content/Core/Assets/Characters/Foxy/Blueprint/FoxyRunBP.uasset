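; Foxy's run attack Blueprint, handling the dash from activation to jumpscare or failure.
; Activate teleports Foxy into position, waits, then fires a DoOnce-gated Run that starts an AI MoveTo alongside timed branches.
; Arrival triggers FoxyStageBP's jumpscare; otherwise a timeout teleports Foxy away, resets its stage, drains Power randomly and plays a door-fail sound.
; Another timed branch signals light-off and run end, and calls Hidden on Pirates Cove.
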(event `Activate`
  ;[1 1 1] Running Prep
  (`self.ResetDoOnce`)
  (if (`self.CanRun`)
    (`self.K2_TeleportTo` (1101.967529 -307.270508 157.512436) (struct :`Yaw` -180.0))
    (set `self.WaitingForCamera` true)
    (`KismetSystemLibrary.Delay` (`self.WaitTime`))
    (set `self.WaitingForCamera` false)
    (`self.Run`)))

(event `Run`
  ;[1 1 1] Running Logic
  (`/Engine/EditorBlueprintResources/StandardMacros.DoOnce` false :!label _label
    (:`Completed`
      (if (`self.CanRun`)
        (`KismetSystemLibrary.PrintString` "RUN RUN RUN")
        (`|ExecutionSequence`
          (:`then_0`
            (`|AIMoveTo` self (-326.520538 -307.270508 157.512405) null 25.0
              (:`then`
                (`self.RunStart`))
              (:`OnSuccess`
                (`self.FoxySucceed`)
                (set `self.FoxSucceed` true)
                (bind _returnvalue (`GameplayStatics.GetActorOfClass` "/Game/Core/Assets/Characters/Foxy/Blueprint/FoxyStageBP.FoxyStageBP_C"))
                (`/Game/Core/Assets/Characters/Foxy/Blueprint/FoxyStageBP.Jumpscare` _returnvalue)
                (`self.FoxySucceed`))))
          (:`then_1`
            (`KismetSystemLibrary.Delay` 2.85)
            (if (not (`self.FoxSucceed`))
              (`/Engine/EditorBlueprintResources/StandardMacros.DoOnce` false :!label _label_2
                (:`Completed`
                  (`KismetSystemLibrary.PrintString` "FAILURE \n" true true (struct :`G` 1.0 :`B` 0.104809 :`A` 1.0))
                  (`self.K2_TeleportTo` (1559.667725 -825.927979 567.512573))
                  (bind _returnvalue_2 (`GameplayStatics.GetActorOfClass` "/Game/Core/Assets/Characters/Foxy/Blueprint/FoxyStageBP.FoxyStageBP_C"))
                  (set `/Game/Core/Assets/Characters/Foxy/Blueprint/FoxyStageBP.Running` false _returnvalue_2)
                  (set `/Game/Core/Assets/Characters/Foxy/Blueprint/FoxyStageBP.CurrentStage` 0 _returnvalue_2)
                  (`/Game/Core/Assets/Characters/Foxy/Blueprint/FoxyStageBP.PositionUpdate` _returnvalue_2)
                  (bind _returnvalue_3 (`GameplayStatics.GetActorOfClass` "/Game/Core/Assets/Interactables/Power.Power_C"))
                  (set `/Game/Core/Assets/Interactables/Power.Power` (- (`/Game/Core/Assets/Interactables/Power.Power` _returnvalue_3) (`KismetMathLibrary.RandomIntegerInRange` 1 3)) _returnvalue_3)
                  (set `/Game/Core/Assets/Interactables/Power.Power` (- (`/Game/Core/Assets/Interactables/Power.Power` _returnvalue_3) (`KismetMathLibrary.RandomIntegerInRange` 1 3)) _returnvalue_3)
                  (set `/Game/Core/Assets/Interactables/Power.Power` (- (`/Game/Core/Assets/Interactables/Power.Power` _returnvalue_3) (`KismetMathLibrary.RandomIntegerInRange` 1 3)) _returnvalue_3)
                  (`GameplayStatics.PlaySound2D` "/Game/Core/Assets/Characters/Foxy/Sounds/FoxyDoorFail_Cue.FoxyDoorFail_Cue" 5.0 1.0 0.0 null null)))))
          (:`then_2`
            (`KismetSystemLibrary.Delay` 2.0)
            (`self.FoxyLightOff`)
            (bind _returnvalue_4 (`GameplayStatics.GetActorOfClass` "/Game/Core/Assets/Props/PiratesCove/Stage/BP_PiratesCove.BP_PiratesCove_C"))
            (`/Game/Core/Assets/Props/PiratesCove/Stage/BP_PiratesCove.Hidden` _returnvalue_4)
            (`self.RunEnd`)))))))

(event `CanRunAgain`
  ;[1 1 1] Running Logic
  (goto _label :!via `Reset`))

(event `ResetDoOnce`
  ;[1 1 1] Running Logic
  (goto _label_2 :!via `Reset`))

(fn `UserConstructionScript`)