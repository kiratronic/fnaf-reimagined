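; Chica animatronic actor that wanders from the stage through the restaurant toward the office's right door, with office-entry and jumpscare poses.
; Level name sets AI difficulty and wait time; timed random rolls against difficulty pick location-specific moves.
; Room events hold position when FreddyBP blocks certain spots, otherwise blur cameras, then teleport and pose via MoveTrigger.
; Tick-polled DoorSequence and movement from the door check door state for office entry.
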(event `Door Sequence`
  (if (`self.AtDoor`)
    (if (`self.RightDoorClosed`)
      (`KismetSystemLibrary.Delay` 0.05)
      (if (not (`self.RightDoorClosed`))
        (`KismetSystemLibrary.Delay` 1.0)
        (if (not (`self.RightDoorClosed`)) :!label _label
          (set `self.InOffice` true)
          (`self.InOfficeLogic`)
          (`KismetSystemLibrary.PrintString` "InOffice")))
      (elif (`self.LightOn`)
        (`KismetSystemLibrary.Delay` 3.0)
        (goto _label)))))

(event `BeginCycle`
  ;[1 1 1] Movement Chance
  (`KismetSystemLibrary.Delay` (`self.WaitTime`))
  (if (`self.CanMove`)
    (if (and (`self.InOffice`) (`self.HoldingPosition`))
      (`self.BeginCycle`)
      (elif (<= (`KismetMathLibrary.RandomIntegerInRange` 0 20) (`self.AIDifficulty`))
        (`self.MovementCycle`)
        (else
          (`self.BeginCycle`))))
    (else
      (`self.BeginCycle`))))

(event `StageMove`
  ;[1 1 1] Teleport And Animation
  (`self.K2_TeleportTo` (2978.659912 182.705856 90.0) (struct :`Yaw` 104.400002) :!label _label_2)
  (`SkeletalMeshComponent.PlayAnimation` (`self.SkeletalMesh`) "/Game/Core/Assets/Characters/Chica/Animations/chica_pose.chica_pose" true))

(event `InOfficeLogic`
  (bind _skeletalmesh (`self.SkeletalMesh`))
  (`self.ChicaInOffice`)
  (`self.K2_TeleportTo` (-357.035309 -10.0 20.0) (struct :`Yaw` -90.0))
  (`SkeletalMeshComponent.PlayAnimation` _skeletalmesh "/Game/Core/Assets/Characters/Chica/Animations/ChicaPreJumpscare.ChicaPreJumpscare" true)
  (`PrimitiveComponent.SetMaterial` _skeletalmesh 1 "/Game/Core/Assets/Characters/Shared/Material/EmmissiveEye_MI.EmmissiveEye_MI")
  (`KismetSystemLibrary.PrintString` "InOffice"))

(event `self.ReceiveBeginPlay`
  (`self.StageMove`)
  (`self.Difficulty Define`))

(event `self.ReceiveTick`
  (params (DeltaSeconds :type "Float (single-precision)"))
  (`self.Door Sequence`))

(event `Jumpscare`
  (`self.ChicaJumpscare`)
  (`SkeletalMeshComponent.PlayAnimation` (`self.SkeletalMesh`) "/Game/Core/Assets/Characters/Chica/Animations/chica_jumpscare_1.chica_jumpscare_1" true)
  (`SceneComponent.SetVisibility` (`self.PointLight`) true false))

(event `MoveTrigger`
  (bind _arrivallocation (`self.ArrivalLocation`))
  ;[1 1 1] Teleport And Animation
  (`KismetSystemLibrary.PrintString` _arrivallocation true true (struct :`G` 0.919115 :`B` 1.0 :`A` 1.0))
  (`|ExecutionSequence`
    (:`then_0`
      (switch `string` (`self.ArrivalLocation`)
        (:`Stage`
          (goto _label_2))
        (:`Dining1`
          (`self.K2_TeleportTo` (2510.675049 93.131943 55.0) (struct :`Yaw` -160.0))
          (`SkeletalMeshComponent.PlayAnimation` (`self.SkeletalMesh`) "/Game/Core/Assets/Characters/Chica/Animations/chica_pose.chica_pose" true))
        (:`Dining2`
          (`self.K2_TeleportTo` (1898.229492 210.247925 20.0) (struct :`Yaw` -170.0))
          (`SkeletalMeshComponent.PlayAnimation` (`self.SkeletalMesh`) "/Game/Core/Assets/Characters/Chica/Animations/ChicaDining2.ChicaDining2" true))
        (:`Bathroom1`
          (`self.K2_TeleportTo` (2158.252441 1008.845764 19.713142) (struct :`Yaw` -85.0))
          (`SkeletalMeshComponent.PlayAnimation` (`self.SkeletalMesh`) "/Game/Core/Assets/Characters/Chica/Animations/ChicaBathroom1v2.ChicaBathroom1v2" true))
        (:`Bathroom2`
          (`self.K2_TeleportTo` (2558.10376 993.032776 34.315838) (struct :`Yaw` -115.0))
          (`SkeletalMeshComponent.PlayAnimation` (`self.SkeletalMesh`) "/Game/Core/Assets/Characters/Chica/Animations/ChicaBathroom2.ChicaBathroom2" true))
        (:`Kitchen`
          (`self.K2_TeleportTo` (0.0 0.0 500.0))
          (`SkeletalMeshComponent.PlayAnimation` (`self.SkeletalMesh`) null true))
        (:`RightHallway1`
          (`self.K2_TeleportTo` (782.735107 314.217865 20.0) (struct :`Yaw` 90.0))
          (`SkeletalMeshComponent.PlayAnimation` (`self.SkeletalMesh`) "/Game/Core/Assets/Characters/Chica/Animations/ChicaHallway1.ChicaHallway1" true))
        (:`RightHallway2`
          (`self.K2_TeleportTo` (229.623734 302.277496 20.0) (struct :`Yaw` 104.91095))
          (`SkeletalMeshComponent.PlayAnimation` (`self.SkeletalMesh`) "/Game/Core/Assets/Characters/Chica/Animations/ChicaHallway2.ChicaHallway2" true))
        (:`RightCorner`
          (`self.K2_TeleportTo` (-521.838684 266.745026 25.5966) (struct :`Yaw` -58.599998))
          (`SkeletalMeshComponent.PlayAnimation` (`self.SkeletalMesh`) "/Game/Core/Assets/Characters/Chica/Animations/ANIM_RightHallCorner.ANIM_RightHallCorner" true))
        (:`RightDoor`
          (`self.K2_TeleportTo` (-48.774742 222.027725 0.0) (struct :`Yaw` -207.244293))
          (`SkeletalMeshComponent.PlayAnimation` (`self.SkeletalMesh`) "/Game/Core/Assets/Characters/Chica/Animations/ChicaDoor.ChicaDoor" true))))
    (:`then_1`
      (if (`KismetStringLibrary.EqualEqual_StrStr` _arrivallocation "LeftDoor")
        (`self.Door Sequence`)
        (`self.BeginCycle`)
        (else
          (`self.BeginCycle`)
          (set `self.AtDoor` false))))))

(event `JumpscareCall`
  (`SkeletalMeshComponent.PlayAnimation` (`self.SkeletalMesh`) "/Game/Core/Assets/Characters/Chica/Animations/chica_jumpscare_1.chica_jumpscare_1" true)
  (`SceneComponent.SetVisibility` (`self.PointLight`) true false))

(event `TryAgain`
  (bind _returnvalue (`KismetMathLibrary.RandomIntegerInRange` 0 3))
  (bind _returnvalue_2 (!= _returnvalue (`self.RNGMove`)))
  ;[1 1 1] Random Movement
  (switch `string` (`self.CurrentLocation`) :!label _label_3
    (:`Stage`
      (switch `int` _returnvalue :!label _label_4
        (:`0`
          (if _returnvalue_2
            (`self.Bathroom1`)
            (set `self.RNGMove` 0)
            (else
              (`KismetSystemLibrary.PrintString` "ChicaTryAgain" true true (struct :`R` 1.0 :`G` 0.133929 :`A` 1.0) :!label _label_5)
              (goto _label_4))))
        (:`1`
          (if _returnvalue_2
            (`self.Dining1`)
            (set `self.RNGMove` 1)
            (else
              (goto _label_5))))
        (:`2`
          (if _returnvalue_2
            (`self.Bathroom2`)
            (set `self.RNGMove` 2)
            (else
              (goto _label_5))))
        (:`3`
          (if _returnvalue_2
            (`self.Dining2`)
            (set `self.RNGMove` 3)
            (else
              (goto _label_5))))))
    (:`Dining1`
      (if (`KismetMathLibrary.RandomBool`)
        (goto _label_4)
        (elif (> (`KismetMathLibrary.RandomIntegerInRange` 0 20) (`self.AIDifficulty`))
          (`self.Dining2`)
          (else
            (`self.Bathroom1`)))))
    (:`Dining2`
      (if (> (`KismetMathLibrary.RandomIntegerInRange` 0 20) (`self.AIDifficulty`))
        (goto _label_4)
        (elif (`KismetMathLibrary.RandomBool`)
          (`self.Kitchen`)
          (else
            (`self.RightHallway1`)))))
    (:`Bathroom1`
      (if (> (`KismetMathLibrary.RandomIntegerInRange` 0 20) (`self.AIDifficulty`))
        (goto _label_4)
        (elif (`KismetMathLibrary.RandomBool`)
          (`self.Bathroom2`)
          (else
            (`self.Dining2`)))))
    (:`Bathroom2`
      (if (`KismetMathLibrary.RandomBool`)
        (`self.Kitchen`)
        (else
          (`self.Dining2`))))
    (:`Kitchen`
      (if (> (`KismetMathLibrary.RandomIntegerInRange` 0 20) (`self.AIDifficulty`))
        (`self.Dining2`)
        (elif (`KismetMathLibrary.RandomBool`)
          (`self.RightHallway1`)
          (else
            (`self.RightHallway2`)))))
    (:`RightHallway1`
      (if (> (`KismetMathLibrary.RandomIntegerInRange` 0 20) (`self.AIDifficulty`))
        (`self.Dining2`)
        (elif (`KismetMathLibrary.RandomBool`)
          (`self.RightHallway2`)
          (else
            (`self.RightCorner`)))))
    (:`RightHallway2`
      (if (> (`KismetMathLibrary.RandomIntegerInRange` 0 20) (`self.AIDifficulty`))
        (`self.Kitchen`)
        (else
          (`self.RightCorner`))))
    (:`RightCorner`
      (if (> (`KismetMathLibrary.RandomIntegerInRange` 0 20) (`self.AIDifficulty`))
        (`self.RightHallway1`)
        (else
          (`self.RightDoor`))))
    (:`RightDoor`
      (if (`self.RightDoorClosed`)
        (if (`KismetMathLibrary.RandomBool`)
          (`self.Dining1`)
          (elif (`KismetMathLibrary.RandomBool`)
            (`self.Dining2`)
            (else
              (`self.RightHallway2`))))
        (`self.ChicaFromDoor`)
        (else
          (set `self.InOffice` true)
          (`self.InOfficeLogic`))))))

(event `MovementCycle`
  ;[1 1 1] Random Movement
  (goto _label_3))

(event `Dining1`
  ;[1 1 1] MovementAction
  (if (`self.HoldingPosition`)
    (`self.BeginCycle`)
    (else
      (bind _output_get (set `self.ArrivalLocation` "Dining1"))
      (`self.CameraBlur`)
      (set `self.CurrentLocation` _output_get)
      (`self.MoveTrigger`))))

(event `Difficulty Define`
  ;[1 1 1] Difficulty
  (bind _returnvalue (`GameplayStatics.GetCurrentLevelName` true))
  (switch `string` _returnvalue
    (:`LVL_NightTemplate`
      (set `self.AIDifficulty` 2)
      (set `self.WaitTime` (`KismetMathLibrary.RandomFloatInRange` 15.0 25.0))
      (`KismetSystemLibrary.Delay` 60.0)
      (set `self.CanMove` true)
      (`self.BeginCycle`))
    (:`LVL_Night2`
      (set `self.AIDifficulty` 5)
      (set `self.WaitTime` (`KismetMathLibrary.RandomFloatInRange` 15.0 25.0))
      (`KismetSystemLibrary.Delay` 60.0)
      (set `self.CanMove` true)
      (`self.BeginCycle`))
    (:`LVL_Night3`
      (set `self.AIDifficulty` 5)
      (set `self.WaitTime` (`KismetMathLibrary.RandomFloatInRange` 15.0 25.0))
      (`KismetSystemLibrary.Delay` 60.0)
      (set `self.CanMove` true)
      (`self.BeginCycle`))
    (:`LVL_Night4`
      (set `self.AIDifficulty` 8)
      (set `self.WaitTime` (`KismetMathLibrary.RandomFloatInRange` 15.0 25.0))
      (`KismetSystemLibrary.Delay` 60.0)
      (set `self.CanMove` true)
      (`self.BeginCycle`))
    (:`LVL_Night5`
      (set `self.AIDifficulty` 12)
      (set `self.WaitTime` (`KismetMathLibrary.RandomFloatInRange` 15.0 25.0))
      (`KismetSystemLibrary.Delay` 60.0)
      (set `self.CanMove` true)
      (`self.BeginCycle`))
    (:`LVL_Night6`
      (set `self.AIDifficulty` 13)
      (set `self.WaitTime` (`KismetMathLibrary.RandomFloatInRange` 15.0 25.0))
      (`KismetSystemLibrary.Delay` 60.0)
      (set `self.CanMove` true)
      (`self.BeginCycle`))))

(event `Dining2`
  ;[1 1 1] MovementAction
  (if (`self.HoldingPosition`)
    (`self.BeginCycle`)
    (else
      (bind _output_get (set `self.ArrivalLocation` "Dining2"))
      (`self.CameraBlur`)
      (set `self.CurrentLocation` _output_get)
      (`self.MoveTrigger`))))

(event `Bathroom1`
  ;[1 1 1] MovementAction
  (if (`self.HoldingPosition`)
    (`self.BeginCycle`)
    (else
      (bind _output_get (set `self.ArrivalLocation` "Bathroom1"))
      (`self.CameraBlur`)
      (set `self.CurrentLocation` _output_get)
      (`self.MoveTrigger`))))

(event `Bathroom2`
  ;[1 1 1] MovementAction
  (if (`self.HoldingPosition`)
    (`self.BeginCycle`)
    (else
      (bind _output_get (set `self.ArrivalLocation` "Bathroom2"))
      (`self.CameraBlur`)
      (set `self.CurrentLocation` _output_get)
      (`self.MoveTrigger`))))

(event `Kitchen`
  (bind _returnvalue (`GameplayStatics.GetActorOfClass` "/Game/Core/Assets/Characters/Freddy/Blueprint/FreddyBP.FreddyBP_C"))
  ;[1 1 1] MovementAction
  (if (`KismetStringLibrary.EqualEqual_StrStr` (`/Game/Core/Assets/Characters/Freddy/Blueprint/FreddyBP.CurrentLocation` _returnvalue) "Kitchen")
    (set `self.HoldingPosition` true)
    (else
      (set `self.HoldingPosition` false)))
  (if (`self.HoldingPosition`)
    (`self.BeginCycle`)
    (else
      (bind _output_get (set `self.ArrivalLocation` "Kitchen"))
      (`self.CameraBlur`)
      (set `self.CurrentLocation` _output_get)
      (`self.MoveTrigger`))))

(event `RightHallway1`
  (bind _returnvalue (`GameplayStatics.GetActorOfClass` "/Game/Core/Assets/Characters/Freddy/Blueprint/FreddyBP.FreddyBP_C"))
  ;[1 1 1] MovementAction
  (if (`KismetStringLibrary.EqualEqual_StrStr` (`/Game/Core/Assets/Characters/Freddy/Blueprint/FreddyBP.CurrentLocation` _returnvalue) "Hallway")
    (set `self.HoldingPosition` true)
    (else
      (set `self.HoldingPosition` false)))
  (if (`self.HoldingPosition`)
    (`self.BeginCycle`)
    (else
      (bind _output_get (set `self.ArrivalLocation` "RightHallway1"))
      (`self.CameraBlur`)
      (set `self.CurrentLocation` _output_get)
      (`self.MoveTrigger`))))

(event `RightHallway2`
  ;[1 1 1] MovementAction
  (if (`self.HoldingPosition`)
    (`self.BeginCycle`)
    (else
      (bind _output_get (set `self.ArrivalLocation` "RightHallway2"))
      (`self.CameraBlur`)
      (set `self.CurrentLocation` _output_get)
      (`self.MoveTrigger`))))

(event `RightCorner`
  (bind _returnvalue (`GameplayStatics.GetActorOfClass` "/Game/Core/Assets/Characters/Freddy/Blueprint/FreddyBP.FreddyBP_C"))
  ;[1 1 1] MovementAction
  (if (`KismetStringLibrary.EqualEqual_StrStr` (`/Game/Core/Assets/Characters/Freddy/Blueprint/FreddyBP.CurrentLocation` _returnvalue) "RightCorner")
    (set `self.HoldingPosition` true)
    (else
      (set `self.HoldingPosition` false)))
  (if (`self.HoldingPosition`)
    (`self.BeginCycle`)
    (else
      (bind _output_get (set `self.ArrivalLocation` "RightCorner"))
      (`self.CameraBlur`)
      (set `self.CurrentLocation` _output_get)
      (`self.MoveTrigger`))))

(event `RightDoor`
  (bind _returnvalue (`GameplayStatics.GetActorOfClass` "/Game/Core/Assets/Characters/Freddy/Blueprint/FreddyBP.FreddyBP_C"))
  ;[1 1 1] MovementAction
  (if (`KismetStringLibrary.EqualEqual_StrStr` (`/Game/Core/Assets/Characters/Freddy/Blueprint/FreddyBP.CurrentLocation` _returnvalue) "Corner")
    (set `self.HoldingPosition` true)
    (else
      (set `self.HoldingPosition` false)))
  (if (`self.HoldingPosition`)
    (`self.BeginCycle`)
    (else
      (`self.ChicaToDoor`)
      (bind _output_get (set `self.ArrivalLocation` "RightDoor"))
      (`self.CameraBlur`)
      (set `self.CurrentLocation` _output_get)
      (`self.MoveTrigger`)
      (set `self.AtDoor` true))))

(fn `UserConstructionScript`)