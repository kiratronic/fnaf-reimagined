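; Door button Blueprint that controls a left or right door and its light, chosen by the Door variable.
; Open, close and light events fire side-specific calls, swap materials or dynamic emissive, and toggle the light's audio.
; A closed door or active light each adds one to the Usage actor, which is then updated.
; CharacterDisable locks interaction and kills the lights without adjusting Usage, while Powerout blacks out the button materials.
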(event `DoorOpen`
  (if (`self.CanInteract`)
    (`PrimitiveComponent.SetMaterial` (`self.StaticMesh`) 2 "/Game/Core/Assets/Props/DoorButtons/MI_DoorLightOpen.MI_DoorLightOpen")
    (switch `int` (`self.Door`)
      (:`0`
        (`self.LeftDoorOpen`))
      (:`1`
        (`self.RightDoorOpen`)))
    (bind _returnvalue (`GameplayStatics.GetActorOfClass` "/Game/Core/Assets/Interactables/Usage.Usage_C"))
    (set `/Game/Core/Assets/Interactables/Usage.Usage` (- (`/Game/Core/Assets/Interactables/Usage.Usage` _returnvalue) 1) _returnvalue)
    (`/Game/Core/Assets/Interactables/Usage.Update` _returnvalue)
    (set `self.DoorClosed` false)))

(event `DoorClose`
  (if (`self.CanInteract`)
    (`PrimitiveComponent.SetMaterial` (`self.StaticMesh`) 2 "/Game/Core/Assets/Props/DoorButtons/MI_DoorLightClosed.MI_DoorLightClosed")
    (switch `int` (`self.Door`)
      (:`0`
        (`self.LeftDoorClosed`))
      (:`1`
        (`self.RightDoorClosed`)))
    (bind _returnvalue (`GameplayStatics.GetActorOfClass` "/Game/Core/Assets/Interactables/Usage.Usage_C"))
    (set `/Game/Core/Assets/Interactables/Usage.Usage` (+ (`/Game/Core/Assets/Interactables/Usage.Usage` _returnvalue) 1) _returnvalue)
    (`/Game/Core/Assets/Interactables/Usage.Update` _returnvalue)
    (set `self.DoorClosed` true)))

(event `self.ReceiveBeginPlay`
  (bind _returnvalue (`PrimitiveComponent.CreateDynamicMaterialInstance` (`self.StaticMesh`) 1 "/Game/Core/Assets/Props/DoorButtons/MI_LightLight.MI_LightLight" "None"))
  (`MaterialInstanceDynamic.SetScalarParameterValue` _returnvalue "Emmisive Multiplier" 0.05))

(event `LightOn`
  (if (`self.LightActive`)
    _
    (elif (`self.CanInteract`)
      (switch `int` (`self.Door`)
        (:`0`
          (`self.LightLeftOn`))
        (:`1`
          (`self.LightRightOn`)))
      (set `self.LightActive` true)
      (bind _returnvalue (`GameplayStatics.GetActorOfClass` "/Game/Core/Assets/Interactables/Usage.Usage_C"))
      (set `/Game/Core/Assets/Interactables/Usage.Usage` (+ (`/Game/Core/Assets/Interactables/Usage.Usage` _returnvalue) 1) _returnvalue)
      (`/Game/Core/Assets/Interactables/Usage.Update` _returnvalue)
      (`MaterialInstanceDynamic.SetScalarParameterValue` (stale `self.ReceiveBeginPlay` _returnvalue) "Emmisive Multiplier" 2.0)
      (`AudioComponent.Play` (`self.Audio`) 0.0))))

(event `LightOff`
  (if (`self.LightActive`)
    (if (`self.CanInteract`)
      (switch `int` (`self.Door`)
        (:`0`
          (`self.LightLeftOff`))
        (:`1`
          (`self.LightRightOff`)))
      (set `self.LightActive` false)
      (bind _returnvalue (`GameplayStatics.GetActorOfClass` "/Game/Core/Assets/Interactables/Usage.Usage_C"))
      (set `/Game/Core/Assets/Interactables/Usage.Usage` (- (`/Game/Core/Assets/Interactables/Usage.Usage` _returnvalue) 1) _returnvalue)
      (`/Game/Core/Assets/Interactables/Usage.Update` _returnvalue)
      (`MaterialInstanceDynamic.SetScalarParameterValue` (stale `self.ReceiveBeginPlay` _returnvalue) "Emmisive Multiplier" 0.05)
      (`AudioComponent.Stop` (`self.Audio`) :!label _label))))

(event `CharacterDisable`
  (set `self.CanInteract` false)
  (`self.LightLeftOff`)
  (`self.LightRightOff`)
  (set `self.LightActive` false)
  (`MaterialInstanceDynamic.SetScalarParameterValue` (stale `self.ReceiveBeginPlay` _returnvalue) "Emmisive Multiplier" 0.05)
  (goto _label))

(event `Powerout`
  (`PrimitiveComponent.SetMaterial` (`self.StaticMesh`) 1 "/Game/Core/Assets/Props/Pizzas/Pizza02/Black.Black")
  (`PrimitiveComponent.SetMaterial` (`self.StaticMesh`) 2 "/Game/Core/Assets/Props/Pizzas/Pizza02/Black.Black"))

(fn `UserConstructionScript`)