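; Hydraulic door prop that slides vertically through Open and Close events.
; Close plays the CloseDoor timeline forward to drive the door's relative Z, and Open reverses it; both play the same 2D sound.
; A FlipFlop on timeline completion triggers a player camera shake on alternate finishes, starting with the first.
; Two DoOnce sound-cooldown chains are left unconnected.
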(event `Close`
  (`GameplayStatics.PlaySound2D` "/Game/Core/Assets/Sound/Door_Close__2_.Door_Close__2_" 1.0 1.0 0.0 null null)
  (bind (_direction _location) (`Timeline|CloseDoor` :!via `PlayFromStart` :!label _label)
    (:`Update`
      (`SceneComponent.K2_SetRelativeLocation` (`self.Door`) (`KismetMathLibrary.MakeVector` 0.0 0.0 (.z _location)) false false))
    (:`Finished`
      (`/Engine/EditorBlueprintResources/StandardMacros.FlipFlop`
        (:`A`
          (`PlayerCameraManager.StartCameraShake` :`self` (`GameplayStatics.GetPlayerCameraManager` 0) :`ShakeClass` "/Game/Core/Player/CameraShake/DoorCameraShakeBP.DoorCameraShakeBP_C"))))))

(event `Open`
  (`GameplayStatics.PlaySound2D` "/Game/Core/Assets/Sound/Door_Close__2_.Door_Close__2_" 1.0 1.0 0.0 null null)
  (goto _label :!via `Reverse`))

(fn `UserConstructionScript`)