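; BP_PiratesCove is the Pirate's Cove stage prop whose two curtains show escalating stages: Hidden, Peek, AboutToRun and Run.
; Each stage is a custom event that instantly snaps both curtain meshes to hardcoded relative rotations, with no interpolation.
; BeginPlay starts it in Hidden; nothing in this Blueprint triggers the other stages.
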(event `self.ReceiveBeginPlay`
  (`self.Hidden`))

(event `Hidden`
  (`SceneComponent.K2_SetRelativeRotation` (`self.SM_PiratesCove_Curtains_Curtain_001`) (struct :`Yaw` 13.589349) false false)
  (`SceneComponent.K2_SetRelativeRotation` (`self.SM_PiratesCove_Curtains_Curtain`) (struct :`Yaw` -11.8) false false))

(event `Peek`
  (`SceneComponent.K2_SetRelativeRotation` (`self.SM_PiratesCove_Curtains_Curtain_001`) (struct :`Yaw` -0.3) false false)
  (`SceneComponent.K2_SetRelativeRotation` (`self.SM_PiratesCove_Curtains_Curtain`) (struct :`Yaw` -15.0) false false))

(event `AboutToRun`
  (`SceneComponent.K2_SetRelativeRotation` (`self.SM_PiratesCove_Curtains_Curtain_001`) (struct :`Yaw` -15.3) false false)
  (`SceneComponent.K2_SetRelativeRotation` (`self.SM_PiratesCove_Curtains_Curtain`) (struct :`Yaw` -0.6) false false))

(event `Run`
  (`SceneComponent.K2_SetRelativeRotation` (`self.SM_PiratesCove_Curtains_Curtain_001`) (struct :`Yaw` -19.5) false false)
  (`SceneComponent.K2_SetRelativeRotation` (`self.SM_PiratesCove_Curtains_Curtain`) (struct :`Yaw` 4.1) false false))

(fn `UserConstructionScript`)