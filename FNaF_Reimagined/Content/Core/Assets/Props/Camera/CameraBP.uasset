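; CameraBP is a security camera prop that can sweep back and forth and shows blur glitches on its view.
; A timeline yaws the sphere when rotary, pausing at each end before flipping direction.
; Glitch events briefly swap the main camera for a blur camera with sound: a long garble only while the player's monitor is up, or a short blip.
; The construction script applies per-instance height, pitch and FOV.
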(event `self.ReceiveBeginPlay`
  (if (`self.IsRotary`)
    (bind (_direction _rotation) (`Timeline|CameraMovement` :!label _label)
      (:`Update`
        (`SceneComponent.K2_SetRelativeRotation` (`self.Sphere`) (`KismetMathLibrary.MakeRotator` 0.0 0.0 _rotation) false false))
      (:`Finished`
        (`KismetSystemLibrary.Delay` 2.0)
        (`/Engine/EditorBlueprintResources/StandardMacros.FlipFlop`
          (:`A`
            (goto _label :!via `Reverse`))
          (:`B`
            (goto _label)))))))

(event `CameraBlurEvent`
  (bind _asplayer_bp (cast `/Game/Core/Player/PlayerBP` (`GameplayStatics.GetPlayerCharacter` 0)))
  (if (`/Game/Core/Player/PlayerBP.MonitorUp` _asplayer_bp)
    (`/Engine/EditorBlueprintResources/StandardMacros.DoOnce` false :!label _label_2
      (:`Completed`
        (set `self.IsBlurEvent` true)
        (`GameplayStatics.PlaySound2D` "/Game/Core/Assets/Sounds/Garble_Cue.Garble_Cue" 1.0 1.0 0.0 null self)
        (`ActorComponent.Deactivate` (`self.Camera`))
        (`ActorComponent.Activate` (`self.BlurCamera`) false)
        (`KismetSystemLibrary.Delay` 4.0)
        (`ActorComponent.Deactivate` (`self.BlurCamera`))
        (`ActorComponent.Activate` (`self.Camera`) false)
        (`self.GarbleReset`)))))

(event `GarbleReset`
  (set `self.IsBlurEvent` false)
  (goto _label_2 :!via `Reset`))

(event `ShortBlur`
  (if (not (`self.IsBlurEvent`))
    (`/Engine/EditorBlueprintResources/StandardMacros.DoOnce` false :!label _label_3
      (:`Completed`
        (`|ExecutionSequence`
          (:`then_0`
            (`GameplayStatics.PlaySound2D` "/Game/Core/Assets/Sounds/Blip_Cue.Blip_Cue" 1.0 1.0 0.0 null null)
            (`ActorComponent.Deactivate` (`self.Camera`))
            (`ActorComponent.Activate` (`self.BlurCamera`) false)
            (`KismetSystemLibrary.Delay` 0.15)
            (`ActorComponent.Deactivate` (`self.BlurCamera`))
            (`ActorComponent.Activate` (`self.Camera`) false))
          (:`then_1`
            (`KismetSystemLibrary.Delay` 0.2)
            (`self.BlipReset`)))))))

(event `BlipReset`
  (goto _label_3 :!via `Reset`))

(fn `UserConstructionScript`
  (`SceneComponent.K2_SetRelativeLocation` (`self.Camera`) (`KismetMathLibrary.MakeVector` 0.0 0.0 (`self.Z-Drop`)) false false)
  (`SceneComponent.K2_SetRelativeRotation` (`self.Camera`) (`KismetMathLibrary.MakeRotator` 0.0 (`self.Pitch`)) false false)
  (`CameraComponent.SetFieldOfView` (`self.Camera`) (`self.FOV`))
  (`CameraComponent.SetFieldOfView` (`self.BlurCamera`) (`self.FOV`)))