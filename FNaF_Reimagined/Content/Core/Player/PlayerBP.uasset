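; Player Blueprint for a Five Nights at Freddy's-style game, handling limited look, office interaction and the camera monitor.
; Interact line-traces to door and light buttons or a honking poster, with resettable DoOnce gates throttling repeats.
; A Space-toggled timeline moves the monitor, swaps the player UI and updates power usage.
; Looping timers drive trace-based autofocus and idle or spooked camera shake, while events handle spooks, power loss and imminent jumpscares.
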(event `0Off`
  (if (stale _isa)
    (bind _isa (`/Engine/EditorBlueprintResources/StandardMacros.FlipFlop` :!label _label)
      (:`A`
        (`/Game/Core/Assets/Interactables/DoorButtonBP.LightOn` (stale `InputAction|Interact` _asdoor_button_bp)))
      (:`B`
        (if (== (`/Game/Core/Assets/Interactables/DoorButtonBP.Door` (stale `InputAction|Interact` _asdoor_button_bp)) 0)
          (`/Game/Core/Assets/Interactables/DoorButtonBP.LightOff` (stale `InputAction|Interact` _asdoor_button_bp)))))))

(event `1Off`
  (if (stale _isa)
    (bind _isa (`/Engine/EditorBlueprintResources/StandardMacros.FlipFlop` :!label _label_2)
      (:`A`
        (`/Game/Core/Assets/Interactables/DoorButtonBP.LightOn` (stale `InputAction|Interact` _asdoor_button_bp)))
      (:`B`
        (if (== (`/Game/Core/Assets/Interactables/DoorButtonBP.Door` (stale `InputAction|Interact` _asdoor_button_bp)) 1)
          (`/Game/Core/Assets/Interactables/DoorButtonBP.LightOff` (stale `InputAction|Interact` _asdoor_button_bp)))))))

(event `LeftDoorReset`
  (goto _label_3 :!via `Reset`))

(event `RightDoorReset`
  (goto _label_4 :!via `Reset`))

(event `InputAction|Interact`
  (params (Key :type "Key Structure"))
  (bind _camera (`self.Camera`))
  (bind _returnvalue (`SceneComponent.K2_GetComponentLocation` _camera))
  (:`Pressed`
    (if (not (`self.MonitorUp`))
      (bind _outhit (`KismetSystemLibrary.LineTraceSingle` _returnvalue (+ _returnvalue (* (`SceneComponent.GetForwardVector` _camera) 250.0)) "TraceTypeQuery2"))
      (bind (_bblockinghit _binitialoverlap _time _distance _location _impactpoint _normal _impactnormal _physmat _hitactor _hitcomponent) (`GameplayStatics.BreakHitResult` _outhit))
      (bind _asdoor_button_bp (cast `/Game/Core/Assets/Interactables/DoorButtonBP` _hitactor)
        (:`then`
          (if (== (`/Game/Core/Assets/Interactables/DoorButtonBP.LightCollision` _asdoor_button_bp) _hitcomponent)
            (bind _door (`/Game/Core/Assets/Interactables/DoorButtonBP.Door` _asdoor_button_bp))
            (switch `int` _door
              (:`0`
                (goto _label))
              (:`1`
                (goto _label_2)))
            (elif (== (`/Game/Core/Assets/Interactables/DoorButtonBP.DoorCollision` _asdoor_button_bp) _hitcomponent)
              (switch `int` _door
                (:`0`
                  (`/Engine/EditorBlueprintResources/StandardMacros.DoOnce` false :!label _label_3
                    (:`Completed`
                      (`/Engine/EditorBlueprintResources/StandardMacros.FlipFlop`
                        (:`A`
                          (`/Game/Core/Assets/Interactables/DoorButtonBP.DoorClose` _asdoor_button_bp))
                        (:`B`
                          (`/Game/Core/Assets/Interactables/DoorButtonBP.DoorOpen` _asdoor_button_bp)))
                      (`KismetSystemLibrary.Delay` 1.75)
                      (`self.LeftDoorReset`))))
                (:`1`
                  (`/Engine/EditorBlueprintResources/StandardMacros.DoOnce` false :!label _label_4
                    (:`Completed`
                      (`/Engine/EditorBlueprintResources/StandardMacros.FlipFlop`
                        (:`A`
                          (`/Game/Core/Assets/Interactables/DoorButtonBP.DoorClose` _asdoor_button_bp))
                        (:`B`
                          (`/Game/Core/Assets/Interactables/DoorButtonBP.DoorOpen` _asdoor_button_bp)))
                      (`KismetSystemLibrary.Delay` 1.75)
                      (`self.RightDoorReset`))))))))
        (:`CastFailed`
          (bind _asfreddy_poster (cast `/Game/Core/Assets/Props/Posters/FreddyPoster` _hitactor))
          (if (== (`/Game/Core/Assets/Props/Posters/FreddyPoster.BoxCollision` _asfreddy_poster) _hitcomponent)
            (`/Engine/EditorBlueprintResources/StandardMacros.DoOnce` false :!label _label_5
              (:`Completed`
                (`GameplayStatics.PlaySound2D` "/Game/Core/Assets/Sounds/Honk_Cue.Honk_Cue" 1.0 1.0 0.0 null null)
                (`KismetSystemLibrary.Delay` 0.5)
                (goto _label_5 :!via `Reset`)))))))))

(event `self.ReceiveBeginPlay`
  (bind _returnvalue (`GameplayStatics.GetPlayerCameraManager` 0))
  ;[1 1 1] Player Look
  (`self.UIActivation`)
  (set `PlayerCameraManager.ViewPitchMin` -15.0 _returnvalue)
  (set `PlayerCameraManager.ViewPitchMax` 25.0 _returnvalue)
  (`KismetSystemLibrary.K2_SetTimerDelegate` (delegate `UpdateDoF`) 0.2 true)
  (`KismetSystemLibrary.K2_SetTimerDelegate` (delegate `CameraIdleShake`) 1.0 true))

(event `MonitorOn`
  (`Widget.RemoveFromParent` (stale `MonitorOff` _returnvalue))
  (`self.CamerasActive`)
  (bind _returnvalue (`GameplayStatics.GetActorOfClass` "/Game/Core/Assets/Interactables/Usage.Usage_C"))
  (set `/Game/Core/Assets/Interactables/Usage.Usage` (+ (`/Game/Core/Assets/Interactables/Usage.Usage` _returnvalue) 1) _returnvalue)
  (`/Game/Core/Assets/Interactables/Usage.Update` _returnvalue))

(event `InputAxis|LookX`
  (params (AxisValue :type "Float (single-precision)"))
  ;[1 1 1] Player Look
  (if (not (`self.MonitorUp`))
    (`self.AddControllerYawInput` AxisValue)))

(event `InputAxis|LookY`
  (params (AxisValue :type "Float (single-precision)"))
  ;[1 1 1] Player Look
  (if (not (`self.MonitorUp`))
    (`self.AddControllerPitchInput` (* AxisValue -1.0))))

(event `MonitorOff`
  (`self.CamerasInactive`)
  (bind _returnvalue (`|CreateWidget` "/Game/Core/Assets/Widgets/PlayerUI.PlayerUI_C" :!label _label_6))
  (`UserWidget.AddToViewport` _returnvalue 0)
  (bind _returnvalue_2 (`GameplayStatics.GetActorOfClass` "/Game/Core/Assets/Interactables/Usage.Usage_C"))
  (set `/Game/Core/Assets/Interactables/Usage.Usage` (- (`/Game/Core/Assets/Interactables/Usage.Usage` _returnvalue_2) 1) _returnvalue_2)
  (`/Game/Core/Assets/Interactables/Usage.Update` _returnvalue_2))

(event `UIActivation`
  (goto _label_6))

(event `Key|F`
  (params (Key :type "Key Structure")))

(event `Blink`
  (`UserWidget.PlayAnimation` (stale `MonitorOff` _returnvalue) (`/Game/Core/Assets/Widgets/PlayerUI.Blink` (stale `MonitorOff` _returnvalue)) 0.0 1 "Forward" 1.0 false))

(event `Key|SpaceBar`
  (params (Key :type "Key Structure"))
  (:`Pressed`
    (`/Engine/EditorBlueprintResources/StandardMacros.FlipFlop`
      (:`A`
        (`/Engine/EditorBlueprintResources/StandardMacros.DoOnce` false :!label _label_7
          (:`Completed`
            (if (`self.CanMonitor?`)
              (`/Engine/EditorBlueprintResources/StandardMacros.FlipFlop`
                (:`A`
                  (`GameplayStatics.PlaySound2D` "/Game/Core/Assets/Sounds/panel_in2.panel_in2" 1.0 1.0 0.0 null null)
                  (set `self.MonitorUp` true)
                  (bind (_direction _movement_z _movementforward) (`Timeline|MonitorMove` :!via `PlayFromStart` :!label _label_8)
                    (:`Update`
                      (`SceneComponent.K2_SetRelativeLocationAndRotation` (`self.Monitor`) (`KismetMathLibrary.MakeVector` _movementforward 0.0 _movement_z) (`KismetMathLibrary.MakeRotator` 0.0 0.0 90.0) false false))
                    (:`Finished`
                      (if (`self.MonitorUp`)
                        (`self.MonitorOn`))
                      (`KismetSystemLibrary.Delay` 0.05)
                      (`self.MonitorAgain`))))
                (:`B`
                  (`GameplayStatics.PlaySound2D` "/Game/Core/Assets/Sounds/panel_out.panel_out" 1.0 1.0 0.0 null null :!label _label_9)
                  (set `self.MonitorUp` false)
                  (`self.MonitorOff`)
                  (goto _label_8 :!via `Reverse`))))))))))

(event `CameraIdleShake`
  (bind _springarm1 (`self.SpringArm1`))
  (if (`self.Spooked`)
    (bind (_direction _shake) (`Timeline|IdleSpooked` :!via `PlayFromStart`)
      (:`Update`
        (`SceneComponent.K2_SetRelativeLocation` _springarm1 (`KismetMathLibrary.MakeVector` (* _shake 2.0) (* _shake 2.0) (* _shake 2.0)) false false)
        (`SceneComponent.K2_SetRelativeRotation` _springarm1 (`KismetMathLibrary.MakeRotator` (* _shake 2.0) (* _shake 2.0) (* _shake 2.0)) false false)
        (`KismetSystemLibrary.Delay` 1.0)
        (`GameplayStatics.PlaySound2D` "/Game/Core/Assets/Sounds/Heartbeat_Fast__patobottos_.Heartbeat_Fast__patobottos_" 1.0 1.0 0.0 null null)))
    (else
      (bind (_direction_2 _x) (`Timeline|Idle` :!via `PlayFromStart`)
        (:`Update`
          (`SceneComponent.K2_SetRelativeLocation` _springarm1 (`KismetMathLibrary.MakeVector` (* _x 0.5) (* _x 0.5) (* _x 0.5)) false false)
          (`SceneComponent.K2_SetRelativeRotation` _springarm1 (`KismetMathLibrary.MakeRotator` (* _x 0.5) (* _x 0.5) (* _x 0.5)) false false))))))

(event `MonitorAgain`
  (goto _label_7 :!via `Reset`))

(event `UpdateDoF`
  (bind _returnvalue (`SceneComponent.K2_GetComponentLocation` (`self.Camera`)))
  (bind (_outhit _returnvalue_2) (`KismetSystemLibrary.LineTraceSingle` _returnvalue (+ (* (`SceneComponent.GetForwardVector` (`self.Camera`)) 10000.0) _returnvalue) "TraceTypeQuery1"))
  (if _returnvalue_2
    (set `self.Focal Length` (`KismetMathLibrary.VSize` (- (`.Location` (`GameplayStatics.BreakHitResult` _outhit)) (`SceneComponent.K2_GetComponentLocation` (`self.Camera`)))))
    (set `CameraComponent.PostProcessSettings` (make `PostProcessSettings` :`DepthOfFieldFstop` 1.0 :`DepthOfFieldMinFstop` 1.0 :`DepthOfFieldFocalDistance` (`self.Focal Length`)) (`self.Camera`))
    (else
      (set `self.Focal Length` 1000000.0))))

(event `MonitorForceDown`
  (goto _label_9))

(event `SpookMovement`
  (bind _camera (`self.Camera`))
  (set `self.Spooked` true)
  (`|ExecutionSequence`
    (:`then_0`
      (bind (_direction _fov) (`Timeline|Spook` :!via `PlayFromStart`)
        (:`Update`
          (`CameraComponent.SetFieldOfView` _camera _fov))))
    (:`then_1`
      (bind (_direction_2 _rot) (`Timeline|RotationalCameraSpook` :!via `PlayFromStart`)
        (:`Update`
          (`SceneComponent.K2_SetRelativeRotation` _camera (`KismetMathLibrary.MakeRotator` (* _rot 0.5) _rot) false false))))
    (:`then_2`
      (`KismetSystemLibrary.Delay` (`KismetMathLibrary.RandomFloatInRange` 8.0 15.0))
      (set `self.Spooked` false))))

(event `PowerOff`
  (bind _monitor (`self.Monitor`))
  (`PrimitiveComponent.SetMaterial` _monitor 1 "/Game/Core/Assets/Props/Pizzas/Pizza02/Black.Black")
  (`PrimitiveComponent.SetMaterial` _monitor 0 "/Game/Core/Assets/Props/Pizzas/Pizza02/Black.Black")
  (`Widget.RemoveFromParent` (stale `MonitorOff` _returnvalue)))

(event `JumpscareImminent`
  (`PlayerCameraManager.StartCameraShake` :`self` (`GameplayStatics.GetPlayerCameraManager` 0) :`ShakeClass` "/Game/Core/Player/CameraShake/SpookCameraShakeBP.SpookCameraShakeBP_C")
  (set `self.JumpscareAboutToHappen` true))

(fn `UserConstructionScript`)